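; BP_InterestPoint_Base is a base interest point for the quest system that displays its text to a player and can reward discovery.
; CheckPawn takes the pawn's PlayerController and sends it the point text through Blueprint Interface messages, regardless of tags.
; If the controller's gameplay tags pass PlayerTagQuery, it also grants experience and adds the interest point's tags.
; No trigger calling CheckPawn is defined here.
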(fn ConstructionScript)

(fn CheckPawn
  (params (Pawn :type Pawn%20Object%20Reference))
  ;[1 1 1] Check pawn and do interest point actions.
  (bind _asplayer_controller (Utilities|Casting|CastToPlayerController (Pawn|GetController Pawn)))
  (Class|BPIPlayer|ShowInterestPointBPI(Message) _asplayer_controller (Variables|InterestPoint|GetPointText))
  (bind _result (Class|BPIPlayer|CheckGameplayTagQueryBPI(Message) _asplayer_controller (Variables|InterestPoint|GetPlayerTagQuery)))
  (if _result
    (Class|BPIPlayer|AddExperienceBPI(Message) _asplayer_controller (Variables|InterestPoint|GetExperience))
    (Class|BPIPlayer|AddGameplayTagsBPI(Message) _asplayer_controller (Variables|InterestPoint|GetInterestPointTags))))