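; BP_SplineMovedActor_Mesh is a spline-moved actor variant that uses static meshes as the moved objects.
; The construction script shows the chosen StaticMesh on a Mesh component, which is destroyed at BeginPlay.
; Overridden parent events add a static mesh component snapped to each spawned scene component and track it in MovedStaticMeshes.
; When a scene is destroyed, meshes attached to it are destroyed before the parent handles the rest.
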(event EventDestroyScene
  (params (Scene :type Scene%20Component%20Object%20Reference))
  ;[1 1 1] Overridden events.
  (for _array_element (Variables|SplineMovedActor|GetMovedStaticMeshes)
    (if (== (Transformation|GetAttachParent _array_element) Scene)
      (Components|DestroyComponent _array_element)))
  (|CallParentFunction 0))

(event EventBeginPlay
  ;[1 1 1] Overridden events.
  (Components|DestroyComponent (Variables|Default|GetMesh))
  (|CallParentFunction))

(event EventSpawnandAttachtoScene
  (params (Scene :type Scene%20Component%20Object%20Reference))
  ;[1 1 1] Overridden events.
  (SplineMovedActor|SpawnMeshComponent Scene))

(fn ConstructionScript
  (|CallParentFunction)
  (Components|StaticMesh|SetStaticMesh (Variables|Default|GetMesh) (Variables|SplineMovedActor|Spawn|GetStaticMesh)))

(fn SpawnMeshComponent
  (params (Scene :type Scene%20Component%20Object%20Reference))
  (bind _returnvalue (AddComponent|AddStaticMeshComponent true))
  (Components|StaticMesh|SetStaticMesh _returnvalue (Variables|SplineMovedActor|Spawn|GetStaticMesh))
  (Utilities|Array|Add (Variables|SplineMovedActor|GetMovedStaticMeshes) _returnvalue)
  (Transformation|AttachComponentToComponent _returnvalue Scene "None" "SnapToTarget" "SnapToTarget" "SnapToTarget" true))