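; Spline-moved actor variant that moves clusters of instanced static meshes in place of a single mesh.
; The Mesh component shows the static mesh from construction and is destroyed at BeginPlay.
; Each scene component passed to the spawn override gets an attached instanced mesh component holding a random number of instances at random offsets within MaxOffsets.
; Destroying a scene also destroys the tracked instanced components attached to it.
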(event EventSpawnandAttachtoScene
  (params (Scene :type Scene%20Component%20Object%20Reference))
  ;[1 1 1] Overridden events.
  (SplineMovedActor|SpawnInstancedComponent Scene))

(event EventDestroyScene
  (params (Scene :type Scene%20Component%20Object%20Reference))
  ;[1 1 1] Overridden events.
  (for _array_element (Variables|SplineMovedActor|GetMovedInstancedMeshes)
    (if (== (Transformation|GetAttachParent _array_element) Scene)
      (Components|DestroyComponent _array_element)))
  (|CallParentFunction Scene))

(event EventBeginPlay
  ;[1 1 1] Overridden events.
  (Components|DestroyComponent (Variables|Default|GetMesh))
  (|CallParentFunction))

(fn ConstructionScript
  (|CallParentFunction)
  (Components|StaticMesh|SetStaticMesh (Variables|Default|GetMesh) (Variables|SplineMovedActor|Spawn|GetStaticMesh)))

(fn SpawnInstancedComponent
  (params (Scene :type Scene%20Component%20Object%20Reference))
  (bind _maxoffsets (Variables|SplineMovedActor|Spawn|GetMaxOffsets))
  (bind (_x _y _z) (Math|Vector|BreakVector _maxoffsets))
  ;[1 1 1] Spawn instanced static mesh component and attach to scene component.
  (bind _returnvalue (AddComponent|AddInstancedStaticMeshComponent true))
  (Components|StaticMesh|SetStaticMesh _returnvalue (Variables|SplineMovedActor|Spawn|GetStaticMesh))
  (Transformation|AttachComponentToComponent _returnvalue Scene "None" "SnapToTarget" "SnapToTarget" "SnapToTarget" true)
  (Utilities|Array|Add (Variables|SplineMovedActor|GetMovedInstancedMeshes) _returnvalue)
  (for _index (range 0 (- (Math|Random|RandomIntegerinRange (Variables|SplineMovedActor|Spawn|GetMinInstancedCount) (Variables|SplineMovedActor|Spawn|GetMaxInstancedCount)) 1))
    (Components|InstancedStaticMesh|AddInstance _returnvalue (Math|Transform|MakeTransform (Math|Vector|MakeVector (Math|Random|RandomFloatinRange (* _x -1.0) _x) (Math|Random|RandomFloatinRange (* _y -1.0) _y) (Math|Random|RandomFloatinRange (* _z -1.0) _z)) "0, 0, 0" "1.000000,1.000000,1.000000") false)))