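; Base actor that spawns scene components and moves them along a spline, with child classes overriding what gets attached and how it is destroyed.
; Spawns come from begin play, random-delay timers or character overlap on a trigger, limited by chance and max count.
; Tick advances parallel scene and time arrays, placing each by spline time, then destroying it or resetting its time at the end.
; Construction derives duration from movement speed and closes cycled splines.
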(event Custom|OnTriggerOverlap
  (params (OverlappedActor :type Actor%20Object%20Reference) (OtherActor :type Actor%20Object%20Reference))
  ;[1 1 1] On character overlap trigger event.
  (Utilities|Casting|CastToCharacter OtherActor)
  (SplineMovedActor|SpawnandMovetoSpline))

(event EventTick
  (params (DeltaSeconds :type Float%20%28single-precision%29))
  ;[1 1 1] Update tick.
  (SplineMovedActor|UpdateTick DeltaSeconds))

(event EventBeginPlay
  (bind _trigger (Variables|SplineMovedActor|Spawn|GetTrigger))
  ;[1 1 1] Begin play. Check spawn on begin play.
  (Utilities|IsValid _trigger
    (:Is%20Valid
      (Collision|BindEventtoOnActorBeginOverlap _trigger (EventDispatchers|CreateEvent :!event Custom|OnTriggerOverlap)))
    (:Is%20Not%20Valid
      _))
  (if (Variables|SplineMovedActor|Spawn|GetSpawnOnBeginPlay)
    (SplineMovedActor|SpawnandMovetoSpline))
  (if (Variables|SplineMovedActor|Spawn|GetSpawnOnTimer)
    (Utilities|Time|SetTimerbyEvent (EventDispatchers|CreateEvent :!event TrytoSpawn) (Math|Random|RandomFloatinRange (Variables|SplineMovedActor|Spawn|GetMinSpawnDelay) (Variables|SplineMovedActor|Spawn|GetMaxSpawnDelay)))))

(fn ConstructionScript
  (bind _spline (Variables|Default|GetSpline))
  (Variables|/Script/Engine.SplineComponent|SetDuration _spline (/ (Spline|GetSplineLength _spline) (Variables|SplineMovedActor|Spawn|GetMovementSpeed)))
  (SplineMovedActor|CorrectCycledSpline))

(fn SpawnandMovetoSpline
  (bind _maxcount (Variables|SplineMovedActor|Spawn|GetMaxCount))
  ;[1 1 1] Spawn scene component and add to moving array.
  (if (and (or (== _maxcount 0) (< (Utilities|Array|Length (Variables|SplineMovedActor|GetMovedScenes)) _maxcount)) (<= (Math|Random|RandomFloat) (Variables|SplineMovedActor|Spawn|GetTriggerChance)))
    (bind _returnvalue (AddComponent|AddSceneComponent false))
    (SplineMovedActor|SpawnandAttachtoScene _returnvalue)
    (SplineMovedActor|UpdateScenePosition _returnvalue 0.0)
    (Utilities|Array|Add (Variables|SplineMovedActor|GetMovedScenes) _returnvalue)
    (Utilities|Array|Add (Variables|SplineMovedActor|GetMovedTimes) 0.0)))

(fn UpdateScenePosition
  (params (Scene :type Scene%20Component%20Object%20Reference) (Time :type Float%20%28single-precision%29))
  ;[1 1 1] Update scene component position on the spline by time.
  (Transformation|SetRelativeTransform Scene (Spline|GetTransformatTime (Variables|Default|GetSpline) Time "Local" false false) false false)
  (Transformation|AddRelativeRotation Scene (Variables|SplineMovedActor|Spawn|GetRelativeRotation) false false))

(fn RefreshPoints
  (bind _spline (Variables|Default|GetSpline))
  (bind _spline_2 (Variables|Default|GetSpline))
  (bind _spline_3 (Variables|Default|GetSpline))
  (bind _returnvalue (Spline|GetNumberOfSplinePoints _spline))
  (bind _returnvalue_2 (- _returnvalue 1))
  ;[1 1 1] Smooth and correct spline points.
  (SplineMovedActor|CorrectCycledSpline)
  (LocalVariables|SetLocalPoints _returnvalue)
  (LocalVariables|SetLocalDif (/ (Spline|GetSplineLength _spline) (Math|Conversions|ToFloat(Integer) _returnvalue_2)))
  (for _index (range 0 _returnvalue_2)
    (Utilities|Array|Add (LocalVariables|GetLocalSplinePoints) (Utilities|Struct|MakeSplinePoint (Math|Conversions|ToFloat(Integer) _index) (Spline|GetLocationatDistanceAlongSpline _spline_2 (* (LocalVariables|GetLocalDif) (Math|Conversions|ToFloat(Integer) _index)) "Local") "0, 0, 0" "0, 0, 0" (Spline|GetRotationatDistanceAlongSpline _spline_2 (* (LocalVariables|GetLocalDif) (Math|Conversions|ToFloat(Integer) _index)) "Local"))))
  (Spline|ClearSplinePoints _spline_3 false)
  (Class|SplineComponent|AddPoints _spline_3 (LocalVariables|GetLocalSplinePoints) true))

(fn CorrectCycledSpline
  (bind _spline (Variables|Default|GetSpline))
  (bind _returnvalue (Spline|GetNumberOfSplinePoints _spline))
  ;[1 1 1] Check spline is cycled and set last point position in first point position.
  (if (and (Variables|SplineMovedActor|Spawn|GetCycledSpline) (> _returnvalue 2))
    (Spline|SetLocationatSplinePoint _spline (- _returnvalue 1) (Spline|GetLocationatSplinePoint (Variables|Default|GetSpline) 0 "Local") "Local" true)))

(fn SpawnandAttachtoScene
  (params (Scene :type Scene%20Component%20Object%20Reference))
  ;[1 1 1] Spawn addition components and attach to scene. Overridden in child class.
)

(fn DestroyScene
  (params (Scene :type Scene%20Component%20Object%20Reference))
  ;[1 1 1] Destroy scene component. Overridden in child class.
  (Components|DestroyComponent Scene))

(fn TrytoSpawn
  ;[1 1 1] Try to spawn scene component.
  (SplineMovedActor|SpawnandMovetoSpline)
  (if (< (Utilities|Array|Length (Variables|SplineMovedActor|GetMovedScenes)) (Variables|SplineMovedActor|Spawn|GetMaxCount))
    (Utilities|Time|SetTimerbyEvent (EventDispatchers|CreateEvent :!event TrytoSpawn) (Math|Random|RandomFloatinRange (Variables|SplineMovedActor|Spawn|GetMinSpawnDelay) (Variables|SplineMovedActor|Spawn|GetMaxSpawnDelay)))))

(fn UpdateTick
  (params (DeltaSeconds :type Float%20%28single-precision%29))
  (bind _movedtimes (Variables|SplineMovedActor|GetMovedTimes))
  (bind _spline (Variables|Default|GetSpline))
  (bind _duration (Variables|/Script/Engine.SplineComponent|GetDuration _spline))
  ;[1 1 1] Update scenes position on the spline.
  (for (_array_element _array_index) (Variables|SplineMovedActor|GetMovedScenes)
    (Utilities|Array|SetArrayElem _movedtimes _array_index (Math|Float|Clamp(Float) (+ (Utilities|Array|Get(acopy) _movedtimes _array_index) DeltaSeconds) 0.0 _duration))
    (SplineMovedActor|UpdateScenePosition _array_element (Utilities|Array|Get(acopy) _movedtimes _array_index))
    (if (== (Math|Float|Clamp(Float) (+ (Utilities|Array|Get(acopy) _movedtimes _array_index) DeltaSeconds) 0.0 _duration) _duration)
      (if (Variables|SplineMovedActor|Spawn|GetDestroyWhenFinish)
        (SplineMovedActor|DestroyScene _array_element)
        (Utilities|Array|RemoveIndex (Variables|SplineMovedActor|GetMovedScenes) _array_index)
        (Utilities|Array|RemoveIndex (Variables|SplineMovedActor|GetMovedTimes) _array_index)
        (Utilities|Time|SetTimerbyEvent (EventDispatchers|CreateEvent :!event TrytoSpawn) (Math|Random|RandomFloatinRange (Variables|SplineMovedActor|Spawn|GetMinSpawnDelay) (Variables|SplineMovedActor|Spawn|GetMaxSpawnDelay)))
        (else
          (Utilities|Array|SetArrayElem (Variables|SplineMovedActor|GetMovedTimes) _array_index 0.0))))))