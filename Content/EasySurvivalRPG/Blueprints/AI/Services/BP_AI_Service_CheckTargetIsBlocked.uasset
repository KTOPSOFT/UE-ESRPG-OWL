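; Behavior tree service that flags in the blackboard whether something blocks the path between the AI pawn and its target actor.
; Each tick it sphere-traces on Visibility toward a valid target, ignoring both actors and stopping short of the target.
; The flag is true only when the hit component blocks GameTraceChannel7; without a valid target it stays unchanged.
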(event EventReceiveTickAI
  (params (OwnerController :type AI%20Controller%20Object%20Reference) (ControlledPawn :type Pawn%20Object%20Reference) (DeltaSeconds :type Float%20%28single-precision%29))
  ;[1 1 1] Check target actor on tick.
  (CallFunction|CheckTargetIsBlockedTarget OwnerController ControlledPawn))

(fn CheckTargetIsBlockedTarget
  (params (OwnerController :type AI%20Controller%20Object%20Reference) (ControlledPawn :type Pawn%20Object%20Reference))
  (bind _returnvalue (Transformation|GetActorLocation ControlledPawn))
  (bind _targetactor (Variables|Blackboard|GetTargetActor))
  (bind _updatetargetisblocked (Variables|Blackboard|GetUpdateTargetIsBlocked))
  (bind _returnvalue_2 (AI|BehaviorTree|GetBlackboardValueasActor _targetactor))
  ;[1 1 1] Update target is blocked blackboard property.
  (Utilities|IsValid _returnvalue_2
    (:Is%20Valid
      (bind _output_get (LocalVariables|SetLocalTargetActor _returnvalue_2))
      (bind (_outhit _returnvalue_3) (Collision|SphereTraceByChannel _returnvalue (CallFunction|GetTraceEnd _returnvalue (Transformation|GetActorLocation _output_get)) 25.0 "TraceTypeQuery1" true (Utilities|Array|MakeArray ControlledPawn (LocalVariables|GetLocalTargetActor)) "None" true "(R=1.000000,G=0.000000,B=0.000000,A=1.000000)" "(R=0.000000,G=1.000000,B=0.000000,A=1.000000)" 1.0))
      (if _returnvalue_3
        (if (Utilities|Enum|Equal(Enum) (Collision|GetCollisionResponsetoChannel (.HitComponent (Collision|BreakHitResult _outhit)) "ECC_GameTraceChannel7") "ECR_Block")
          (Class|BTFunctionLibrary|SetBlackboardValueasBool _updatetargetisblocked true)
          (else
            (Class|BTFunctionLibrary|SetBlackboardValueasBool _updatetargetisblocked false :!label _label)))
        (else
          (goto _label)))
      (return true))))

(fn GetTraceEnd
  (params (PawnLocation :type Vector) (TargetLocation :type Vector))
  (bind _returnvalue (- TargetLocation PawnLocation))
  (bind _returnvalue_2 (Math|Vector|VectorLength _returnvalue))
  (bind _returnvalue_3 (- _returnvalue_2 1e+02))
  ;[1 1 1] Returns trace end location.
  (return (+ PawnLocation (* (Math|Vector|Normalize _returnvalue) (Math|Float|Clamp(Float) _returnvalue_3 0.0 _returnvalue_3)))))