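; Base behavior tree service for AI actions that runs an action on each tick when its conditions pass.
; Conditions check an ability cooldown, the blackboard target's distance against a range, and its yaw angle within a sight cone, the latter two invertible.
; Cooldowns go through the pawn's BP_AbilitySystemComponent and pass if it or the ID is missing.
; DoActions here only starts the cooldown and returns true.
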(event EventReceiveTickAI
  (params (OwnerController :type AI%20Controller%20Object%20Reference) (ControlledPawn :type Pawn%20Object%20Reference) (DeltaSeconds :type Float%20%28single-precision%29))
  ;[1 1 1] Check action conditions and do action on service tick.
  (bind _success (CallFunction|CheckConditions ControlledPawn))
  (if _success
    (CallFunction|DoActions ControlledPawn)))

(fn CheckDistancetoTarget
  (params (ControlledPawn :type Pawn%20Object%20Reference))
  (bind _targetactor (Variables|Blackboard|GetTargetActor))
  (bind _range (Variables|Settings|CheckDistance|GetRange))
  (bind _returnvalue (AI|BehaviorTree|GetBlackboardValueasActor _targetactor))
  (bind _returnvalue_2 (Transformation|GetDistanceTo _returnvalue ControlledPawn))
  (bind _returnvalue_3 (<= _returnvalue_2 _range))
  ;[1 1 1] Check distance to target actor.
  (if (> (Variables|Settings|CheckDistance|GetRange) 0.0)
    (Utilities|IsValid _returnvalue
      (:Is%20Valid
        (return (select (Variables|Settings|CheckDistance|GetInRange) _returnvalue_3 (not _returnvalue_3))))
      (:Is%20Not%20Valid
        (return false)))
    (else
      (return true))))

(fn CheckTargetinSight
  (params (ControlledPawn :type Pawn%20Object%20Reference))
  (bind _returnvalue (Transformation|GetActorLocation ControlledPawn))
  (bind _returnvalue_2 (Transformation|GetActorRotation ControlledPawn))
  (bind _targetactor (Variables|Blackboard|GetTargetActor))
  (bind _sightangle (Variables|Settings|CheckSight|GetSightAngle))
  (bind _returnvalue_3 (AI|BehaviorTree|GetBlackboardValueasActor _targetactor))
  (bind _returnvalue_4 (Math|Rotator|MakeRotator 0.0 0.0 (.yaw _returnvalue_2)))
  (bind _returnvalue_5 (Transformation|GetActorLocation _returnvalue_3))
  (bind _returnvalue_6 (Math|Rotator|FindLookatRotation _returnvalue _returnvalue_5))
  (bind _returnvalue_7 (Math|Rotator|MakeRotator 0.0 0.0 (.yaw _returnvalue_6)))
  (bind _returnvalue_8 (Math|Rotator|Equal(Rotator) _returnvalue_4 _returnvalue_7 _sightangle))
  ;[1 1 1] Check that the target actor in sight of the pawn.
  (if (> (Variables|Settings|CheckSight|GetSightAngle) 0.0)
    (Utilities|IsValid _returnvalue_3
      (:Is%20Valid
        (return (select (Variables|Settings|CheckSight|GetInSight) _returnvalue_8 (not _returnvalue_8))))
      (:Is%20Not%20Valid
        (return false)))
    (else
      (return true))))

(fn CheckConditions
  (params (ControlledPawn :type Pawn%20Object%20Reference))
  ;[1 1 1] Check action conditions.
  (bind _success (CallFunction|CheckCooldown ControlledPawn))
  (if _success
    (bind _success_2 (CallFunction|CheckDistancetoTarget ControlledPawn))
    (if _success_2
      (bind _success_3 (CallFunction|CheckTargetinSight ControlledPawn))
      (if _success_3
        (return true)
        (else
          (return false)))
      (else
        (return false)))
    (else
      (return false))))

(fn DoActions
  (params (ControlledPawn :type Pawn%20Object%20Reference))
  ;[1 1 1] Do actions and start cooldown.
  (Utilities|FlowControl|Sequence
    (:then_0
      (if (> (Variables|Settings|Cooldown|GetCooldownTime) 0.0)
        (CallFunction|StartCooldown ControlledPawn)))
    (:then_1
      (return true))))

(fn CheckCooldown
  (params (ControlledPawn :type Pawn%20Object%20Reference))
  (bind _returnvalue (Actor|GetComponentbyClass ControlledPawn "/Game/EasySurvivalRPG/Blueprints/Components/BP_AbilitySystemComponent.BP_AbilitySystemComponent_C"))
  ;[1 1 1] Check action conditions.
  (if (Utilities|Name|NotEqual(Name) (Variables|Settings|Cooldown|GetAbilityCooldownID) "None")
    (Utilities|IsValid _returnvalue
      (:Is%20Valid
        (bind _success (Default|CheckAbilityCooldown _returnvalue (Variables|Settings|Cooldown|GetAbilityCooldownID)))
        (return _success))
      (:Is%20Not%20Valid
        _)))
  (return true))

(fn StartCooldown
  (params (ControlledPawn :type Pawn%20Object%20Reference))
  (bind _returnvalue (Actor|GetComponentbyClass ControlledPawn "/Game/EasySurvivalRPG/Blueprints/Components/BP_AbilitySystemComponent.BP_AbilitySystemComponent_C"))
  ;[1 1 1] Check action conditions.
  (if (Utilities|Name|NotEqual(Name) (Variables|Settings|Cooldown|GetAbilityCooldownID) "None")
    (Utilities|IsValid _returnvalue
      (:Is%20Valid
        (bind _success (Default|StartAbilityCooldown _returnvalue (Variables|Settings|Cooldown|GetAbilityCooldownID) (Variables|Settings|Cooldown|GetCooldownTime)))
        (return _success))
      (:Is%20Not%20Valid
        _)))
  (return true))