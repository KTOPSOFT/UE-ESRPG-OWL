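; Behavior tree service for EasySurvivalRPG AI that validates the blackboard target actor on every service tick.
; The target must be alive and closer to GuardLocation than ChasingDistance, measured from that guard point rather than the pawn, with CheckChasingDistance enabled.
; A passing target gets controller focus.
; Otherwise, including when CheckChasingDistance is off, it clears the pawn's target through an interface message and drops focus.
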(event EventReceiveTickAI
  (params (OwnerController :type AI%20Controller%20Object%20Reference) (ControlledPawn :type Pawn%20Object%20Reference) (DeltaSeconds :type Float%20%28single-precision%29))
  ;[1 1 1] Check target actor on tick.
  (CallFunction|CheckTargetActor OwnerController ControlledPawn))

(fn CheckTargetActor
  (params (OwnerController :type AI%20Controller%20Object%20Reference) (ControlledPawn :type Pawn%20Object%20Reference))
  ;[1 1 1] Check that target actor is alive and it is in chasing distance.
  (bind _output_get (LocalVariables|SetLocalTargetActor (AI|BehaviorTree|GetBlackboardValueasActor (Variables|Blackboard|GetTargetActor))))
  (Utilities|IsValid _output_get
    (:Is%20Valid
      (bind _result (Class|BPICharacter|IsAliveBPI(Message) _output_get))
      (if _result
        (bind _success (CallFunction|CheckChaseTarget))
        (if _success
          (AI|SetFocus OwnerController (LocalVariables|GetLocalTargetActor))
          (return _success)
          (else
            _))))
    (:Is%20Not%20Valid
      _))
  (Class|BPICharacter|ClearTargetActorBPI(Message) ControlledPawn)
  (AI|ClearFocus OwnerController)
  (return true))

(fn CheckChaseTarget
  ;[1 1 1] Returns true if target actor is in chasing distance.
  (if (Class|BTFunctionLibrary|GetBlackboardValueasBool (Variables|Blackboard|GetCheckChasingDistance))
    (bind _output_get (LocalVariables|SetLocalTargetActor (AI|BehaviorTree|GetBlackboardValueasActor (Variables|Blackboard|GetTargetActor))))
    (Utilities|IsValid _output_get
      (:Is%20Valid
        (return (> (Class|BTFunctionLibrary|GetBlackboardValueasFloat (Variables|Blackboard|GetChasingDistance)) (Math|Vector|VectorLength (- (Transformation|GetActorLocation _output_get) (Class|BTFunctionLibrary|GetBlackboardValueasVector (Variables|Blackboard|GetGuardLocation)))))))
      (:Is%20Not%20Valid
        _)))
  (return false))