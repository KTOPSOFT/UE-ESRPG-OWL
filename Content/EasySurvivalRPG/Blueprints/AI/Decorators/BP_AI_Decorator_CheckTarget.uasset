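; AI behavior tree decorator that gates a branch on whether the controlled pawn's target actor is still alive.
; It reads the TargetActor blackboard value and queries it through an IsAlive interface message, passing only when the target is valid and alive.
; Otherwise it fails and, as a side effect of the check, calls ClearTargetActor on the pawn if it is a BP_Character_Base.
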(fn PerformConditionCheckAI
  (params (OwnerController :type AI%20Controller%20Object%20Reference) (ControlledPawn :type Pawn%20Object%20Reference))
  ;[1 1 1] Return true if target is Alive. Else clear Target.
  (bind _output_get (LocalVariables|SetLocalTargetActor (AI|BehaviorTree|GetBlackboardValueasActor (Variables|Blackboard|GetTargetActor))))
  (Utilities|IsValid _output_get
    (:Is%20Valid
      (bind _result (Class|BPICharacter|IsAliveBPI(Message) _output_get))
      (if _result
        (return true)
        (else
          _)))
    (:Is%20Not%20Valid
      _))
  (bind _asbp_character_base (Utilities|Casting|CastToBP_Character_Base ControlledPawn)
    (:then
      (Default|ClearTargetActor _asbp_character_base))
    (:CastFailed
      _))
  (return false))