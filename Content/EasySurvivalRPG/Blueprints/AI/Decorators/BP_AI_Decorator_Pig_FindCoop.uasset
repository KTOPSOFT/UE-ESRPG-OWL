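; Behavior tree decorator for pig AI that passes when the controlled animal needs to find a coop.
; On observer activation, it casts the controlled pawn to BP_Character_Pig, or failing that BP_Character_Swine, and caches the reference.
; The condition check returns the NeedToFindCoop flag from whichever cached reference is valid, checking the pig first.
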(event EventReceiveObserverActivatedAI
  (params (OwnerController :type AI%20Controller%20Object%20Reference) (ControlledPawn :type Pawn%20Object%20Reference))
  ;[1 1 1] Set correct character reference.
  (bind _asbp_character_pig (Utilities|Casting|CastToBP_Character_Pig ControlledPawn)
    (:then
      (Variables|Default|SetPigReference _asbp_character_pig))
    (:CastFailed
      (bind _asbp_character_swine (Utilities|Casting|CastToBP_Character_Swine ControlledPawn))
      (Variables|Default|SetSwineReference _asbp_character_swine))))

(fn PerformConditionCheckAI
  (params (OwnerController :type AI%20Controller%20Object%20Reference) (ControlledPawn :type Pawn%20Object%20Reference))
  ;[1 1 1] Returns true, if pig wants to find a coop.
  (Utilities|IsValid (Variables|Default|GetPigReference)
    (:Is%20Valid
      (return (Variables|/Game/EasySurvivalRPG/Blueprints/Characters/Base/BP_Character_Pig.BP_Character_Pig_C|GetNeedToFindCoop (Variables|Default|GetPigReference))))
    (:Is%20Not%20Valid
      (Utilities|IsValid (Variables|Default|GetSwineReference)
        (:Is%20Valid
          (return (Variables|/Game/EasySurvivalRPG/Blueprints/Characters/Base/BP_Character_Swine.BP_Character_Swine_C|GetNeedToFindCoop (Variables|Default|GetSwineReference))))))))