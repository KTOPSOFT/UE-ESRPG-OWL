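; Behavior tree decorator that passes when the blackboard Target actor lies within the AI pawn's facing angle.
; It compares the pawn's yaw with the look-at yaw toward the target, using SightAngle as the tolerance and ignoring pitch and roll.
; It fails when the target is invalid, and checks neither distance nor line of sight.
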(fn PerformConditionCheckAI
  (params (OwnerController :type AI%20Controller%20Object%20Reference) (ControlledPawn :type Pawn%20Object%20Reference))
  (bind _target (Variables|Blackboard|GetTarget))
  (bind _returnvalue (AI|BehaviorTree|GetBlackboardValueasActor _target))
  ;[1 1 1] Return true if target actor in controller sight.
  (Utilities|IsValid _returnvalue
    (:Is%20Valid
      (return (Math|Rotator|Equal(Rotator) (Math|Rotator|MakeRotator 0.0 0.0 (.yaw (Transformation|GetActorRotation ControlledPawn))) (Math|Rotator|MakeRotator 0.0 0.0 (.yaw (Math|Rotator|FindLookatRotation (Transformation|GetActorLocation ControlledPawn) (Transformation|GetActorLocation _returnvalue)))) (Variables|Default|GetSightAngle))))
    (:Is%20Not%20Valid
      (return false))))