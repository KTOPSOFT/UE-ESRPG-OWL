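; Behavior tree decorator for chicken AI that passes when the controlled chicken wants to find food.
; On observer activation it casts the controlled pawn to hen, rooster or chick and caches the matching reference.
; The condition check returns that character's NeedToFindFood flag from whichever cached reference is valid.
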(event EventReceiveObserverActivatedAI
  (params (OwnerController :type AI%20Controller%20Object%20Reference) (ControlledPawn :type Pawn%20Object%20Reference))
  ;[1 1 1] Set correct character reference.
  (bind _asbp_character_hen (Utilities|Casting|CastToBP_Character_Hen ControlledPawn)
    (:then
      (Variables|Default|SetHenReference _asbp_character_hen))
    (:CastFailed
      (bind _asbp_character_rooster (Utilities|Casting|CastToBP_Character_Rooster ControlledPawn)
        (:then
          (Variables|Default|SetRoosterReference _asbp_character_rooster))
        (:CastFailed
          (bind _asbp_character_chick (Utilities|Casting|CastToBP_Character_Chick ControlledPawn))
          (Variables|Default|SetChickReference _asbp_character_chick))))))

(fn PerformConditionCheckAI
  (params (OwnerController :type AI%20Controller%20Object%20Reference) (ControlledPawn :type Pawn%20Object%20Reference))
  ;[1 1 1] Returns true, if chicken wants to find a food.
  (Utilities|IsValid (Variables|Default|GetHenReference)
    (:Is%20Valid
      (return (Variables|/Game/EasySurvivalRPG/Blueprints/Characters/Base/BP_Character_Hen.BP_Character_Hen_C|GetNeedToFindFood (Variables|Default|GetHenReference))))
    (:Is%20Not%20Valid
      (Utilities|IsValid (Variables|Default|GetRoosterReference)
        (:Is%20Valid
          (return (Variables|/Game/EasySurvivalRPG/Blueprints/Characters/Base/BP_Character_Rooster.BP_Character_Rooster_C|GetNeedToFindFood (Variables|Default|GetRoosterReference))))
        (:Is%20Not%20Valid
          (Utilities|IsValid (Variables|Default|GetChickReference)
            (:Is%20Valid
              (return (Variables|/Game/EasySurvivalRPG/Blueprints/Characters/Base/BP_Character_Chick.BP_Character_Chick_C|GetNeedToFindFood (Variables|Default|GetChickReference))))))))))