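; Behavior tree decorator that gates food-seeking behavior for pig-family AI: pigs, swine and piglets.
; When the observer activates, it casts the controlled pawn to each of the three character classes and caches the matching reference.
; The condition check returns that character's NeedToFindFood flag, testing the cached references in pig, swine, piglet order.
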(event EventReceiveObserverActivatedAI
  (params (OwnerController :type AI%20Controller%20Object%20Reference) (ControlledPawn :type Pawn%20Object%20Reference))
  ;[1 1 1] Set correct character reference.
  (bind _asbp_character_pig (Utilities|Casting|CastToBP_Character_Pig ControlledPawn)
    (:then
      (Variables|Default|SetPigReference _asbp_character_pig))
    (:CastFailed
      (bind _asbp_character_swine (Utilities|Casting|CastToBP_Character_Swine ControlledPawn)
        (:then
          (Variables|Default|SetSwineReference _asbp_character_swine))
        (:CastFailed
          (bind _asbp_character_piglet (Utilities|Casting|CastToBP_Character_Piglet ControlledPawn))
          (Variables|Default|SetPigletReference _asbp_character_piglet))))))

(fn PerformConditionCheckAI
  (params (OwnerController :type AI%20Controller%20Object%20Reference) (ControlledPawn :type Pawn%20Object%20Reference))
  ;[1 1 1] Returns true, if pig wants to find a food.
  (Utilities|IsValid (Variables|Default|GetPigReference)
    (:Is%20Valid
      (return (Variables|/Game/EasySurvivalRPG/Blueprints/Characters/Base/BP_Character_Pig.BP_Character_Pig_C|GetNeedToFindFood (Variables|Default|GetPigReference))))
    (:Is%20Not%20Valid
      (Utilities|IsValid (Variables|Default|GetSwineReference)
        (:Is%20Valid
          (return (Variables|/Game/EasySurvivalRPG/Blueprints/Characters/Base/BP_Character_Swine.BP_Character_Swine_C|GetNeedToFindFood (Variables|Default|GetSwineReference))))
        (:Is%20Not%20Valid
          (Utilities|IsValid (Variables|Default|GetPigletReference)
            (:Is%20Valid
              (return (Variables|/Game/EasySurvivalRPG/Blueprints/Characters/Base/BP_Character_Piglet.BP_Character_Piglet_C|GetNeedToFindFood (Variables|Default|GetPigletReference))))))))))