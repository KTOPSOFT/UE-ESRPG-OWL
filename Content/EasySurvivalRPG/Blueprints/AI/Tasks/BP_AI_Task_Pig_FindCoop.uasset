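; Behavior tree task that sends an AI pig or swine to its assigned coop in the survival RPG.
; It clears the pawn's NeedToFindCoop flag, reads its TargetCoop, moves there and calls TryToLetInPig on arrival.
; A failed move still finishes the task as successful; only an unsupported pawn type reports failure.
; The PigToJoinCoop helper is an unused stub.
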(event EventReceiveExecuteAI
  (params (OwnerController :type AI%20Controller%20Object%20Reference) (ControlledPawn :type Pawn%20Object%20Reference))
  ;[1 1 1] Move to available feeder and play eat animation.
  (bind _success (CallFunction|PigResetVariables ControlledPawn))
  (if _success
    (bind (_found _targetcoop) (CallFunction|GetTargetCoop ControlledPawn))
    (if _found
      (AI|AIMoveTo ControlledPawn "0, 0, 0" _targetcoop 1e+02 true
        (:OnSuccess
          (Default|TrytoLetinPig _targetcoop ControlledPawn))
        (:OnFail
          _))
      (AI|BehaviorTree|FinishExecute true)
      (else
        (AI|BehaviorTree|FinishExecute false :!label _label)))
    (else
      (goto _label))))

(fn GetTargetCoop
  (params (ControlledPawn :type Pawn%20Object%20Reference))
  ;[1 1 1] Returns target pig coop.
  (bind _asbp_character_pig (Utilities|Casting|CastToBP_Character_Pig ControlledPawn)
    (:then
      (return true (Variables|/Game/EasySurvivalRPG/Blueprints/Characters/Base/BP_Character_Pig.BP_Character_Pig_C|GetTargetCoop _asbp_character_pig)))
    (:CastFailed
      (bind _asbp_character_swine (Utilities|Casting|CastToBP_Character_Swine ControlledPawn)
        (:then
          (return true (Variables|/Game/EasySurvivalRPG/Blueprints/Characters/Base/BP_Character_Swine.BP_Character_Swine_C|GetTargetCoop _asbp_character_swine)))
        (:CastFailed
          (return false 0))))))

(fn PigResetVariables
  (params (ControlledPawn :type Pawn%20Object%20Reference))
  ;[1 1 1] Reset variables.
  (bind _asbp_character_pig (Utilities|Casting|CastToBP_Character_Pig ControlledPawn)
    (:then
      (Variables|/Game/EasySurvivalRPG/Blueprints/Characters/Base/BP_Character_Pig.BP_Character_Pig_C|SetNeedToFindCoop _asbp_character_pig false))
    (:CastFailed
      (bind _asbp_character_swine (Utilities|Casting|CastToBP_Character_Swine ControlledPawn)
        (:then
          (Variables|/Game/EasySurvivalRPG/Blueprints/Characters/Base/BP_Character_Swine.BP_Character_Swine_C|SetNeedToFindCoop _asbp_character_swine false))
        (:CastFailed
          (return false)))))
  (return true))

(fn PigtoJoinCoop
  (params (ControlledPawn :type Pawn%20Object%20Reference) (TargetCoop :type BP%20Building%20Pig%20Coop%20Object%20Reference))
  ;[1 1 1] Try to eat.
  (Utilities|Casting|CastToBP_Character_Pig ControlledPawn
    (:CastFailed
      (Utilities|Casting|CastToBP_Character_Swine ControlledPawn
        (:CastFailed
          (return false))))))