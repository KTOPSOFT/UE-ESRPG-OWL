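; Behavior tree task that backs an AI pawn away from its target actor while keeping focus on it.
; It picks a random-distance point on the line between target and pawn, projects it onto the navmesh and validates it with a path trace.
; A valid point is written to the blackboard during the move, and the task succeeds even if the move fails.
; Otherwise it flags the target as blocked and fails.
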(event EventReceiveExecuteAI
  (params (OwnerController :type AI%20Controller%20Object%20Reference) (ControlledPawn :type Pawn%20Object%20Reference))
  (bind _updatetargetlocation (Variables|Blackboard|GetUpdateTargetLocation))
  ;[1 1 1] Move back from target actor.
  (bind _output_get (Variables|State|SetOwnerController OwnerController))
  (Variables|State|SetControlledPawn ControlledPawn)
  (AI|SetFocus _output_get (AI|BehaviorTree|GetBlackboardValueasActor (Variables|Blackboard|GetTargetActor)))
  (bind (_found _targetlocation) (CallFunction|FindBackLocation))
  (if _found
    (AI|BehaviorTree|SetBlackboardValueasVector (Variables|Blackboard|GetUpdateTargetLocation) _targetlocation)
    (AI|AIMoveTo (Variables|State|GetControlledPawn) _targetlocation 0 (Variables|Settings|GetAcceptanceRadius) true
      (:OnSuccess
        (Class|BTFunctionLibrary|ClearBlackboardValue _updatetargetlocation))
      (:OnFail
        (Class|BTFunctionLibrary|ClearBlackboardValue _updatetargetlocation)))
    (AI|BehaviorTree|FinishExecute true)
    (else
      (Class|BTFunctionLibrary|SetBlackboardValueasBool (Variables|Blackboard|GetUpdateTargetIsBlocked) true)
      (AI|BehaviorTree|FinishExecute false))))

(fn FindBackLocation
  ;[1 1 1] Try to find back location.
  (bind _output_get (LocalVariables|SetLocalTargetLocation (+ (.ProjectedLocation (AI|Navigation|ProjectPointtoNavigation (CallFunction|GetLocationBetweenActors (AI|BehaviorTree|GetBlackboardValueasActor (Variables|Blackboard|GetTargetActor)) (Variables|State|GetControlledPawn) (Math|Random|RandomFloatinRange (Variables|Settings|GetMinDistance) (Variables|Settings|GetMaxDistance))) 0 0 "0, 0, 0")) "0, 0,50.000000")))
  (bind _result (CallFunction|CheckPathbyTrace (Variables|State|GetControlledPawn) _output_get 3e+01))
  (if _result
    (return true (LocalVariables|GetLocalTargetLocation))
    (else
      (return false "0, 0, 0"))))