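; Behavior tree task that sends a hen, rooster or chick to a nearby chicken feeder to eat.
; It restarts the bird's find-food timer, sphere-traces around it for a feeder with food, then moves there with AIMoveTo.
; On arrival the bird tries to eat, restarts its timer and the feeder consumes food.
; A failed move still finishes as success; only an unsupported pawn or no feeder found fails the task.
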(event EventReceiveExecuteAI
  (params (OwnerController :type AI%20Controller%20Object%20Reference) (ControlledPawn :type Pawn%20Object%20Reference))
  ;[1 1 1] Move to available feeder and play eat animation.
  (bind _success (CallFunction|ChickenStartFindFoodTimer ControlledPawn))
  (if _success
    (bind (_found _targetactor) (CallFunction|TrytoFindFood ControlledPawn))
    (if _found
      (AI|AIMoveTo ControlledPawn "0, 0, 0" _targetactor 75.0 true
        (:OnSuccess
          (CallFunction|ChickenTryEat ControlledPawn _targetactor))
        (:OnFail
          _))
      (AI|BehaviorTree|FinishExecute true)
      (else
        (AI|BehaviorTree|FinishExecute false :!label _label)))
    (else
      (goto _label))))

(fn TrytoFindFood
  (params (ControlledPawn :type Pawn%20Object%20Reference))
  (bind _returnvalue (Transformation|GetActorLocation ControlledPawn))
  ;[1 1 1] Try to find available feeder.
  (bind _outhits (Collision|MultiSphereTraceForObjects _returnvalue _returnvalue 5e+02 (Utilities|Array|MakeArray "ObjectTypeQuery2") false 0 "None"))
  (for _array_element _outhits
    (bind _asbp_building_chicken_feeder (Utilities|Casting|CastToBP_Building_ChickenFeeder (.HitActor (Collision|BreakHitResult _array_element))))
    (if (Variables|/Game/EasySurvivalRPG/Blueprints/InteractionObjects/BuildingObjects/Farming/BP_Building_ChickenFeeder.BP_Building_ChickenFeeder_C|GetHasFood _asbp_building_chicken_feeder)
      (return true _asbp_building_chicken_feeder (Transformation|GetActorLocation _asbp_building_chicken_feeder))))
  (return false 0 "0, 0, 0"))

(fn ChickenStartFindFoodTimer
  (params (ControlledPawn :type Pawn%20Object%20Reference))
  ;[1 1 1] Start find food timer.
  (bind _asbp_character_hen (Utilities|Casting|CastToBP_Character_Hen ControlledPawn)
    (:then
      (Default|StartFindFoodTimer _asbp_character_hen))
    (:CastFailed
      (bind _asbp_character_rooster (Utilities|Casting|CastToBP_Character_Rooster ControlledPawn)
        (:then
          (Default|StartFindFoodTimer _asbp_character_rooster))
        (:CastFailed
          (bind _asbp_character_chick (Utilities|Casting|CastToBP_Character_Chick ControlledPawn)
            (:then
              (Default|StartFindFoodTimer _asbp_character_chick))
            (:CastFailed
              (return false)))))))
  (return true))

(fn ChickenTryEat
  (params (ControlledPawn :type Pawn%20Object%20Reference) (TargetActor :type Actor%20Object%20Reference))
  ;[1 1 1] Try to eat.
  (bind _asbp_character_hen (Utilities|Casting|CastToBP_Character_Hen ControlledPawn)
    (:then
      (Default|TryEat _asbp_character_hen)
      (Default|StartFindFoodTimer _asbp_character_hen)
      (bind _asbp_building_chicken_feeder (Utilities|Casting|CastToBP_Building_ChickenFeeder TargetActor :!label _label)
        (:then
          _)
        (:CastFailed
          (return false))))
    (:CastFailed
      (bind _asbp_character_rooster (Utilities|Casting|CastToBP_Character_Rooster ControlledPawn)
        (:then
          (Default|TryEat _asbp_character_rooster)
          (Default|StartFindFoodTimer _asbp_character_rooster)
          (goto _label))
        (:CastFailed
          (bind _asbp_character_chick (Utilities|Casting|CastToBP_Character_Chick ControlledPawn)
            (:then
              (Default|TryEat _asbp_character_chick)
              (Default|StartFindFoodTimer _asbp_character_chick)
              (goto _label))
            (:CastFailed
              (return false)))))))
  (Default|ConsumeFood _asbp_building_chicken_feeder)
  (return true))