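; Behavior Tree task that sends a Pig, Swine or Piglet to a nearby mud pile to play its mud animation.
; It starts the animal's find-mud timer, then sphere-traces WorldDynamic objects around the pawn for a mud pile.
; AIMoveTo leads to the animation on arrival; the task still succeeds if movement fails.
; It fails only when the pawn is another type or no pile is found.
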(event EventReceiveExecuteAI
  (params (OwnerController :type AI%20Controller%20Object%20Reference) (ControlledPawn :type Pawn%20Object%20Reference))
  ;[1 1 1] Move to available feeder and play eat animation.
  (bind _success (CallFunction|PigStartFindMudTimer ControlledPawn))
  (if _success
    (bind (_found _targetactor _targetlocation) (CallFunction|TrytoFindMud ControlledPawn))
    (if _found
      (AI|AIMoveTo ControlledPawn _targetlocation 0 1e+02 true
        (:OnSuccess
          (CallFunction|PigTryPlayMudAnimation ControlledPawn _targetactor))
        (:OnFail
          _))
      (AI|BehaviorTree|FinishExecute true)
      (else
        (AI|BehaviorTree|FinishExecute false :!label _label)))
    (else
      (goto _label))))

(fn TrytoFindMud
  (params (ControlledPawn :type Pawn%20Object%20Reference))
  (bind _returnvalue (Transformation|GetActorLocation ControlledPawn))
  ;[1 1 1] Try to find mud pile.
  (bind _outhits (Collision|MultiSphereTraceForObjects _returnvalue _returnvalue 5e+02 (Utilities|Array|MakeArray "ObjectTypeQuery2") false 0 "None"))
  (for _array_element _outhits
    (bind _asbp_building_mud_pile (Utilities|Casting|CastToBP_Building_MudPile (.HitActor (Collision|BreakHitResult _array_element))))
    (return true _asbp_building_mud_pile (+ (Transformation|GetActorLocation _asbp_building_mud_pile) "0, 0,50.000000")))
  (return false 0 "0, 0, 0"))

(fn PigStartFindMudTimer
  (params (ControlledPawn :type Pawn%20Object%20Reference))
  ;[1 1 1] Start find mud timer.
  (bind _asbp_character_pig (Utilities|Casting|CastToBP_Character_Pig ControlledPawn)
    (:then
      (Default|StartFindMudTimer _asbp_character_pig))
    (:CastFailed
      (bind _asbp_character_swine (Utilities|Casting|CastToBP_Character_Swine ControlledPawn)
        (:then
          (Default|StartFindMudTimer _asbp_character_swine))
        (:CastFailed
          (bind _asbp_character_piglet (Utilities|Casting|CastToBP_Character_Piglet ControlledPawn)
            (:then
              (Default|StartFindMudTimer _asbp_character_piglet))
            (:CastFailed
              (return false)))))))
  (return true))

(fn PigTryPlayMudAnimation
  (params (ControlledPawn :type Pawn%20Object%20Reference) (TargetActor :type Actor%20Object%20Reference))
  ;[1 1 1] Try to play mud animation.
  (bind _asbp_character_pig (Utilities|Casting|CastToBP_Character_Pig ControlledPawn)
    (:then
      (Default|TryPlayMudAnimation _asbp_character_pig))
    (:CastFailed
      (bind _asbp_character_swine (Utilities|Casting|CastToBP_Character_Swine ControlledPawn)
        (:then
          (Default|TryPlayMudAnimation _asbp_character_swine))
        (:CastFailed
          (bind _asbp_character_piglet (Utilities|Casting|CastToBP_Character_Piglet ControlledPawn)
            (:then
              (Default|TryPlayMudAnimation _asbp_character_piglet))
            (:CastFailed
              (return false)))))))
  (return true))