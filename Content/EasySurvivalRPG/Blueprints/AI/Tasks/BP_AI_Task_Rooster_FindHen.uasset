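; Behavior tree task that sends a rooster to a nearby hen to start her egg production.
; It restarts the rooster's find-hen timer, then sphere-traces surrounding pawns for a hen without a spawn egg timer.
; The rooster moves to that hen and, on arrival, starts her egg timer and restarts its own.
; The task succeeds even if the move fails, and fails only without a valid rooster or hen.
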(event EventReceiveExecuteAI
  (params (OwnerController :type AI%20Controller%20Object%20Reference) (ControlledPawn :type Pawn%20Object%20Reference))
  ;[1 1 1] Move to available hen and start egg progress timer.
  (bind _asbp_character_rooster (Utilities|Casting|CastToBP_Character_Rooster ControlledPawn)
    (:then
      (Default|StartFindHenTimer _asbp_character_rooster)
      (bind (_found _targethen) (CallFunction|TrytoFindHen _asbp_character_rooster))
      (if _found
        (AI|AIMoveTo _asbp_character_rooster "0, 0, 0" _targethen 75.0 true
          (:OnSuccess
            (Default|StartSpawnEggTimer _targethen 0.0)
            (Default|StartFindHenTimer _asbp_character_rooster))
          (:OnFail
            _))
        (AI|BehaviorTree|FinishExecute true)
        (else
          (AI|BehaviorTree|FinishExecute false :!label _label))))
    (:CastFailed
      (goto _label))))

(fn TrytoFindHen
  (params (ControlledPawn :type Pawn%20Object%20Reference))
  (bind _returnvalue (Transformation|GetActorLocation ControlledPawn))
  ;[1 1 1] Try to find available hen that does not have spawn egg timer.
  (bind _outhits (Collision|MultiSphereTraceForObjects _returnvalue _returnvalue 5e+02 (Utilities|Array|MakeArray "ObjectTypeQuery3") false 0 "None"))
  (for _array_element _outhits
    (bind _asbp_character_hen (Utilities|Casting|CastToBP_Character_Hen (.HitActor (Collision|BreakHitResult _array_element))))
    (if (not (Utilities|Time|IsValidTimerHandle (Variables|/Game/EasySurvivalRPG/Blueprints/Characters/Base/BP_Character_Hen.BP_Character_Hen_C|GetSpawnEggTimer _asbp_character_hen)))
      (return true _asbp_character_hen)))
  (return false 0))