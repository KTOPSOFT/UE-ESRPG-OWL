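; Fishing rod launch ability that spawns a floater projectile and hands it to the instigator's equipped fishing rod.
; The spawn point is the weapon socket, or a point above the actor when the socket location is zero.
; The floater is aimed along the instigator's forward rotation; a camera-focus trace aiming branch exists but is disconnected.
; Both Player and PlayerMerged characters are supported when calling InitFloater on the rod.
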(fn ConstructionScript
  (|CallParentFunction))

(fn SpawnProjectile
  (bind _returnvalue (Game|GetInstigator))
  (bind _returnvalue_2 (Game|GetInstigator))
  ;[1 1 1] Spawn and launch floater actor.
  (Utilities|IsValid _returnvalue_2
    (:Is%20Valid
      (bind _sockettransform (Class|BPICharacter|GetWeaponSocketTransformBPI(Message) _returnvalue_2 (Variables|Default|GetWeaponStartSocketName)))
      (bind _output_get (LocalVariables|SetLocalStartLocation (select (Math|Vector|Equal(Vector) (.Location (Math|Transform|BreakTransform _sockettransform)) "0, 0, 0" 0.0001) (+ (Transformation|GetActorLocation _returnvalue_2) "0, 0,100.000000") (.Location (Math|Transform|BreakTransform _sockettransform)))))
      (LocalVariables|SetLocalRotation (Math|Rotator|FindLookatRotation (LocalVariables|GetLocalStartLocation) (+ _output_get (* (Math|Vector|GetForwardVector (Transformation|GetActorRotation (Game|GetInstigator))) 1e+04))))
      (bind _returnvalue_3 (Game|SpawnActorfromClass (Variables|Default|GetProjectileClass) (Math|Transform|MakeTransform (LocalVariables|GetLocalStartLocation) (LocalVariables|GetLocalRotation) (Variables|Default|GetProjectileScale)) "Undefined" 0 (Utilities|Struct|BreakSTR_AbilityInstance (Variables|Default|GetAbilitySettings)) _returnvalue))
      (bind _asbp_character_player (Utilities|Casting|CastToBP_Character_Player _returnvalue)
        (:then
          (bind _asbp_usable_item_fishing_rod (Utilities|Casting|CastToBP_UsableItem_FishingRod (Variables|/Game/EasySurvivalRPG/Blueprints/Characters/Base/BP_Character_Player.BP_Character_Player_C|GetUsableItemActor _asbp_character_player)))
          (Default|InitFloater _asbp_usable_item_fishing_rod _returnvalue_3))
        (:CastFailed
          (bind _asbp_character_player_merged (Utilities|Casting|CastToBP_Character_PlayerMerged _returnvalue))
          (bind _asbp_usable_item_fishing_rod_2 (Utilities|Casting|CastToBP_UsableItem_FishingRod (Variables|/Game/EasySurvivalRPG/ESRPG_Integration/BP_Character_PlayerMerged.BP_Character_PlayerMerged_C|GetUsableItemActor _asbp_character_player_merged)))
          (Default|InitFloater _asbp_usable_item_fishing_rod_2 _returnvalue_3))))
    (:Is%20Not%20Valid
      (return false))))