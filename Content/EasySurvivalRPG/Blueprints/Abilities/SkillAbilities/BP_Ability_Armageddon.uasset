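; Skill ability that calls down an Armageddon meteor shower around the instigator while darkening the scene.
; On use, it caches a directional light and a sky light, then a timeline lerps their intensity, plus the sun's color, toward target values.
; A looping timer launches randomly offset, angled and scaled projectiles from high above, passing ability attributes to each.
; The actor destroys itself once the meteor count runs out, with no light restoration here.
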(event Custom|ToDarkness
  (bind _skylightcomponent (Variables|State|GetSkyLightComponent))
  (bind _sunlightcomponent (Variables|State|GetSunLightComponent))
  ;[1 1 1] Update intensity of light components.
  (bind _alpha (Timeline|DarknessTimeline Play)
    (:Update
      (Utilities|FlowControl|Sequence
        (:then_0
          (Utilities|IsValid _sunlightcomponent
            (:Is%20Valid
              (Rendering|Components|Light|SetIntensity _sunlightcomponent (Math|Float|Lerp (Variables|State|GetInitialSunLightIntensity) (Variables|Settings|GetTargetSunLightIntensity) _alpha))
              (Rendering|Components|Light|SetLightColor _sunlightcomponent (Math|Color|Lerp(LinearColor) (Variables|State|GetInitialSunLightColor) (Variables|Settings|GetTargetSunLightColor) _alpha) true))))
        (:then_1
          (Utilities|IsValid _skylightcomponent
            (:Is%20Valid
              (Rendering|Components|Light|SetIntensity _skylightcomponent (Math|Float|Lerp (Variables|State|GetInitialSkyLightIntensity) (Variables|Settings|GetTargetSkyLightIntensity) _alpha)))))))))

(event EventUse
  ;[1 1 1] Start armageddon on use.
  (CallFunction|StartArmageddon))

(fn ConstructionScript
  (|CallParentFunction))

(fn StartArmageddon
  (bind _returnvalue (Game|GetInstigator))
  (bind _returnvalue_2 (Transformation|GetActorLocation _returnvalue))
  ;[1 1 1] Start darkness timeline and start spawn timer for meteors spawning.
  (CallFunction|StartDarkness)
  (bind _output_get (LocalVariables|SetLocalSpawnLocation (+ _returnvalue_2 "0, 0,10000.000000")))
  (Variables|State|SetSpawnLocation _output_get)
  (Variables|State|SetSpawnRotation (Math|Rotator|FindLookatRotation (LocalVariables|GetLocalSpawnLocation) _returnvalue_2))
  (Variables|State|SetCountRemaining (Variables|Settings|GetMeteorsCount))
  (Utilities|Time|SetTimerbyEvent (EventDispatchers|CreateEvent :!event SpawnMeteor) 0.075 true)
  (return true))

(fn SpawnMeteor
  ;[1 1 1] Spawn meteor from the sky.
  (if (> (Variables|State|GetCountRemaining) 0)
    (Variables|State|SetCountRemaining (- (Variables|State|GetCountRemaining) 1))
    (LocalVariables|SetLocalRandomScale (Math|Random|RandomFloatinRange 1.0 2.0))
    (CallFunction|LaunchProjectile (Variables|Settings|GetProjectileClass) (+ (Variables|State|GetSpawnLocation) (Math|Vector|MakeVector (Math|Random|RandomFloatinRange -1e+04 1e+04) (Math|Random|RandomFloatinRange -1e+04 1e+04) 0.0)) (Math|Rotator|CombineRotators (Variables|State|GetSpawnRotation) (Math|Rotator|MakeRotator 0.0 (Math|Random|RandomFloatinRange -15.0 15.0) (Math|Random|RandomFloatinRange -15.0 15.0))) (Math|Vector|MakeVector (LocalVariables|GetLocalRandomScale) (LocalVariables|GetLocalRandomScale) (LocalVariables|GetLocalRandomScale)))
    (else
      (Actor|DestroyActor))))

(fn LaunchProjectile
  (params (ProjectileClass :type BP%20Projectile%20Base%20Class%20Reference) (SpawnLocation :type Vector) (Rotation :type Rotator) (Scale :type Vector))
  ;[1 1 1] Launch projectile with specific attributes.
  (bind _returnvalue (Game|SpawnActorfromClass ProjectileClass (Math|Transform|MakeTransform SpawnLocation Rotation Scale) "AlwaysSpawn" 0 (Utilities|Struct|BreakSTR_AbilityInstance (Variables|Default|GetAbilitySettings)) (Game|GetInstigator)))
  (if (Variables|Settings|GetUseInstigatorAttributes)
    (Default|UpdateProjectileAttributes _returnvalue))
  (return true))

(fn StartDarkness
  ;[1 1 1] Set sun light and sky light components and start darkness timeline.
  (Utilities|FlowControl|Sequence
    (:then_0
      (bind _outactors (Actor|GetAllActorsOfClass "/Script/Engine.DirectionalLight"))
      (for _array_element _outactors
        (bind _output_get (Variables|State|SetSunLightComponent (Variables|/Script/Engine.Light|GetLightComponent _array_element)))
        (Variables|State|SetInitialSunLightIntensity (Variables|/Script/Engine.LightComponentBase|GetIntensity _output_get))
        (Variables|State|SetInitialSunLightColor (Rendering|Components|Light|GetLightColor _output_get))))
    (:then_1
      (bind _outactors_2 (Actor|GetAllActorsOfClass "/Script/Engine.SkyLight"))
      (for _array_element_2 _outactors_2
        (Variables|State|SetSkyLightComponent (Variables|/Script/Engine.SkyLight|GetLightComponent _array_element_2))
        (Variables|State|SetInitialSkyLightIntensity (Variables|/Script/Engine.LightComponentBase|GetIntensity (Variables|/Script/Engine.SkyLight|GetLightComponent _array_element_2))))
      (CallFunction|ToDarkness))))