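; BP_EffectZone_Capsule is a capsule-shaped effect zone that tracks the characters inside it.
; Its construction script runs the parent's, then sizes the collision capsule from the radius and half-height variables.
; Begin and end overlap events cast the other actor to Character and add or remove it as an overlapping character.
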(event OnComponentBeginOverlap(CapsuleCollision)
  (params (OverlappedComponent :type Primitive%20Component%20Object%20Reference) (OtherActor :type Actor%20Object%20Reference) (OtherComp :type Primitive%20Component%20Object%20Reference) (OtherBodyIndex :type Integer) (bFromSweep :type Boolean) (SweepResult :type Hit%20Result%20Structure%20%28by%20ref%29))
  ;[1 1 1] Overlap events.
  (bind _ascharacter (Utilities|Casting|CastToCharacter OtherActor))
  (CallFunction|AddOverlappingCharacter _ascharacter))

(event OnComponentEndOverlap(CapsuleCollision)
  (params (OverlappedComponent :type Primitive%20Component%20Object%20Reference) (OtherActor :type Actor%20Object%20Reference) (OtherComp :type Primitive%20Component%20Object%20Reference) (OtherBodyIndex :type Integer))
  ;[1 1 1] Overlap events.
  (bind _ascharacter (Utilities|Casting|CastToCharacter OtherActor))
  (CallFunction|RemoveOverlappingCharacter _ascharacter))

(fn ConstructionScript
  (bind _capsulecollision (Variables|Default|GetCapsuleCollision))
  ;[1 1 1] Set collision variables.
  (|CallParentFunction)
  (Components|Capsule|SetCapsuleRadius _capsulecollision (Variables|Settings|GetCapsuleRadius) true)
  (Components|Capsule|SetCapsuleHalfHeight _capsulecollision (Variables|Settings|GetCapsuleHalfHeight) true))