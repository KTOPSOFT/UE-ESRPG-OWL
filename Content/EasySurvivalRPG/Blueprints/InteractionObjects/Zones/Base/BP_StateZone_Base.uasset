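; Base zone actor that changes health, energy, mana, hunger, thirst and oxygen of characters registered as overlapping.
; Adding a character, optionally players only, applies one-time overlap changes if the zone is active, while tick applies per-second rates.
; Changes reach characters as flat and percent interface messages.
; It runs on authority only, destroying itself on remotes; activation toggles interval-based ticking, and construction flags whether any rate is nonzero.
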(event EventTick
  (params (DeltaSeconds :type Float%20%28single-precision%29))
  ;[1 1 1] Event tick. Change characters state by tick if activated.
  (if (and (Variables|State|GetIsActivated) (Variables|State|GetUpdateStatesByTick))
    (for _array_element (Variables|State|GetOverlappingCharacters)
      (CallFunction|ChangeStatesbyTick _array_element DeltaSeconds))))

(event EventBeginPlay
  ;[1 1 1] Begin play. Set activated state.
  (Networking|SwitchHasAuthority
    (:Authority
      (CallFunction|SetActivatedState (Variables|Settings|GetInitiallyActivated)))
    (:Remote
      (Actor|DestroyActor))))

(fn ConstructionScript
  ;[1 1 1] Set tick variables variables.
  (Variables|State|SetUpdateStatesByTick (Math|Boolean|ORBoolean (!= (Variables|Settings|Health|GetHealthPerSecond) 0.0) (!= (Variables|Settings|Health|GetHealth%25PerSecond) 0.0) (!= (Variables|Settings|Energy|GetEnergyPerSecond) 0.0) (!= (Variables|Settings|Energy|GetEnergy%25PerSecond) 0.0) (!= (Variables|Settings|Hunger|GetHungerPerSecond) 0.0) (!= (Variables|Settings|Hunger|GetHunger%25PerSecond) 0.0) (!= (Variables|Settings|Thirst|GetThirstPerSecond) 0.0) (!= (Variables|Settings|Thirst|GetThirst%25PerSecond) 0.0) (!= (Variables|Settings|Oxygen|GetOxygenPerSecond) 0.0) (!= (Variables|Settings|Oxygen|GetOxygen%25PerSecond) 0.0) (!= (Variables|Settings|Mana|GetManaPerSecond) 0.0) (!= (Variables|Settings|Mana|GetMana%25PerSecond) 0.0)))
  (Actor|Tick|SetActorTickInterval (Variables|Settings|GetTickInterval)))

(fn AddOverlappingCharacter
  (params (Character :type Character%20Object%20Reference))
  ;[1 1 1] Add character to the overlapping characters array and change state.
  (if (Variables|Settings|GetOnlyPlayerCharacters)
    (Utilities|Casting|CastToPlayerController (Pawn|GetController Character)))
  (Utilities|Array|AddUnique (Variables|State|GetOverlappingCharacters) Character)
  (CallFunction|ChangeStatesbyOverlap Character)
  (return true))

(fn RemoveOverlappingCharacter
  (params (Character :type Character%20Object%20Reference))
  ;[1 1 1] Remove character from overlapping characters array.
  (Utilities|Array|RemoveItem (Variables|State|GetOverlappingCharacters) Character)
  (return true))

(fn ChangeStatesbyOverlap
  (params (Character :type Character%20Object%20Reference))
  ;[1 1 1] Change character states depending on overlap variables.
  (LocalVariables|SetLocalCharacter Character)
  (if (Variables|State|GetIsActivated)
    (CallFunction|ChangeCharacterHealth (LocalVariables|GetLocalCharacter) (Variables|Settings|Health|GetHealthByOverlap) (Variables|Settings|Health|GetHealth%25ByOverlap))
    (CallFunction|ChangeCharacterEnergy (LocalVariables|GetLocalCharacter) (Variables|Settings|Energy|GetEnergyByOverlap) (Variables|Settings|Energy|GetEnergy%25ByOverlap))
    (CallFunction|ChangeCharacterMana (LocalVariables|GetLocalCharacter) (Variables|Settings|Mana|GetManaByOverlap) (Variables|Settings|Mana|GetMana%25ByOverlap))
    (CallFunction|ChangeCharacterHunger (LocalVariables|GetLocalCharacter) (Variables|Settings|Hunger|GetHungerByOverlap) (Variables|Settings|Hunger|GetHunger%25ByOverlap))
    (CallFunction|ChangeCharacterThirst (LocalVariables|GetLocalCharacter) (Variables|Settings|Thirst|GetThirstByOverlap) (Variables|Settings|Thirst|GetThirst%25ByOverlap))
    (CallFunction|ChangeCharacterOxygen (LocalVariables|GetLocalCharacter) (Variables|Settings|Oxygen|GetOxygenByOverlap) (Variables|Settings|Oxygen|GetOxygen%25ByOverlap))
    (return true)))

(fn ChangeStatesbyTick
  (params (Character :type Character%20Object%20Reference) (DeltaSeconds :type Float%20%28single-precision%29))
  ;[1 1 1] Change character state by event tick.
  (LocalVariables|SetLocalCharacter Character)
  (LocalVariables|SetLocalDeltaSeconds DeltaSeconds)
  (CallFunction|ChangeCharacterHealth (LocalVariables|GetLocalCharacter) (* (Variables|Settings|Health|GetHealthPerSecond) (LocalVariables|GetLocalDeltaSeconds)) (* (Variables|Settings|Health|GetHealth%25PerSecond) (LocalVariables|GetLocalDeltaSeconds)))
  (CallFunction|ChangeCharacterEnergy (LocalVariables|GetLocalCharacter) (* (Variables|Settings|Energy|GetEnergyPerSecond) (LocalVariables|GetLocalDeltaSeconds)) (* (Variables|Settings|Energy|GetEnergy%25PerSecond) (LocalVariables|GetLocalDeltaSeconds)))
  (CallFunction|ChangeCharacterMana (LocalVariables|GetLocalCharacter) (* (Variables|Settings|Mana|GetManaPerSecond) (LocalVariables|GetLocalDeltaSeconds)) (* (Variables|Settings|Mana|GetMana%25PerSecond) (LocalVariables|GetLocalDeltaSeconds)))
  (CallFunction|ChangeCharacterHunger (LocalVariables|GetLocalCharacter) (* (Variables|Settings|Hunger|GetHungerPerSecond) (LocalVariables|GetLocalDeltaSeconds)) (* (Variables|Settings|Hunger|GetHunger%25PerSecond) (LocalVariables|GetLocalDeltaSeconds)))
  (CallFunction|ChangeCharacterThirst (LocalVariables|GetLocalCharacter) (* (Variables|Settings|Thirst|GetThirstPerSecond) (LocalVariables|GetLocalDeltaSeconds)) (* (Variables|Settings|Thirst|GetThirst%25PerSecond) (LocalVariables|GetLocalDeltaSeconds)))
  (CallFunction|ChangeCharacterOxygen (LocalVariables|GetLocalCharacter) (* (Variables|Settings|Oxygen|GetOxygenPerSecond) (LocalVariables|GetLocalDeltaSeconds)) (* (Variables|Settings|Oxygen|GetOxygen%25PerSecond) (LocalVariables|GetLocalDeltaSeconds)))
  (return true))

(fn ChangeCharacterHealth
  (params (Character :type Character%20Object%20Reference) (Health :type Float%20%28single-precision%29) (Health%25 :type Float%20%28single-precision%29))
  ;[1 1 1] Check and change character health state.
  (Utilities|FlowControl|Sequence
    (:then_0
      (if (!= Health 0.0)
        (Class|BPICharacter|ChangeHealthBPI(Message) Character Health false)))
    (:then_1
      (if (!= Health%25 0.0)
        (Class|BPICharacter|ChangeHealthBPI(Message) Character Health%25 true)))
    (:then_2
      (return true))))

(fn ChangeCharacterEnergy
  (params (Character :type Character%20Object%20Reference) (Energy :type Float%20%28single-precision%29) (Energy%25 :type Float%20%28single-precision%29))
  ;[1 1 1] Check and change character energy state.
  (Utilities|FlowControl|Sequence
    (:then_0
      (if (!= Energy 0.0)
        (Class|BPICharacter|ChangeEnergyBPI(Message) Character Energy false)))
    (:then_1
      (if (!= Energy%25 0.0)
        (Class|BPICharacter|ChangeEnergyBPI(Message) Character Energy%25 true)))
    (:then_2
      (return true))))

(fn ChangeCharacterHunger
  (params (Character :type Character%20Object%20Reference) (Hunger :type Float%20%28single-precision%29) (Hunger%25 :type Float%20%28single-precision%29))
  ;[1 1 1] Check and change character hunger state.
  (Utilities|FlowControl|Sequence
    (:then_0
      (if (!= Hunger 0.0)
        (Class|BPIPlayerCharacter|ChangeHungerBPI(Message) Character Hunger false)))
    (:then_1
      (if (!= Hunger%25 0.0)
        (Class|BPIPlayerCharacter|ChangeHungerBPI(Message) Character Hunger%25 true)))
    (:then_2
      (return true))))

(fn ChangeCharacterThirst
  (params (Character :type Character%20Object%20Reference) (Thirst :type Float%20%28single-precision%29) (Thirst%25 :type Float%20%28single-precision%29))
  ;[1 1 1] Check and change character thirst state.
  (Utilities|FlowControl|Sequence
    (:then_0
      (if (!= Thirst 0.0)
        (Class|BPIPlayerCharacter|ChangeThirstBPI(Message) Character Thirst false)))
    (:then_1
      (if (!= Thirst%25 0.0)
        (Class|BPIPlayerCharacter|ChangeThirstBPI(Message) Character Thirst%25 true)))
    (:then_2
      (return true))))

(fn ChangeCharacterOxygen
  (params (Character :type Character%20Object%20Reference) (Oxygen :type Float%20%28single-precision%29) (Oxygen%25 :type Float%20%28single-precision%29))
  ;[1 1 1] Check and change character oxygen state.
  (Utilities|FlowControl|Sequence
    (:then_0
      (if (!= Oxygen 0.0)
        (Class|BPIPlayerCharacter|ChangeOxygenBPI(Message) Character Oxygen false)))
    (:then_1
      (if (!= Oxygen%25 0.0)
        (Class|BPIPlayerCharacter|ChangeOxygenBPI(Message) Character Oxygen%25 true)))
    (:then_2
      (return true))))

(fn ChangeCharacterMana
  (params (Character :type Character%20Object%20Reference) (Mana :type Float%20%28single-precision%29) (Mana%25 :type Float%20%28single-precision%29))
  ;[1 1 1] Check and change character mana state.
  (Utilities|FlowControl|Sequence
    (:then_0
      (if (!= Mana 0.0)
        (Class|BPICharacter|ChangeManaBPI(Message) Character Mana false)))
    (:then_1
      (if (!= Mana%25 0.0)
        (Class|BPICharacter|ChangeManaBPI(Message) Character Mana%25 true)))
    (:then_2
      (return true))))

(fn SetActivatedState
  (params (NewActivatedState :type Boolean))
  ;[1 1 1] Set activated state.
  (bind _output_get (Variables|State|SetIsActivated NewActivatedState))
  (Actor|Tick|SetActorTickEnabled _output_get)
  (return true))