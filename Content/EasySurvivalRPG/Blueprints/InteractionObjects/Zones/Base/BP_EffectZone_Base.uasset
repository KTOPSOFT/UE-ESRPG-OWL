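; Base effect zone actor that adds, removes or clears status effects on characters inside it, optionally limited to player-controlled ones.
; Add/RemoveOverlappingCharacter maintain the occupant list and trigger begin/end overlap effects; no overlap events are bound here.
; While activated, Tick processes occupants at a set interval, if construction found any tick effects configured.
; It runs only with authority, destroying itself on remotes at BeginPlay.
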(event EventTick
  (params (DeltaSeconds :type Float%20%28single-precision%29))
  ;[1 1 1] Event tick. Apply status effects characters by tick if activated.
  (if (and (Variables|State|GetIsActivated) (Variables|State|GetUpdateStatesByTick))
    (for _array_element (Variables|State|GetOverlappingCharacters)
      (CallFunction|CheckCharacterbyTick _array_element DeltaSeconds))))

(event EventBeginPlay
  ;[1 1 1] Begin play. Set activated state.
  (Networking|SwitchHasAuthority
    (:Authority
      (CallFunction|SetActivatedState (Variables|Settings|GetInitiallyActivated)))
    (:Remote
      (Actor|DestroyActor))))

(fn ConstructionScript
  ;[1 1 1] Set tick variables variables.
  (Variables|State|SetUpdateStatesByTick (Math|Boolean|ORBoolean (Variables|Settings|Tick|GetClearAllEffectsOnTick) (Utilities|Array|IsValidIndex (Variables|Settings|Tick|GetTickEffectsToAdd)) (Utilities|Array|IsValidIndex (Variables|Settings|Tick|GetTickEffectsToRemove)) (Utilities|Array|IsValidIndex (Variables|Settings|Tick|GetTickEffectsIDsToRemove))))
  (Actor|Tick|SetActorTickInterval (Variables|Settings|GetTickInterval)))

(fn AddOverlappingCharacter
  (params (Character :type Character%20Object%20Reference))
  ;[1 1 1] Add character to the overlapping characters array and do begin overlap actions.
  (if (Variables|Settings|GetOnlyPlayerCharacters)
    (Utilities|Casting|CastToPlayerController (Pawn|GetController Character)))
  (Utilities|Array|AddUnique (Variables|State|GetOverlappingCharacters) Character)
  (CallFunction|CheckCharacterbyOverlap Character false)
  (return true))

(fn RemoveOverlappingCharacter
  (params (Character :type Character%20Object%20Reference))
  ;[1 1 1] Remove character from overlapping characters array and do end overlap events.
  (if (Variables|Settings|GetOnlyPlayerCharacters)
    (Utilities|Casting|CastToPlayerController (Pawn|GetController Character)))
  (Utilities|Array|RemoveItem (Variables|State|GetOverlappingCharacters) Character)
  (CallFunction|CheckCharacterbyOverlap Character true)
  (return true))

(fn CheckCharacterbyOverlap
  (params (Character :type Character%20Object%20Reference) (EndOverlap :type Boolean))
  ;[1 1 1] Check and apply overlap actions to character.
  (LocalVariables|SetLocalCharacter Character)
  (if (Variables|State|GetIsActivated)
    (if (select EndOverlap (Variables|Settings|EndOverlap|GetClearAllEffectsOnEndOverlap) (Variables|Settings|BeginOverlap|GetClearAllEffectsOnOverlap))
      (CallFunction|ClearStatusEffectsfromActor (LocalVariables|GetLocalCharacter))
      (else
        (CallFunction|ApplyEffectstoCharacter (LocalVariables|GetLocalCharacter) (select EndOverlap (Variables|Settings|EndOverlap|GetEndOverlapEffectsToAdd) (Variables|Settings|BeginOverlap|GetOverlapEffectsToAdd)))
        (CallFunction|RemoveEffectsfromCharacter (LocalVariables|GetLocalCharacter) (select EndOverlap (Variables|Settings|EndOverlap|GetEndOverlapEffectsToRemove) (Variables|Settings|BeginOverlap|GetOverlapEffectsToRemove)))
        (CallFunction|RemoveEffectsIDsfromCharacter (LocalVariables|GetLocalCharacter) (select EndOverlap (Variables|Settings|EndOverlap|GetEndOverlapEffectsIDsToRemove) (Variables|Settings|BeginOverlap|GetOverlapEffectsIDsToRemove)))))
    (return true)))

(fn CheckCharacterbyTick
  (params (Character :type Character%20Object%20Reference) (DeltaSeconds :type Float%20%28single-precision%29))
  ;[1 1 1] Check and apply tick actions to character.
  (LocalVariables|SetLocalCharacter Character)
  (if (Variables|State|GetIsActivated)
    (if (Variables|Settings|Tick|GetClearAllEffectsOnTick)
      (CallFunction|ClearStatusEffectsfromActor (LocalVariables|GetLocalCharacter))
      (else
        (CallFunction|ApplyEffectstoCharacter (LocalVariables|GetLocalCharacter) (Variables|Settings|Tick|GetTickEffectsToAdd))
        (CallFunction|RemoveEffectsfromCharacter (LocalVariables|GetLocalCharacter) (Variables|Settings|Tick|GetTickEffectsToRemove))
        (CallFunction|RemoveEffectsIDsfromCharacter (LocalVariables|GetLocalCharacter) (Variables|Settings|Tick|GetTickEffectsIDsToRemove))))
    (return true)))

(fn ApplyEffectstoCharacter
  (params (Character :type Character%20Object%20Reference) (StatusEffectHandle :type Array%20of%20Data%20Table%20Row%20Handle%20Structures))
  ;[1 1 1] Apply status effects to character.
  (for _array_element StatusEffectHandle
    (CallFunction|ApplyStatusEffecttoActor Character _array_element Character))
  (return true))

(fn RemoveEffectsfromCharacter
  (params (Character :type Character%20Object%20Reference) (StatusEffectHandle :type Array%20of%20Data%20Table%20Row%20Handle%20Structures))
  ;[1 1 1] Remove status effects from character.
  (for _array_element StatusEffectHandle
    (CallFunction|RemoveStatusEffectfromActorbyHandle Character _array_element))
  (return true))

(fn RemoveEffectsIDsfromCharacter
  (params (Character :type Character%20Object%20Reference) (StatusEffectHandle :type Array%20of%20Names))
  ;[1 1 1] Remove status effects with IDs from character.
  (for _array_element StatusEffectHandle
    (CallFunction|RemoveStatusEffectfromActorbyID Character _array_element))
  (return true))

(fn SetActivatedState
  (params (NewActivatedState :type Boolean))
  ;[1 1 1] Set activated state.
  (bind _output_get (Variables|State|SetIsActivated NewActivatedState))
  (Actor|Tick|SetActorTickEnabled _output_get)
  (return true))