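; Base Blueprint for placeable spiked walls that deal melee damage to actors touching their spikes.
; Once built, it enables collision on components tagged DamageCollision.
; On the authority, top-spike overlaps deal immediate point damage with a multicast sound, track actors in parallel actor/location arrays, and run a looping timer while the list is occupied.
; CheckOverlappedActors re-damages only actors whose location has changed, so standing still avoids further damage.
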(event OnComponentBeginOverlap(TopDamageCollision)
  (params (OverlappedComponent :type Primitive%20Component%20Object%20Reference) (OtherActor :type Actor%20Object%20Reference) (OtherComp :type Primitive%20Component%20Object%20Reference) (OtherBodyIndex :type Integer) (bFromSweep :type Boolean) (SweepResult :type Hit%20Result%20Structure%20%28by%20ref%29))
  ;[1 1 1] Deal damage from top spikes.
  (SpikedWall|AddOverlappedActor OtherActor))

(event OnComponentEndOverlap(TopDamageCollision)
  (params (OverlappedComponent :type Primitive%20Component%20Object%20Reference) (OtherActor :type Actor%20Object%20Reference) (OtherComp :type Primitive%20Component%20Object%20Reference) (OtherBodyIndex :type Integer))
  ;[1 1 1] Deal damage from top spikes.
  (SpikedWall|RemoveOverlappedActor OtherActor))

(event EventBeginPlay
  ;[1 1 1] Begin play. Disable damage collisions in build mode.
  (|CallParentFunction)
  (if (Variables|Default|GetBuilt)
    (SpikedWall|EnableDamageCollisions)))

(fn ConstructionScript
  (|CallParentFunction))

(fn AddOverlappedActor
  (params (Actor :type Actor%20Object%20Reference))
  ;[1 1 1] Start deal damage to overlapped actor.
  (Networking|SwitchHasAuthority
    (:Authority
      (if (not (Utilities|Array|ContainsItem (Variables|State|SpikedWall|GetOverlappedActors) Actor))
        (Utilities|Array|Add (Variables|State|SpikedWall|GetOverlappedActorsLocations) (Transformation|GetActorLocation))
        (Utilities|Array|Add (Variables|State|SpikedWall|GetOverlappedActors) Actor)
        (SpikedWall|DealSpikedDamage Actor)
        (if (not (Utilities|Time|IsValidTimerHandle (Variables|State|SpikedWall|GetDealDamageTimer)))
          (SpikedWall|StartDealDamageTimer))))))

(fn RemoveOverlappedActor
  (params (Actor :type Actor%20Object%20Reference))
  (bind _overlappedactors (Variables|State|SpikedWall|GetOverlappedActors))
  (bind _returnvalue (Utilities|Array|FindItem _overlappedactors Actor))
  ;[1 1 1] Stop deal damage to overlapped actor.
  (Networking|SwitchHasAuthority
    (:Authority
      (if (Utilities|Array|ContainsItem _overlappedactors Actor)
        (Utilities|Array|RemoveIndex _overlappedactors _returnvalue)
        (Utilities|Array|RemoveIndex (Variables|State|SpikedWall|GetOverlappedActorsLocations) _returnvalue)
        (if (not (Utilities|Array|IsValidIndex (Variables|State|SpikedWall|GetOverlappedActors)))
          (SpikedWall|StopDealDamageTimer))))))

(fn StartDealDamageTimer
  ;[1 1 1] Start deal damage timer.
  (bind _returnvalue (Utilities|Time|SetTimerbyEvent (EventDispatchers|CreateEvent :!event CheckOverlappedActors) (Variables|Settings|SpikedWall|GetDealDamageTimerTickTime) true))
  (Variables|State|SpikedWall|SetDealDamageTimer _returnvalue))

(fn StopDealDamageTimer
  ;[1 1 1] Stop deal damage timer.
  (Utilities|Time|ClearandInvalidateTimerbyHandle (Variables|State|SpikedWall|GetDealDamageTimer)))

(fn DealSpikedDamage
  (params (TargetActor :type Actor%20Object%20Reference))
  ;[1 1 1] Deal spiked damage to target actor.
  (bind _resultdamage (Default|CalculatePossibleDamage (Variables|Default|GetDamageSystemComponent) (Variables|Settings|SpikedWall|GetDamagePerTick) "/Game/EasySurvivalRPG/Blueprints/Misc/DamageTypes/BP_DamageType_Melee.BP_DamageType_Melee_C"))
  (Class|BPIDamageSystemActor|ApplyPointDamageBPI(Message) :self TargetActor :DamageData (Utilities|Struct|MakeSTR_DamageData _resultdamage "/Game/EasySurvivalRPG/Blueprints/Misc/DamageTypes/BP_DamageType_Melee.BP_DamageType_Melee_C" false false false false) :HitFromDirection (Transformation|GetActorLocation) :DamageCauser self)
  (CallFunction|PlaySoundatLocation(Multicast) (Variables|Settings|SpikedWall|GetSpikedDamageSound) (Transformation|GetActorLocation TargetActor)))

(fn CheckOverlappedActors
  (bind _overlappedactorslocations (Variables|State|SpikedWall|GetOverlappedActorsLocations))
  ;[1 1 1] Check each actor from overlapped actors and deal damage to actor if the location of the actor is changed.
  (for (_array_element _array_index) (Variables|State|SpikedWall|GetOverlappedActors)
    (if (Math|Vector|NotEqual(Vector) (Transformation|GetActorLocation _array_element) (Utilities|Array|Get(acopy) _overlappedactorslocations _array_index) 0.0001)
      (Utilities|Array|SetArrayElem _overlappedactorslocations _array_index (Transformation|GetActorLocation _array_element))
      (SpikedWall|DealSpikedDamage _array_element))))

(fn EnableDamageCollisions
  ;[1 1 1] Disable damage collisions.
  (for _array_element (Actor|GetComponentsbyTag "/Script/Engine.PrimitiveComponent" "DamageCollision")
    (Collision|SetCollisionEnabled _array_element "QueryOnly")))