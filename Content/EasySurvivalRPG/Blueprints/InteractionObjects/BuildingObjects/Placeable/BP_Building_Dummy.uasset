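; Placeable training dummy building object that plays a hit reaction animation when damaged.
; On begin play and mesh updates, the Built flag swaps visibility: static mesh while unbuilt, animated skeletal mesh once built.
; Damage events trigger a multicast hit animation on the skeletal mesh if the dummy can be damaged and still has durability.
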(event Custom|UpdateBuildedMeshes
  (bind _built (Variables|Default|GetBuilt))
  ;[1 1 1] Begin play. Update meshes.
  (Development|SetHiddeninGame (Variables|Default|GetStaticMesh) _built true)
  (Development|SetHiddeninGame (Variables|Default|GetSkeletalMesh) (not _built) true))

(event Custom|PlayHit%20%28Multicast%29
  ;[1 1 1] Interactions when takes damage.
  (Components|Animation|PlayAnimation (Variables|Default|GetSkeletalMesh) "/Game/EasySurvivalRPG/Meshes/SKMeshes/A_Dummy_Hit.A_Dummy_Hit" false))

(event Custom|DamageTaken?
  (params (DamageData :type STR%20Damage%20Data%20Structure%20%28by%20ref%29) (InstigatedBy :type Controller%20Object%20Reference) (DamageCauser :type Actor%20Object%20Reference) (HitInfo :type Hit%20Result%20Structure))
  ;[1 1 1] Interactions when takes damage.
  (if (and (Variables|Default|GetbCanBeDamaged) (> (Variables|Default|GetDurability) 0.0))
    (CallFunction|PlayHit(Multicast))))

(event EventBeginPlay
  ;[1 1 1] Begin play. Update meshes.
  (|CallParentFunction)
  (CallFunction|UpdateBuildedMeshes))

(fn ConstructionScript
  (|CallParentFunction))