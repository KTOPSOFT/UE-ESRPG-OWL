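; Buildable pig coop that players open or close, where a pig and a swine mate to start the pig's breeding timer.
; Entering animals are destroyed with their health stored, then respawned on release; a lone animal is kicked out after a delay.
; A looping timer drives mating, with RepNotify updates to the animation and camera-facing progress widget.
; Closing or EndPlay ejects occupants, and coop state persists through the save system.
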(event Custom|UpdateBuildedMeshes
  (bind _built (Variables|Default|GetBuilt))
  ;[1 1 1] Begin play.
  (Development|SetHiddeninGame (Variables|Default|GetStaticMesh) _built true)
  (Development|SetHiddeninGame (Variables|Default|GetSkeletalMesh) (not _built) true))

(event EventTryInteractBPI
  (params (Release :type Boolean) (PlayerController :type Player%20Controller%20Object%20Reference))
  ;[1 1 1] Interactions.
  (if Release
    (if (Variables|State|PigCoop|GetCoopIsOpened)
      (Variables|State|PigCoop|SetCoopIsOpened false)
      (PigCoop|KickPigsfromCoop)
      (else
        (Variables|State|PigCoop|SetCoopIsOpened true)))))

(event EventEndPlay
  (params (EndPlayReason :type EEndPlayReason%20Enum :default "Destroyed"))
  ;[1 1 1] Kick pigs on end play.
  (|CallParentFunction EndPlayReason)
  (PigCoop|KickPigsfromCoop))

(event EventBeginPlay
  ;[1 1 1] Begin play.
  (|CallParentFunction)
  (CallFunction|UpdateBuildedMeshes)
  (if (Variables|Default|GetBuilt)
    (PigCoop|InitMatingWidget)))

(event EventTick
  (params (DeltaSeconds :type Float%20%28single-precision%29))
  ;[1 1 1] Event tick.
  (|CallParentFunction DeltaSeconds)
  (PigCoop|RotateMatingWidget))

(fn ConstructionScript
  (bind _progresswidget (Variables|Default|GetProgressWidget))
  ;[1 1 1] Set construction settings.
  (|CallParentFunction)
  (Rendering|SetVisibility _progresswidget false false)
  (Rendering|SetCastShadow _progresswidget false))

(fn InitMatingWidget
  ;[1 1 1] Init mating progress widget.
  (bind _asui_world_progress_state (Utilities|Casting|CastToUI_WorldProgressState (UserInterface|GetUserWidgetObject (Variables|Default|GetProgressWidget))))
  (Default|SetProgressName _asui_world_progress_state "Mating"))

(fn StartMatingTimer
  (params (MatingTime :type Float%20%28double-precision%29))
  ;[1 1 1] Start mating progress timer.
  (Variables|State|PigCoop|SetMatingTime MatingTime)
  (Variables|State|PigCoop|SetMatingInProcess true)
  (bind _returnvalue (Utilities|Time|SetTimerbyEvent (EventDispatchers|CreateEvent :!event UpdateMatingTime) (Variables|Settings|PigCoop|GetMatingTickInterval) true))
  (Variables|State|PigCoop|SetMatingTimerHandle _returnvalue)
  (Rendering|SetVisibility (Variables|Default|GetProgressWidget) true false))

(fn StopMatingTimer
  ;[1 1 1] Stop mating progress timer.
  (Variables|State|PigCoop|SetMatingTime 0.0)
  (Variables|State|PigCoop|SetMatingInProcess false)
  (Utilities|Time|ClearandInvalidateTimerbyHandle (Variables|State|PigCoop|GetMatingTimerHandle))
  (Rendering|SetVisibility (Variables|Default|GetProgressWidget) false false))

(fn UpdateMatingTime
  ;[1 1 1] Update mating time. Release pigs after mating and start breeding timer for a pig.
  (bind _output_get (Variables|State|PigCoop|SetMatingTime (+ (stale _output_get) (Variables|Settings|PigCoop|GetMatingTickInterval))))
  (if (>= _output_get (Variables|Settings|PigCoop|GetMatingTimeRequired))
    (PigCoop|StopMatingTimer)
    (bind _pigreference (PigCoop|ReleasePigs))
    (Default|StartBreedingTimer _pigreference 0.0)))

(fn OnRepMatingTime
  ;[1 1 1] Update mating progress widget.
  (bind _asui_world_progress_state (Utilities|Casting|CastToUI_WorldProgressState (UserInterface|GetUserWidgetObject (Variables|Default|GetProgressWidget))))
  (Default|SetProgressValue _asui_world_progress_state (Variables|State|PigCoop|GetMatingTime) (Variables|Settings|PigCoop|GetMatingTimeRequired)))

(fn RotateMatingWidget
  (bind _returnvalue (Game|GetPlayerCameraManager 0))
  (bind _progresswidget (Variables|Default|GetProgressWidget))
  ;[1 1 1] Rotate state widgets face to the local player controller.
  (if (Rendering|IsVisible _progresswidget)
    (Utilities|IsValid _returnvalue
      (:Is%20Valid
        (Transformation|SetWorldRotation (Variables|Default|GetProgressWidget) (Math|Rotator|FindLookatRotation (Transformation|GetWorldLocation _progresswidget) (Camera|GetCameraLocation _returnvalue)) false false)))))

(fn OnRepMatinginProcess
  (bind _skeletalmesh (Variables|Default|GetSkeletalMesh))
  ;[1 1 1] Update mating progress animation.
  (if (Variables|State|PigCoop|GetMatingInProcess)
    (Audio|Components|Audio|Play _skeletalmesh true)
    (elif (Audio|Components|Audio|IsPlaying _skeletalmesh)
      (Audio|Components|Audio|Play _skeletalmesh false))))

(fn CoopIsEmpty
  ;[1 1 1] Returns true, if coop is opened and is empty.
  (if (Variables|Default|GetBuilt)
    (return (Math|Boolean|ANDBoolean (Variables|State|PigCoop|GetCoopIsOpened) (not (Variables|State|PigCoop|GetPigInside)) (not (Variables|State|PigCoop|GetSwineInside))))
    (else
      (return false))))

(fn TrytoLetinPig
  (params (TargetPig :type Pawn%20Object%20Reference))
  ;[1 1 1] Let in pig or swine into coop.
  (if (Variables|State|PigCoop|GetCoopIsOpened)
    (bind _asbp_character_pig (Utilities|Casting|CastToBP_Character_Pig TargetPig)
      (:then
        (if (not (Variables|State|PigCoop|GetPigInside))
          (Variables|State|PigCoop|SetPigInside true)
          (Variables|State|PigCoop|SetPigHealth (Variables|/Game/EasySurvivalRPG/Blueprints/Characters/Base/BP_Character_Base.BP_Character_Base_C|GetHealth _asbp_character_pig))
          (Actor|DestroyActor _asbp_character_pig)
          (PigCoop|CheckMating)
          (return true)
          (else
            _)))
      (:CastFailed
        (bind _asbp_character_swine (Utilities|Casting|CastToBP_Character_Swine TargetPig)
          (:then
            (if (not (Variables|State|PigCoop|GetSwineInside))
              (Variables|State|PigCoop|SetSwineInside true)
              (Variables|State|PigCoop|SetSwineHealth (Variables|/Game/EasySurvivalRPG/Blueprints/Characters/Base/BP_Character_Base.BP_Character_Base_C|GetHealth _asbp_character_swine))
              (Actor|DestroyActor _asbp_character_swine)
              (PigCoop|CheckMating)
              (return true)
              (else
                _)))
          (:CastFailed
            _)))))
  (return false))

(fn CheckMating
  ;[1 1 1] Check that pig and swine in the coop and start mating timer.
  (if (Math|Boolean|ANDBoolean (Variables|State|PigCoop|GetPigInside) (Variables|State|PigCoop|GetSwineInside) (not (Variables|State|PigCoop|GetMatingInProcess)))
    (PigCoop|StartMatingTimer 0.0)
    (Utilities|Time|ClearandInvalidateTimerbyHandle (Variables|State|PigCoop|GetKickPigsTimerHandle))
    (else
      (PigCoop|StartKickPigsTimer 1e+01))))

(fn KickPigsfromCoop
  ;[1 1 1] Kick pigs from the coop.
  (PigCoop|ReleasePigs)
  (PigCoop|StopMatingTimer))

(fn ReleasePigs
  (bind _releaselocation2 (Variables|Default|GetReleaseLocation2))
  (bind _releaselocation1 (Variables|Default|GetReleaseLocation1))
  ;[1 1 1] Release pigs from the coop.
  (Utilities|FlowControl|Sequence
    (:then_0
      (if (Variables|State|PigCoop|GetPigInside)
        (Variables|State|PigCoop|SetPigInside false)
        (bind _returnvalue (Game|SpawnActorfromClass "/Game/EasySurvivalRPG/Blueprints/Characters/Base/BP_Character_Pig.BP_Character_Pig_C" (Math|Transform|MakeTransform (Transformation|GetWorldLocation _releaselocation1) (Transformation|GetWorldRotation _releaselocation1) "1.000000,1.000000,1.000000") "AlwaysSpawn" 0 0))
        (bind _output_get (LocalVariables|SetLocalPigReference _returnvalue))
        (Utilities|IsValid _output_get
          (:Is%20Valid
            (Variables|/Game/EasySurvivalRPG/Blueprints/Characters/Base/BP_Character_Base.BP_Character_Base_C|SetHealth _output_get (Variables|State|PigCoop|GetPigHealth))))))
    (:then_1
      (if (Variables|State|PigCoop|GetSwineInside)
        (Variables|State|PigCoop|SetSwineInside false)
        (bind _returnvalue_2 (Game|SpawnActorfromClass "/Game/EasySurvivalRPG/Blueprints/Characters/Base/BP_Character_Swine.BP_Character_Swine_C" (Math|Transform|MakeTransform (Transformation|GetWorldLocation _releaselocation2) (Transformation|GetWorldRotation _releaselocation2) "1.000000,1.000000,1.000000") "AlwaysSpawn" 0 0))
        (bind _output_get_2 (LocalVariables|SetLocalSwineReference _returnvalue_2))
        (Utilities|IsValid _output_get_2
          (:Is%20Valid
            (Variables|/Game/EasySurvivalRPG/Blueprints/Characters/Base/BP_Character_Base.BP_Character_Base_C|SetHealth _output_get_2 (Variables|State|PigCoop|GetSwineHealth))))))
    (:then_2
      (return (LocalVariables|GetLocalPigReference) (LocalVariables|GetLocalSwineReference)))))

(fn LoadDataBPI
  (params (SaveData :type Save%20Game%20Object%20Reference))
  ;[1 1 1] Load pig coop data.
  (bind _output_get (LocalVariables|SetLocalSaveData SaveData))
  (bind _success (|CallParentFunction _output_get))
  (if _success
    (bind _savedata (Class|BPIGameSave|GetActorSaveDataBPI(Message) _output_get (Variables|Default|GetSaveID)))
    (LocalVariables|SetLocalFormattedVariables (Utilities|Struct|BreakSTR_SaveData_Actor _savedata))
    (Utilities|FlowControl|Sequence
      (:then_0
        (bind (_success_2 _value) (CallFunction|GetFormattedVariableBooleanValue (LocalVariables|GetLocalFormattedVariables) "MatingInProcess"))
        (bind (_success_3 _value_2) (CallFunction|GetFormattedVariableFloatValue (LocalVariables|GetLocalFormattedVariables) "MatingTime"))
        (if (and _success_2 _success_3)
          (bind _output_get_2 (Variables|State|PigCoop|SetMatingInProcess _value))
          (bind _output_get_3 (Variables|State|PigCoop|SetMatingTime _value_2))
          (if _output_get_2
            (PigCoop|StartMatingTimer _output_get_3))
          (else
            (return false))))
      (:then_1
        (Utilities|FlowControl|Sequence
          (:then_0
            (bind (_success_4 _value_3) (CallFunction|GetFormattedVariableBooleanValue (LocalVariables|GetLocalFormattedVariables) "PigInside"))
            (bind (_success_5 _value_4) (CallFunction|GetFormattedVariableFloatValue (LocalVariables|GetLocalFormattedVariables) "PigHealth"))
            (bind (_success_6 _value_5) (CallFunction|GetFormattedVariableBooleanValue (LocalVariables|GetLocalFormattedVariables) "SwineInside"))
            (bind (_success_7 _value_6) (CallFunction|GetFormattedVariableFloatValue (LocalVariables|GetLocalFormattedVariables) "SwineHealth"))
            (if (Math|Boolean|ANDBoolean _success_4 _success_5 _success_6 _success_7)
              (bind _output_get_4 (Variables|State|PigCoop|SetPigInside _value_3))
              (Variables|State|PigCoop|SetPigHealth _value_4)
              (bind _output_get_5 (Variables|State|PigCoop|SetSwineInside _value_5))
              (Variables|State|PigCoop|SetSwineHealth _value_6)
              (if (or _output_get_4 _output_get_5)
                (bind (_success_8 _value_7) (CallFunction|GetFormattedVariableFloatValue (LocalVariables|GetLocalFormattedVariables) "KickTimerTime"))
                (if _success_8
                  (PigCoop|StartKickPigsTimer _value_7)
                  (else
                    (return false))))
              (else
                (return false))))
          (:then_1
            (Utilities|FlowControl|Sequence
              (:then_0
                (bind (_success_9 _value_8) (CallFunction|GetFormattedVariableBooleanValue (LocalVariables|GetLocalFormattedVariables) "CoopIsOpened"))
                (if _success_9
                  (Variables|State|PigCoop|SetCoopIsOpened _value_8)
                  (else
                    (return false))))
              (:then_1
                (return true)))))))
    (else
      (return _success))))

(fn GetFormattedVariablesBPI
  ;[1 1 1] Format variables for the save system.
  (bind _formattedvariables (|CallParentFunction))
  (Utilities|Array|AppendArray _formattedvariables (Utilities|Array|MakeArray (CallFunction|FormatBooleanVariabletoString "MatingInProcess" (Variables|State|PigCoop|GetMatingInProcess)) (CallFunction|FormatFloatVariabletoString "MatingTime" (Variables|State|PigCoop|GetMatingTime)) (CallFunction|FormatBooleanVariabletoString "PigInside" (Variables|State|PigCoop|GetPigInside)) (CallFunction|FormatFloatVariabletoString "PigHealth" (Variables|State|PigCoop|GetPigHealth)) (CallFunction|FormatBooleanVariabletoString "SwineInside" (Variables|State|PigCoop|GetSwineInside)) (CallFunction|FormatFloatVariabletoString "SwineHealth" (Variables|State|PigCoop|GetSwineHealth)) (CallFunction|FormatBooleanVariabletoString "CoopIsOpened" (Variables|State|PigCoop|GetCoopIsOpened)) (CallFunction|FormatFloatVariabletoString "KickTimerTime" (Utilities|Time|GetTimerRemainingTimebyHandle (Variables|State|PigCoop|GetKickPigsTimerHandle)))))
  (return _formattedvariables))

(fn StartKickPigsTimer
  (params (Time :type Float%20%28double-precision%29))
  ;[1 1 1] Start kick pigs timer.
  (bind _returnvalue (Utilities|Time|SetTimerbyEvent (EventDispatchers|CreateEvent :!event KickPigsfromCoop) Time))
  (Variables|State|PigCoop|SetKickPigsTimerHandle _returnvalue))

(fn CheckCanInteractBPI
  (params (PlayerController :type Player%20Controller%20Object%20Reference))
  ;[1 1 1] Always allows interact with object.
  (return true))

(fn GetInteractionObjectNameBPI
  ;[1 1 1] Returns interaction object name.
  (return (.Name (Utilities|Struct|BreakSTR_BuildingObjectSettings (Variables|Default|GetBuildingObjectSettings)))))

(fn GetInteractionTextBPI
  (params (PlayerController :type Player%20Controller%20Object%20Reference))
  ;[1 1 1] Returns interaction text.
  (return (select (Variables|State|PigCoop|GetCoopIsOpened) "Close pig coop" "Open pig coop")))

(fn IsTurnedonBPI
  ;[1 1 1] Is not used.
  (return false))