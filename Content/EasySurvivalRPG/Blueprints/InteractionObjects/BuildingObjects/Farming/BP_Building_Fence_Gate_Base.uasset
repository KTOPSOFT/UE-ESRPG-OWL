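; Base fence gate building object for farming that players can open and close through the interaction interface.
; Interacting on release toggles GateIsOpened and multicasts the matching open or close sound.
; A RepNotify plays or reverses a timeline that yaws GateAxis, so the swing follows the replicated state.
; The open state is appended to the parent's formatted save variables and restored on load.
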(event Custom|PlayOpenGate
  ;[1 1 1] Open and close gate.
  (bind _rotationz (Timeline|OpenGateTimeline Play)
    (:Update
      (Transformation|SetRelativeRotation (Variables|Default|GetGateAxis) (Math|Rotator|MakeRotator 0.0 0.0 _rotationz) false true))))

(event Custom|PlayCloseGate
  ;[1 1 1] Open and close gate.
  (bind _rotationz (Timeline|OpenGateTimeline Reverse)
    (:Update
      (Transformation|SetRelativeRotation (Variables|Default|GetGateAxis) (Math|Rotator|MakeRotator 0.0 0.0 _rotationz) false true))))

(event EventTryInteractBPI
  (params (Release :type Boolean) (PlayerController :type Player%20Controller%20Object%20Reference))
  ;[1 1 1] Open / close gate interaction.
  (if Release
    (if (Variables|State|Gate|GetGateIsOpened)
      (Gate|CloseGate)
      (else
        (Gate|OpenGate)))))

(fn ConstructionScript
  (|CallParentFunction))

(fn OpenGate
  ;[1 1 1] Open gate and update Is opened variables.
  (Variables|State|Gate|SetGateIsOpened true)
  (CallFunction|PlaySoundatLocation(Multicast) (Variables|Settings|Gate|GetOpenGateSound) (Transformation|GetActorLocation)))

(fn OnRepDoorIsOpened
  ;[1 1 1] Play gate animation depending on DoorIsOpened variable.
  (if (Variables|State|Gate|GetGateIsOpened)
    (CallFunction|PlayOpenGate)
    (else
      (CallFunction|PlayCloseGate))))

(fn CloseGate
  ;[1 1 1] Close gate and update Is opened variables.
  (Variables|State|Gate|SetGateIsOpened false)
  (CallFunction|PlaySoundatLocation(Multicast) (Variables|Settings|Gate|GetCloseGateSound) (Transformation|GetActorLocation)))

(fn GetFormattedVariablesBPI
  ;[1 1 1] Save important variables.
  (bind _formattedvariables (|CallParentFunction))
  (Utilities|Array|AppendArray _formattedvariables (Utilities|Array|MakeArray (CallFunction|FormatBooleanVariabletoString "GateIsOpened" (Variables|State|Gate|GetGateIsOpened))))
  (return _formattedvariables))

(fn LoadDataBPI
  (params (SaveData :type Save%20Game%20Object%20Reference))
  ;[1 1 1] Load data for the gate.
  (bind _success (|CallParentFunction SaveData))
  (bind _savedata (Class|BPIGameSave|GetActorSaveDataBPI(Message) SaveData (Variables|Default|GetSaveID)))
  (bind (_success_2 _value) (CallFunction|GetFormattedVariableBooleanValue (Utilities|Struct|BreakSTR_SaveData_Actor _savedata) "GateIsOpened"))
  (if _success_2
    (Variables|State|Gate|SetGateIsOpened _value)
    (return _success)))

(fn CheckCanInteractBPI
  (params (PlayerController :type Player%20Controller%20Object%20Reference))
  ;[1 1 1] Always allows interact with object.
  (return true))

(fn GetInteractionObjectNameBPI
  ;[1 1 1] Returns interaction object name.
  (return (.Name (Utilities|Struct|BreakSTR_BuildingObjectSettings (Variables|Default|GetBuildingObjectSettings)))))

(fn GetInteractionTextBPI
  (params (PlayerController :type Player%20Controller%20Object%20Reference))
  ;[1 1 1] Returns interaction text.
  (return (select (Variables|State|Gate|GetGateIsOpened) "Close the gate" "Open the gate")))

(fn IsTurnedonBPI
  ;[1 1 1] Is not used.
  (return false))