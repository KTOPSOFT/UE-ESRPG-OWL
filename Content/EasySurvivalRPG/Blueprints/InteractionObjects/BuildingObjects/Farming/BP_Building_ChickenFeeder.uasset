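; BP_Building_ChickenFeeder is a farming building object that stores feed in a container players open by interacting.
; Once built, the server initializes the container and adds starting feed on BeginPlay.
; Slot changes set the replicated HasFood flag, whose OnRep swaps the mesh between full and empty.
; ConsumeFood removes one item from the first slot; nothing in this Blueprint calls it.
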(event OnSlotItemChanged(ContainerComponent)
  (params (Slot :type Integer) (Item :type STR%20Item%20Data%20Structure))
  (bind _isvalid (CallFunction|ItemIsValid Item))
  ;[1 1 1] Interactions with feeder container.
  (if (Math|Boolean|NotEqual(Boolean) (Variables|State|ChickenFeeder|GetHasFood) _isvalid)
    (Variables|State|ChickenFeeder|SetHasFood _isvalid)))

(event EventBeginPlay
  (bind _containercomponent (Variables|Default|GetContainerComponent))
  ;[1 1 1] Begin play. Update feeder mesh and add starting feed to the container.
  (|CallParentFunction)
  (ChickenFeeder|UpdateFeederMesh)
  (if (Variables|Default|GetBuilt)
    (Networking|SwitchHasAuthority
      (:Authority
        (Default|InitComponent _containercomponent)
        (Default|TryAddItemsorDrop _containercomponent (CallFunction|MakeLootItems (Variables|Settings|ChickenFeeder|GetStartingFeedHandle)))))))

(event EventTryInteractBPI
  (params (Release :type Boolean) (PlayerController :type Player%20Controller%20Object%20Reference))
  ;[1 1 1] Interactions with feeder container.
  (if Release
    (Class|BPIPlayer|OpenContainerBPI(Message) PlayerController (Variables|Default|GetContainerComponent))))

(fn ConstructionScript
  (|CallParentFunction))

(fn OnRepHasFood
  ;[1 1 1] Update feeder mesh when has food state is changed.
  (ChickenFeeder|UpdateFeederMesh))

(fn UpdateFeederMesh
  ;[1 1 1] Update chicken feeder mesh depending on has food state.
  (Components|StaticMesh|SetStaticMesh (Variables|Default|GetStaticMesh) (select (Variables|State|ChickenFeeder|GetHasFood) (Variables|Settings|ChickenFeeder|GetFoodMesh) (Variables|Settings|ChickenFeeder|GetEmptyMesh))))

(fn ConsumeFood
  ;[1 1 1] Consume food item in chicken feeder.
  (Default|ConsumeItem (Variables|Default|GetContainerComponent) 0 1))

(fn CheckCanInteractBPI
  (params (PlayerController :type Player%20Controller%20Object%20Reference))
  ;[1 1 1] Always allows interact with object.
  (return true))

(fn GetInteractionObjectNameBPI
  ;[1 1 1] Returns interaction object name.
  (return (.Name (Utilities|Struct|BreakSTR_BuildingObjectSettings (Variables|Default|GetBuildingObjectSettings)))))

(fn GetInteractionTextBPI
  (params (PlayerController :type Player%20Controller%20Object%20Reference))
  ;[1 1 1] Returns interaction text.
  (return (.Name (Utilities|Struct|BreakSTR_BuildingObjectSettings (Variables|Default|GetBuildingObjectSettings)))))

(fn IsTurnedonBPI
  ;[1 1 1] Is not used.
  (return false))