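; Base interaction switcher that players toggle on or off, exposing its name, state-dependent prompt text and on/off state through Blueprint interface functions.
; Interaction toggles on release, unless SwitchedOnce is set and the switcher is already on; interface turn-on/off events skip this check.
; All changes go through SetSwitchedOn, which calls OnSwitchedByPlayer.
; IsSwitchedOn's RepNotify calls OnSwitchedOnReplication, an empty hook here.
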(event EventTryTurnOffBPI
  ;[1 1 1] Interactions. Switch the switcher by player.
  (Switcher|SetSwitchedon 0 false))

(event EventTryInteractBPI
  (params (Release :type Boolean) (PlayerController :type Player%20Controller%20Object%20Reference))
  ;[1 1 1] Interactions. Switch the switcher by player.
  (if Release
    (bind _caninteract (CallFunction|CheckCanInteractBPI PlayerController))
    (if _caninteract
      (Switcher|SetSwitchedon PlayerController (not (Variables|Settings|GetIsSwitchedOn))))))

(event EventTryTurnonBPI
  ;[1 1 1] Interactions. Switch the switcher by player.
  (Switcher|SetSwitchedon 0 true))

(fn ConstructionScript)

(fn SetSwitchedon
  (params (PlayerController :type Player%20Controller%20Object%20Reference) (SwitchedOn :type Boolean))
  ;[1 1 1] Set switched on variable and call switched event.
  (bind _output_get (Variables|Settings|SetIsSwitchedOn SwitchedOn))
  (Default|CallOnSwitchedbyPlayer PlayerController _output_get))

(fn OnRepIsSwitchedon
  (Switcher|OnSwitchedonReplication))

(fn OnSwitchedonReplication)

(fn CheckCanInteractBPI
  (params (PlayerController :type Player%20Controller%20Object%20Reference))
  (return (not (and (Variables|Settings|GetIsSwitchedOn) (Variables|Settings|GetSwitchedOnce)))))

(fn GetInteractionObjectNameBPI
  (return (Variables|Settings|GetName)))

(fn GetInteractionTextBPI
  (params (PlayerController :type Player%20Controller%20Object%20Reference))
  (return (select (Variables|Settings|GetIsSwitchedOn) (Variables|Settings|GetSwitchOffText) (Variables|Settings|GetSwitchOnText))))

(fn IsTurnedonBPI
  (return (Variables|Settings|GetIsSwitchedOn)))