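; Fishing floater projectile that handles bites and catches after landing in water.
; On water overlap the server starts a bite timer from an overlapped fishing place, or optional defaults, and multicasts the stop and splash.
; A timed hook window picks a loot handle, with a replicated flag driving the animation.
; TryCatchFish adds hooked loot to the player's inventory and destroys the floater, whose destruction resets the instigator's fishing state.
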(event OnComponentBeginOverlap(CheckWaterCollision)
  (params (OverlappedComponent :type Primitive%20Component%20Object%20Reference) (OtherActor :type Actor%20Object%20Reference) (OtherComp :type Primitive%20Component%20Object%20Reference) (OtherBodyIndex :type Integer) (bFromSweep :type Boolean) (SweepResult :type Hit%20Result%20Structure%20%28by%20ref%29))
  ;[1 1 1] Start fishing on water overlap.
  (Networking|SwitchHasAuthority
    (:Authority
      (Floater|StartFishing)
      (CallFunction|WaterHit(Multicast)))))

(event Custom|WaterHit%20%28Multicast%29
  ;[1 1 1] Water hit.
  (Floater|WaterHit))

(event Custom|FishingRodDestroyed
  (params (FishingRod :type Actor%20Object%20Reference))
  ;[1 1 1] Destroy floater with fishing rod.
  (Networking|SwitchHasAuthority
    (:Authority
      (Actor|DestroyActor))))

(event EventDestroyed
  ;[1 1 1] Reset fishing state for character when floater is destroyed.
  (Networking|SwitchHasAuthority
    (:Authority
      (Class|BPIPlayerCharacter|SetFishingStateBPI(Message) (Game|GetInstigator) false))))

(event Collision|EventHit
  (params (MyComp :type Primitive%20Component%20Object%20Reference) (Other :type Actor%20Object%20Reference) (OtherComp :type Primitive%20Component%20Object%20Reference) (bSelfMoved :type Boolean) (HitLocation :type Vector :default "0, 0, 0") (HitNormal :type Vector :default "0, 0, 0") (NormalImpulse :type Vector :default "0, 0, 0") (Hit :type Hit%20Result%20Structure%20%28by%20ref%29))
  ;[1 1 1] Destroy floater on hit.
  (Networking|SwitchHasAuthority
    (:Authority
      (Actor|DestroyActor))))

(fn ConstructionScript
  (|CallParentFunction))

(fn SetFishingRod
  (params (FishingRod :type BP%20Usable%20Item%20Fishing%20Rod%20Object%20Reference))
  ;[1 1 1] Set fishing rod reference.
  (bind _output_get (Variables|State|SetFishingRodReference FishingRod))
  (Game|BindEventtoOnDestroyed _output_get (EventDispatchers|CreateEvent :!event Custom|FishingRodDestroyed)))

(fn StartFishing
  (bind _returnvalue (Transformation|GetActorLocation))
  ;[1 1 1] Check fishing place and start catch fish timer.
  (bind _outhits (Collision|MultiSphereTraceForObjects _returnvalue _returnvalue 1.0 (Utilities|Array|MakeArray "ObjectTypeQuery2") false 0 "None"))
  (for _array_element _outhits
    (bind _asbp_fishing_place_base (Utilities|Casting|CastToBP_FishingPlace_Base (.HitActor (Collision|BreakHitResult _array_element))))
    (Variables|State|SetFishingPlaceReference _asbp_fishing_place_base)
    (Utilities|Time|SetTimerbyEvent (EventDispatchers|CreateEvent :!event FishontheHook) (Default|GetRandomCatchFishTime _asbp_fishing_place_base))
    (return true))
  (if (not (Variables|Settings|GetUseOnlyFishingPlaces))
    (Utilities|Time|SetTimerbyEvent (EventDispatchers|CreateEvent :!event FishontheHook) (Math|Random|RandomFloatinRange (Variables|Settings|GetMinCatchFishTime) (Variables|Settings|GetMaxCatchFishTime)))
    (return true)))

(fn TryCatchFish
  ;[1 1 1] Try catch a fish and add fish loot to the player's inventory.
  (if (Variables|State|GetIsFishOnTheHook)
    (bind (_success _items) (Floater|MakeCatchedItems (Variables|State|GetCatchedFishLootHandle)))
    (if _success
      (bind _inventorycontainer (Class|BPIPlayer|GetInventoryContainerBPI(Message) (Game|GetInstigatorController)))
      (Default|TryAddItems _inventorycontainer _items)))
  (Actor|DestroyActor)
  (CallFunction|PlaySoundatLocation(Multicast) (Variables|Settings|GetTryCatchSound) (Transformation|GetActorLocation))
  (return true))

(fn WaterHit
  (bind _projectilemovement (Variables|Default|GetProjectileMovement))
  ;[1 1 1] Stop projectile movement and play water splash sound.
  (Variables|State|SetIsFishOnTheHook false)
  (Components|Movement|StopMovementImmediately _projectilemovement)
  (Components|DestroyComponent _projectilemovement)
  (Physics|SetEnableGravity (Variables|Default|GetProjectileMesh) false)
  (CallFunction|PlaySoundatLocation(Multicast) (Variables|Settings|GetSplashSound) (Transformation|GetActorLocation)))

(fn FishontheHook
  (bind _fishingplacereference (Variables|State|GetFishingPlaceReference))
  ;[1 1 1] Set the fish on the hook state and start fish off timer.
  (Variables|State|SetIsFishOnTheHook true)
  (Utilities|IsValid _fishingplacereference
    (:Is%20Valid
      (Variables|State|SetCatchedFishLootHandle (Default|GetRandomFishLootHandle _fishingplacereference))
      (Utilities|Time|SetTimerbyEvent (EventDispatchers|CreateEvent :!event FishOfftheHook) (Default|GetRandomFishOffTime _fishingplacereference)))
    (:Is%20Not%20Valid
      (Variables|State|SetCatchedFishLootHandle (Floater|GetRandomCatchFishHandle))
      (Utilities|Time|SetTimerbyEvent (EventDispatchers|CreateEvent :!event FishOfftheHook) (Math|Random|RandomFloatinRange (Variables|Settings|GetMinFishOffTime) (Variables|Settings|GetMaxFishOffTime))))))

(fn FishOfftheHook
  ;[1 1 1] Reset the fish is catched state.
  (Variables|State|SetIsFishOnTheHook false))

(fn OnRepIsFishontheHook
  ;[1 1 1] Play animation depending on the fish on the hook variable.
  (Components|Animation|PlayAnimation (Variables|Default|GetFloaterMesh) (select (Variables|State|GetIsFishOnTheHook) "/Game/EasySurvivalRPG/Characters/Jess/Weapons/A_Floater_Take.A_Floater_Take" "/Game/EasySurvivalRPG/Characters/Jess/Weapons/A_Floater_Idle.A_Floater_Idle") true))

(fn GetRandomCatchFishHandle
  (bind _catchfishloothandles (Variables|Settings|GetCatchFishLootHandles))
  ;[1 1 1] Returns random fish loot handle.
  (bind _output_get (LocalVariables|SetLocalIndex (Math|Random|RandomIntegerinRange 0 (Utilities|Array|LastIndex _catchfishloothandles))))
  (if (Utilities|Array|IsValidIndex _catchfishloothandles _output_get)
    (return (Utilities|Array|Get(acopy) _catchfishloothandles _output_get))))

(fn MakeCatchedItems
  (params (LootHandle :type Data%20Table%20Row%20Handle%20Structure))
  ;[1 1 1] Make catched items from loot handle.
  (if (CallFunction|HandleIsValid LootHandle)
    (if (Variables|Settings|GetCatchSingleRandomItem)
      (return true (Utilities|Array|MakeArray (CallFunction|MakeRandomLootItem LootHandle)))
      (else
        (return true (CallFunction|MakeLootItems LootHandle))))
    (else
      (return false 0))))