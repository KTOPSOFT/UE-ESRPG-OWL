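; Settings SaveGame object for EasySurvivalRPG that tracks the names of singleplayer and multiplayer game saves.
; Adding a save removes any existing entry and reinserts it at index 0, keeping each list free of duplicates and ordered by most recently added.
; Removing a save also deletes its slot from storage.
; Every add or remove immediately writes the object itself to the settings slot.
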(fn SaveSettings
  ;[1 1 1] Save settings to default settings save slot.
  (SaveGame|SaveGametoSlot self (Variables|Default|GetGameSettingsSlot)))

(fn AddSingleplayerSave
  (params (SaveName :type String))
  (bind _singleplayergamesavenames (Variables|Default|GetSingleplayerGameSaveNames))
  ;[1 1 1] Add singleplayer save name and save settings.
  (Utilities|Array|RemoveItem _singleplayergamesavenames SaveName)
  (Utilities|Array|Insert _singleplayergamesavenames SaveName)
  (CallFunction|SaveSettings))

(fn RemoveSingleplayerSave
  (params (SaveName :type String))
  ;[1 1 1] Remove singleplayer save name and save settings.
  (bind _output_get (LocalVariables|SetLocalSlotName SaveName))
  (SaveGame|DeleteGameinSlot _output_get)
  (Utilities|Array|RemoveItem (Variables|Default|GetSingleplayerGameSaveNames) (LocalVariables|GetLocalSlotName))
  (CallFunction|SaveSettings))

(fn AddMultiplayerSave
  (params (SaveName :type String))
  (bind _multiplayergamesavenames (Variables|Default|GetMultiplayerGameSaveNames))
  ;[1 1 1] Add multiplayer save name and save settings.
  (Utilities|Array|RemoveItem _multiplayergamesavenames SaveName)
  (Utilities|Array|Insert _multiplayergamesavenames SaveName)
  (CallFunction|SaveSettings))

(fn RemoveMultiplayerSave
  (params (SaveName :type String))
  ;[1 1 1] Remove multiplayer save name and save settings.
  (bind _output_get (LocalVariables|SetLocalSlotName SaveName))
  (SaveGame|DeleteGameinSlot _output_get)
  (Utilities|Array|RemoveItem (Variables|Default|GetMultiplayerGameSaveNames) (LocalVariables|GetLocalSlotName))
  (CallFunction|SaveSettings))