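; Anim notify state that switches which socket a character's weapon is attached to during an animation.
; On notify begin it sends the start socket to the mesh owner through a SetWeaponSocket Blueprint interface message.
; On notify end it sends the end socket the same way, leaving the actual attachment to the owning actor.
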(fn GetNotifyName
  (return "Change Weapon Socket"))

(fn ReceivedNotifyBegin
  (params (MeshComp :type Skeletal%20Mesh%20Component%20Object%20Reference) (Animation :type Anim%20Sequence%20Base%20Object%20Reference) (TotalDuration :type Float%20%28single-precision%29))
  ;[1 1 1] Attach weapon to start weapon socket.
  (Class|BPIPlayerCharacter|SetWeaponSocketBPI(Message) (Components|GetOwner MeshComp) (Variables|Default|GetStartWeaponSocket))
  (return false))

(fn ReceivedNotifyEnd
  (params (MeshComp :type Skeletal%20Mesh%20Component%20Object%20Reference) (Animation :type Anim%20Sequence%20Base%20Object%20Reference))
  ;[1 1 1] Attach weapon to end weapon socket.
  (Class|BPIPlayerCharacter|SetWeaponSocketBPI(Message) (Components|GetOwner MeshComp) (Variables|Default|GetEndWeaponSocket))
  (return false))