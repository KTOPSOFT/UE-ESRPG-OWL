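; Component that provides an on-screen RPM web view that can be shown and hidden during play.
; On BeginPlay it creates the WBP_RPM_WebViewWrapper widget, adds it to the viewport hidden and keeps a reference.
; ToggleRPMWebView flips that widget's visibility and shows or hides player 0's mouse cursor to match.
; Input mode switching nodes exist but are unconnected, so toggling leaves the input mode unchanged.
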(event EventBeginPlay
  (CallFunction|InitRPMWebView))

(event EventTick
  (params (DeltaSeconds :type Float%20%28single-precision%29)))

(fn InitRPMWebView
  (bind _returnvalue (UserInterface|CreateWidget "/RpmWebView/Widgets/WBP_RPM_WebViewWrapper.WBP_RPM_WebViewWrapper_C"))
  (bind _output_get (Variables|Default|SetRPM_Webview_Instance _returnvalue))
  (UserInterface|Viewport|AddtoViewport _output_get 0)
  (Widget|SetVisibility _output_get "Hidden"))

(fn ToggleRPMWebView
  (bind _returnvalue (Game|GetPlayerController 0))
  (bind _output_get (Variables|Default|SetRPM_Webview_Instance (Variables|Default|GetRPM_Webview_Instance)))
  (if (Widget|IsVisible (Variables|Default|GetRPM_Webview_Instance))
    (Variables|/Script/UMG.Widget|SetVisibility _output_get "Hidden")
    (Variables|/Script/Engine.PlayerController|SetbShowMouseCursor _returnvalue false)
    (else
      (Variables|/Script/UMG.Widget|SetVisibility _output_get "Visible")
      (Variables|/Script/Engine.PlayerController|SetbShowMouseCursor _returnvalue true))))