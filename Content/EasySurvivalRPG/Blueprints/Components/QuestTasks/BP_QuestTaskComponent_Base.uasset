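; Base quest task component for the survival RPG, meant to be subclassed for concrete task types.
; It stores the player manager reference on init and declares overridable stubs for getting progress, progress text and loading progress.
; CheckFinished turns the finished state into completion or, when FailWhenFinished is set, failure, and fires the matching callback with itself.
; An unfinished task has both completed and failed flags cleared.
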(fn InitComponent
  (params (PlayerManagerComponent :type BP%20Player%20Manager%20Component%20Object%20Reference))
  ;[1 1 1] Init quest task component. Overridden in child class.
  (Variables|State|SetPlayerManagerComponent PlayerManagerComponent))

(fn GetProgress
  ;[1 1 1] Returns current task progress. Overridden in child class.
  (return ""))

(fn GetProgressText
  ;[1 1 1] Returns quest task progress text. Overridden in child class.
  (return ""))

(fn LoadProgress
  (params (Progress :type String))
  ;[1 1 1] Load quest task progress. Overridden in child class.
  (return true))

(fn CheckFinished
  (bind _self self)
  ;[1 1 1] Check finished state and complete or fail the quest task.
  (if (Variables|State|GetIsFinished)
    (if (Variables|Settings|GetFailWhenFinished)
      (Variables|State|SetIsFailed true)
      (Default|CallOnFailed _self)
      (else
        (Variables|State|SetIsCompleted true)
        (Default|CallOnCompleted _self)))
    (else
      (Variables|State|SetIsCompleted false)
      (Variables|State|SetIsFailed false))))