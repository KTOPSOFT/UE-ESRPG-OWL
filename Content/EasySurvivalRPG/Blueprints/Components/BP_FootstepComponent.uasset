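; Per-foot character component that plays footstep sounds, particles and decals, emits noise scaled by step type, and calculates foot IK.
; Settings come from a data table preset, with an override handle whose RepNotify refreshes them on clients.
; Footsteps trace for the physical surface, then check surface overrider actors or water to choose surface and splash data.
; When enabled, Tick traces the ground and interpolates foot rotation and height, exposed with a two-leg pelvis offset.
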(event EventBeginPlay
  ;[1 1 1] Init references and update footstep settings on begin play.
  (|CallParentFunction)
  (bind _ascharacter (Utilities|Casting|CastToCharacter (Components|GetOwner)))
  (Variables|State|References|SetCharacter _ascharacter)
  (FootstepComponent|Footsteps|CheckandUpdateSettings))

(event EventTick
  (params (DeltaSeconds :type Float%20%28single-precision%29))
  ;[1 1 1] Calculate IK variables.
  (|CallParentFunction DeltaSeconds)
  (if (Variables|Settings|IK|GetIK_Enabled)
    (FootstepComponent|IK|CalculateIK DeltaSeconds)
    (else
      (Components|Tick|SetComponentTickEnabled false))))

(fn OnRepOverriddenPresetHandle
  ;[1 1 1] Check and update settings footstep settings for all clients.
  (FootstepComponent|Footsteps|CheckandUpdateSettings))

(fn TrytoPlayFootstep
  (params (InFootSocket :type Name) (FootstepType :type E_FootstepType%20Enum :default "NewEnumerator7") (PlaySounds :type Boolean) (SpawnEffects :type Boolean))
  ;[1 1 1] Try to play footstep sounds and effects for a foot with target settings.
  (if (Utilities|Name|Equal(Name) InFootSocket (Variables|Settings|Footsteps|GetFootSocket))
    (if (Variables|State|Footsteps|GetSettingsAreCorrect)
      (bind (_success _location _surfacetype _playsplash) (FootstepComponent|Footsteps|CheckSurface))
      (if _success
        (LocalVariables|SetLocalLocation _location)
        (LocalVariables|SetLocalSurfaceType _surfacetype)
        (LocalVariables|SetLocalPlaySplash _playsplash)
        (bind (_success_2 _footsteptypedata) (CallFunction|FindFootstepTypeData (Variables|Settings|Footsteps|GetFootstepsData) FootstepType))
        (if _success_2
          (LocalVariables|SetLocalFootstepTypeData _footsteptypedata)
          (if PlaySounds
            (FootstepComponent|Footsteps|PlayFootstepSounds (LocalVariables|GetLocalLocation) (LocalVariables|GetLocalFootstepTypeData) (LocalVariables|GetLocalSurfaceType) (LocalVariables|GetLocalPlaySplash)))
          (if SpawnEffects
            (FootstepComponent|Footsteps|SpawnFootstepEffects (LocalVariables|GetLocalLocation) (LocalVariables|GetLocalFootstepTypeData) (LocalVariables|GetLocalSurfaceType) (LocalVariables|GetLocalPlaySplash)))
          (Default|CallOnFootstepPlayed self (LocalVariables|GetLocalLocation) FootstepType (LocalVariables|GetLocalSurfaceType) (LocalVariables|GetLocalPlaySplash) (LocalVariables|GetLocalFootstepTypeData))
          (return true)
          (else
            (return false)))
        (else
          (return false)))
      (else
        _)))
  (return false))

(fn CheckandUpdateSettings
  (bind _character (Variables|State|References|GetCharacter))
  (bind _overriddenpresethandle (Variables|State|Footsteps|GetOverriddenPresetHandle))
  ;[1 1 1] Checks references and footstep settings and returns true if everything set correctly.
  (Utilities|IsValid _character
    (:Is%20Valid
      (Variables|State|References|SetCharacterSkeletalMesh (Variables|/Script/Engine.Character|GetMesh _character))
      (FootstepComponent|Footsteps|UpdateFootstepSettingsbyHandle (select (CallFunction|PresetIsValid _overriddenpresethandle) _overriddenpresethandle (Variables|Settings|Footsteps|GetPresetHandle)))
      (bind _output_get (Variables|State|Footsteps|SetSettingsAreCorrect (Transformation|DoesSocketExist (Variables|State|References|GetCharacterSkeletalMesh) (Variables|Settings|Footsteps|GetFootSocket))))
      (return _output_get))
    (:Is%20Not%20Valid
      (bind _output_get_2 (Variables|State|Footsteps|SetSettingsAreCorrect false))
      (return _output_get_2))))

(fn UpdateFootstepSettingsbyHandle
  (params (PresetHandle :type Data%20Table%20Row%20Handle%20Structure))
  (bind (_datatable _rowname) (Utilities|Struct|BreakDataTableRowHandle PresetHandle))
  ;[1 1 1] Update footstep settings by target preset handle from data table.
  (if (CallFunction|PresetIsValid PresetHandle)
    (bind _returnvalue (Utilities|GetDataTableRow _datatable _rowname)
      (:then
        (Variables|Settings|Footsteps|SetFootSocket (.FootSocket (Utilities|Struct|BreakSTR_FootstepSettings _returnvalue)))
        (Variables|Settings|Footsteps|SetSurfaceCheckStartOffset (.SurfaceCheckStartOffset (Utilities|Struct|BreakSTR_FootstepSettings _returnvalue)))
        (Variables|Settings|Footsteps|SetSurfaceCheckEndOffset (.SurfaceCheckEndOffset (Utilities|Struct|BreakSTR_FootstepSettings _returnvalue)))
        (Variables|Settings|Footsteps|SetWaterCheckStartOffset (.WaterCheckStartOffset (Utilities|Struct|BreakSTR_FootstepSettings _returnvalue)))
        (Variables|Settings|Footsteps|SetWaterCheckEndOffset (.WaterCheckEndOffset (Utilities|Struct|BreakSTR_FootstepSettings _returnvalue)))
        (Variables|Settings|Footsteps|SetFootstepsData (.FootstepsData (Utilities|Struct|BreakSTR_FootstepSettings _returnvalue)))
        (return true))
      (:RowNotFound
        _)))
  (return false))

(fn GetFootLocation
  (bind _settingsarecorrect (Variables|State|Footsteps|GetSettingsAreCorrect))
  ;[1 1 1] Get foot location if foot socket exist.
  (return _settingsarecorrect (select _settingsarecorrect (Transformation|GetSocketLocation (Variables|State|References|GetCharacterSkeletalMesh) (Variables|Settings|Footsteps|GetFootSocket)) "0, 0, 0")))

(fn CheckSurface
  ;[1 1 1] Check surface in foot location and get hit location, hit surface type and play splash variables.
  (bind (_success _footlocation) (FootstepComponent|Footsteps|GetFootLocation))
  (if _success
    (LocalVariables|SetLocalFootLocation _footlocation)
    (bind (_outhit _returnvalue) (Collision|LineTraceByChannel (+ (LocalVariables|GetLocalFootLocation) (Math|Vector|MakeVector 0.0 0.0 (Variables|Settings|Footsteps|GetSurfaceCheckStartOffset))) (+ (LocalVariables|GetLocalFootLocation) (Math|Vector|MakeVector 0.0 0.0 (Variables|Settings|Footsteps|GetSurfaceCheckEndOffset))) "TraceTypeQuery1" false (Utilities|Array|MakeArray (Components|GetOwner)) (select (Variables|Settings|Debug|GetDebugMode) "ForDuration" "None") true "(R=1.000000,G=0.000000,B=0.000000,A=1.000000)" "(R=0.000000,G=1.000000,B=0.000000,A=1.000000)" (Variables|Settings|Debug|GetDebugTraceTime)))
    (if _returnvalue
      (bind _output_get (LocalVariables|SetLocalHitLocation (.Location (Collision|BreakHitResult _outhit))))
      (LocalVariables|SetLocalSurfaceType (Collision|GetSurfaceType _outhit))
      (bind (_override _surfacetype _playsplash) (FootstepComponent|Footsteps|CheckOverriddenSurface _output_get))
      (if _override
        (LocalVariables|SetLocalSurfaceType _surfacetype)
        (LocalVariables|SetLocalPlaySplash _playsplash)
        (else
          (bind _returnvalue_2 (Collision|LineTraceForObjects (+ (LocalVariables|GetLocalHitLocation) (Math|Vector|MakeVector 0.0 0.0 (Variables|Settings|Footsteps|GetWaterCheckStartOffset))) (+ (LocalVariables|GetLocalHitLocation) (Math|Vector|MakeVector 0.0 0.0 (Variables|Settings|Footsteps|GetWaterCheckEndOffset))) (Utilities|Array|MakeArray (CallFunction|GetWaterObjectTypeQuery)) false (Utilities|Array|MakeArray (Components|GetOwner)) (select (Variables|Settings|Debug|GetDebugMode) "ForDuration" "None") true "(R=0.000000,G=0.000000,B=1.000000,A=1.000000)" "(R=0.000000,G=0.000000,B=0.000000,A=1.000000)" (Variables|Settings|Debug|GetDebugTraceTime)))
          (LocalVariables|SetLocalPlaySplash _returnvalue_2)))
      (return true (LocalVariables|GetLocalHitLocation) (LocalVariables|GetLocalSurfaceType) (LocalVariables|GetLocalPlaySplash))
      (else
        (return false "0, 0, 0" "SurfaceType_Default" false)))
    (else
      (return false "0, 0, 0" "SurfaceType_Default" false))))

(fn CheckOverriddenSurface
  (params (Location :type Vector))
  ;[1 1 1] Check surface overrider actor in target location and get overridden surface and play splash variables.
  (bind (_outhit _returnvalue) (Collision|SphereTraceForObjects Location Location 1.0 (Utilities|Array|MakeArray (CallFunction|GetSurfaceOverriderObjectTypeQuery)) false (Utilities|Array|MakeArray (Components|GetOwner)) (select (Variables|Settings|Debug|GetDebugMode) "ForDuration" "None") true "(R=1.000000,G=0.000000,B=0.000000,A=1.000000)" "(R=0.000000,G=1.000000,B=0.000000,A=1.000000)" (Variables|Settings|Debug|GetDebugTraceTime)))
  (if _returnvalue
    (bind _asbp_surface_overrider_base (Utilities|Casting|CastToBP_SurfaceOverrider_Base (.HitActor (Collision|BreakHitResult _outhit)))
      (:then
        (return true (Variables|/Game/EasySurvivalRPG/Blueprints/Misc/WaterSurfaceSystem/BP_SurfaceOverrider_Base.BP_SurfaceOverrider_Base_C|GetSurfaceType _asbp_surface_overrider_base) (Variables|/Game/EasySurvivalRPG/Blueprints/Misc/WaterSurfaceSystem/BP_SurfaceOverrider_Base.BP_SurfaceOverrider_Base_C|GetPlaySplash _asbp_surface_overrider_base)))
      (:CastFailed
        _)))
  (return false "SurfaceType_Default" false))

(fn SetOverriddenFootstepPreset
  (params (NewPresetHandle :type Data%20Table%20Row%20Handle%20Structure))
  ;[1 1 1] Override footstep preset handle and update footstep settings from the data table.
  (Variables|State|Footsteps|SetOverriddenPresetHandle NewPresetHandle)
  (return true))

(fn ClearOverriddenFootstepPreset
  ;[1 1 1] Clear overridden preset handle and update footstep settings from the data table if default preset handle is set.
  (Variables|State|Footsteps|SetOverriddenPresetHandle "")
  (return true))

(fn PlayFootstepSounds
  (params (Location :type Vector) (FootstepTypeData :type STR%20Footstep%20Type%20Data%20Structure) (SurfaceType :type EPhysicalSurface%20Enum :default "SurfaceType_Default") (PlaySplash :type Boolean))
  ;[1 1 1] Try to play footstep sound at location.
  (Utilities|FlowControl|Sequence
    (:then_0
      (bind (_success _outdata) (CallFunction|FindFootstepSoundData (Utilities|Struct|BreakSTR_FootstepTypeData FootstepTypeData) SurfaceType))
      (if _success
        (Utilities|IsValid (Utilities|Struct|BreakSTR_FootstepSoundData _outdata)
          (:Is%20Valid
            (Audio|PlaySoundatLocation (Utilities|Struct|BreakSTR_FootstepSoundData _outdata) Location "0, 0, 0" (select PlaySplash 0.5 1.0) 1.0 0.0 0 0 0)))))
    (:then_1
      (if PlaySplash
        (bind (_success_2 _outdata_2) (CallFunction|FindFootstepSoundData (Utilities|Struct|BreakSTR_FootstepTypeData FootstepTypeData) SurfaceType))
        (if _success_2
          (Utilities|IsValid (Utilities|Struct|BreakSTR_FootstepSoundData _outdata_2)
            (:Is%20Valid
              (Audio|PlaySoundatLocation (Utilities|Struct|BreakSTR_FootstepSoundData _outdata_2) Location "0, 0, 0" 1.0 1.0 0.0 0 0 0))))))
    (:then_2
      (FootstepComponent|Footsteps|MakeNoise Location (Utilities|Struct|BreakSTR_FootstepTypeData FootstepTypeData))
      (return true))))

(fn SpawnFootstepEffects
  (params (Location :type Vector) (FootstepTypeData :type STR%20Footstep%20Type%20Data%20Structure) (SurfaceType :type EPhysicalSurface%20Enum :default "SurfaceType_Default") (PlaySplash :type Boolean))
  ;[1 1 1] Try to spawn footstep effects and decals at location.
  (Utilities|FlowControl|Sequence
    (:then_0
      (if PlaySplash
        (Utilities|FlowControl|Sequence
          (:then_0
            (bind (_success _outdata) (CallFunction|FindFootstepEffectData (Utilities|Struct|BreakSTR_FootstepTypeData FootstepTypeData) SurfaceType))
            (if _success
              (LocalVariables|SetLocalFootstepEffectData _outdata)
              (Utilities|IsValid (Utilities|Struct|BreakSTR_FootstepEffectData (LocalVariables|GetLocalFootstepEffectData)) :!label _label
                (:Is%20Valid
                  (Effects|SpawnEmitteratLocation (Utilities|Struct|BreakSTR_FootstepEffectData (LocalVariables|GetLocalFootstepEffectData)) Location)))))
          (:then_1
            (bind (_success_2 _outdata_2) (CallFunction|FindFootstepDecalData (Utilities|Struct|BreakSTR_FootstepTypeData FootstepTypeData) SurfaceType))
            (if _success_2
              (LocalVariables|SetLocalFootstepDecalData _outdata_2))))
        (else
          (Utilities|FlowControl|Sequence
            (:then_0
              (bind (_success_3 _outdata_3) (CallFunction|FindFootstepEffectData (Utilities|Struct|BreakSTR_FootstepTypeData FootstepTypeData) SurfaceType))
              (if _success_3
                (LocalVariables|SetLocalFootstepEffectData _outdata_3)
                (goto _label)))
            (:then_1
              (bind (_success_4 _outdata_4) (CallFunction|FindFootstepDecalData (Utilities|Struct|BreakSTR_FootstepTypeData FootstepTypeData) SurfaceType))
              (if _success_4
                (LocalVariables|SetLocalFootstepDecalData _outdata_4)
                (Utilities|IsValid (.DecalMaterial (Utilities|Struct|BreakSTR_FootstepDecalData (LocalVariables|GetLocalFootstepDecalData)))
                  (:Is%20Valid
                    (Rendering|Decal|SpawnDecalatLocation (.DecalMaterial (Utilities|Struct|BreakSTR_FootstepDecalData (LocalVariables|GetLocalFootstepDecalData))) (.DecalSize (Utilities|Struct|BreakSTR_FootstepDecalData (LocalVariables|GetLocalFootstepDecalData))) Location (Math|Rotator|MakeRotator 9e+01 -9e+01 (.yaw (Transformation|GetActorRotation (Variables|State|References|GetCharacter)))) (.DecalLifeSpan (Utilities|Struct|BreakSTR_FootstepDecalData (LocalVariables|GetLocalFootstepDecalData))))))))))))
    (:then_1
      (return true))))

(fn CalculateIK
  (params (DeltaTime :type Float%20%28single-precision%29))
  (bind _characterskeletalmesh (Variables|State|References|GetCharacterSkeletalMesh))
  (bind _returnvalue (Transformation|GetWorldLocation _characterskeletalmesh))
  ;[1 1 1] Calculate and update IK bone variables.
  (if (Variables|State|Footsteps|GetSettingsAreCorrect)
    (bind _output_get (LocalVariables|SetLocalFootLocation (Transformation|GetSocketLocation _characterskeletalmesh (Variables|Settings|IK|GetIK_FootSocket))))
    (bind (_outhit _returnvalue_2) (Collision|LineTraceByChannel (Math|Vector|MakeVector (.x _output_get) (.y _output_get) (+ (Variables|Settings|IK|GetIK_TraceStartOffset) (.z _returnvalue))) (Math|Vector|MakeVector (.x _output_get) (.y _output_get) (+ (Variables|Settings|IK|GetIK_TraceEndOffset) (.z _returnvalue))) "TraceTypeQuery1" false (Utilities|Array|MakeArray (Components|GetOwner)) (select (Variables|Settings|Debug|GetDebugIK) "ForDuration" "None") true "(R=1.000000,G=0.000000,B=0.000000,A=1.000000)" "(R=0.000000,G=1.000000,B=0.000000,A=1.000000)" (Variables|Settings|Debug|GetDebugTraceTime)))
    (if _returnvalue_2
      (Variables|State|IK|SetIK_BoneTargetRotation (Math|Rotator|MakeRotator (Math|Float|Clamp(Float) (Class|KismetMathLibrary|DegAtan2 (.y (.Normal (Collision|BreakHitResult _outhit))) (.z (.Normal (Collision|BreakHitResult _outhit)))) -1e+01 1e+01) (* (Math|Float|Clamp(Float) (Class|KismetMathLibrary|DegAtan2 (.x (.Normal (Collision|BreakHitResult _outhit))) (.z (.Normal (Collision|BreakHitResult _outhit)))) -3e+01 3e+01) -1.0) 0.0))
      (Variables|State|IK|SetIK_BoneTargetTranslation (Math|Float|Clamp(Float) (- (.z (.Location (Collision|BreakHitResult _outhit))) (.z _returnvalue)) -3e+01 2e+01))
      (else
        (Variables|State|IK|SetIK_BoneTargetRotation "0, 0, 0")
        (Variables|State|IK|SetIK_BoneTargetTranslation 0.0)))
    (Variables|State|IK|SetIK_BoneCurrentRotation (Math|Interpolation|RInterpTo (Variables|State|IK|GetIK_BoneCurrentRotation) (Variables|State|IK|GetIK_BoneTargetRotation) DeltaTime (Variables|Settings|IK|GetIK_BoneRotationInterpSpeed)))
    (Variables|State|IK|SetIK_BoneCurrentTranslation (Math|Interpolation|FInterpTo (Variables|State|IK|GetIK_BoneCurrentTranslation) (Variables|State|IK|GetIK_BoneTargetTranslation) DeltaTime (Variables|Settings|IK|GetIK_BoneTranslationInterpSpeed)))
    (return true)
    (else
      (return false))))

(fn GetTwoLegsPelvisBoneTranslation
  (params (RightFootstepComponent :type BP%20Footstep%20Component%20Object%20Reference))
  (bind _ik_bonecurrenttranslation (Variables|BP_FootstepComponent_C|GetIK_BoneCurrentTranslation RightFootstepComponent))
  (bind _ik_bonecurrenttranslation_2 (Variables|State|IK|GetIK_BoneCurrentTranslation))
  ;[1 1 1] Returns the translation of the pelvis bone for a character with two legs.
  (Utilities|IsValid RightFootstepComponent
    (:Is%20Valid
      (return true (select (> _ik_bonecurrenttranslation_2 _ik_bonecurrenttranslation) _ik_bonecurrenttranslation _ik_bonecurrenttranslation_2)))
    (:Is%20Not%20Valid
      (return false 0.0))))

(fn GetFootBoneRotationandTranslation
  ;[1 1 1] Returns the translation and rotation IK variables.
  (return (Variables|State|IK|GetIK_BoneCurrentRotation) (Variables|State|IK|GetIK_BoneCurrentTranslation)))

(fn MakeNoise
  (params (Location :type Vector) (FootstepType :type E_FootstepType%20Enum :default "NewEnumerator7"))
  ;[1 1 1] Make noise in target location.
  (Class|Actor|MakeNoise (Components|GetOwner) 1.0 0 Location (Utilities|Select :Index FootstepType :NewEnumerator7 1e+03 :NewEnumerator8 3e+02 :NewEnumerator1 6e+02 :NewEnumerator2 1e+03 :NewEnumerator5 6e+02 :NewEnumerator6 1e+03) "None")
  (return true))