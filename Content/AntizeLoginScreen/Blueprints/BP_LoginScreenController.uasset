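; Player controller for the login screen that creates W_LoginScreen, puts it on the viewport and switches to UI-only input with a visible cursor.
; It also drives the widget's text animation, hosting the timeline here because widgets cannot run one.
; Each cycle has the widget pick a random animation, feeds it the timeline alpha, then repeats after a short delay.
; PauseAnimation stops the timeline.
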(event Custom|CallAnimation
  (bind _loginscreenref (Variables|Default|GetLoginScreenRef))
  (bind _loginscreenref_2 (Variables|Default|GetLoginScreenRef))
  ;[1 1 1] Timeline here because it can't be called in a widget
  (Utilities|IsValid _loginscreenref
    (:Is%20Valid
      (Default|GetRandomAnimation _loginscreenref)
      (bind _alpha (Timeline|MyAnimation PlayFromStart)
        (:Update
          (Utilities|IsValid _loginscreenref_2
            (:Is%20Valid
              (Default|DoTextAnimation _loginscreenref_2 _alpha))))
        (:Finished
          (Utilities|FlowControl|Delay 2.0)
          (CallFunction|CallAnimation))))))

(event Custom|PauseAnimation
  (bind _loginscreenref (Variables|Default|GetLoginScreenRef))
  ;[1 1 1] Timeline here because it can't be called in a widget
  (bind _alpha (Timeline|MyAnimation Stop)
    (:Update
      (Utilities|IsValid _loginscreenref
        (:Is%20Valid
          (Default|DoTextAnimation _loginscreenref _alpha))))
    (:Finished
      (Utilities|FlowControl|Delay 2.0)
      (CallFunction|CallAnimation))))

(event EventBeginPlay
  ;[1 1 1] Create the LoginScreen widget and call the text animation
  (bind _returnvalue (UserInterface|CreateWidget "/Game/AntizeLoginScreen/Widgets/W_LoginScreen.W_LoginScreen_C"))
  (bind _output_get (Variables|Default|SetLoginScreenRef _returnvalue))
  (UserInterface|Viewport|AddtoViewport _output_get 999999)
  (Input|SetInputModeUIOnly self (Variables|Default|GetLoginScreenRef) "DoNotLock" false)
  (Variables|Default|SetbShowMouseCursor self true)
  (CallFunction|CallAnimation))

(fn ConstructionScript)