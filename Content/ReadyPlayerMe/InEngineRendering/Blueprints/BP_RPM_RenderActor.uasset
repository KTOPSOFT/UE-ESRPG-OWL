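; BP_RPM_RenderActor loads a Ready Player Me avatar from a URL and renders it in-engine into a material.
; A SceneCaptureComponent2D limited to the actor's own components writes to a runtime render target, fed into a uniquely named dynamic instance of M_DynamicTargetMat.
; With CaptureAnimation on, it captures continuously; otherwise it captures one frame and destroys itself.
; Both paths pass the material to OnCaptured listeners.
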(event Custom|OnLoadCompleted
  (bind _captureanimation (Variables|Default|GetCaptureAnimation))
  (bind _scenecapturecomponent2d (Variables|Default|GetSceneCaptureComponent2D))
  ;[1 1 1] Create render target and connect it with the material instance
  (bind _returnvalue (Rendering|CreateRenderTarget2D 1024 1024 "RTF_RGBA16f"))
  (bind _output_get (Variables|/Script/Engine.SceneCaptureComponent2D|SetTextureTarget (Variables|Default|GetSceneCaptureComponent2D) _returnvalue))
  (bind _returnvalue_2 (Rendering|Material|CreateDynamicMaterialInstance "/Game/ReadyPlayerMe/InEngineRendering/Materials/M_DynamicTargetMat.M_DynamicTargetMat" (Utilities|String|StringToName (Utilities|String|Append "RenderCharacter" (Utilities|String|ToString(Integer) (Class|KismetMathLibrary|RandomInteger64 10000000)))) "None" :!class /Script/Engine.KismetMaterialLibrary))
  (Rendering|Material|SetTextureParameterValue _returnvalue_2 "RenderTexture" _output_get)
  (Variables|Default|SetRenderTargetMaterial _returnvalue_2)
  ;[1 1 1] Enable the scene capture component
  (Development|SetHiddeninGame _scenecapturecomponent2d false false)
  (Rendering|SetVisibility _scenecapturecomponent2d true false)
  (Variables|/Script/Engine.SceneCaptureComponent|SetbCaptureEveryFrame _scenecapturecomponent2d _captureanimation)
  (Variables|/Script/Engine.SceneCaptureComponent|SetbCaptureOnMovement _scenecapturecomponent2d _captureanimation)
  ;[1 1 1] Capture image or animation
  (if _captureanimation
    (Default|CallOnCaptured (Variables|Default|GetRenderTargetMaterial))
    (else
      (Rendering|SceneCapture|CaptureScene (Variables|Default|GetSceneCaptureComponent2D) :!class /Script/Engine.SceneCaptureComponent2D)
      (Default|CallOnCaptured (Variables|Default|GetRenderTargetMaterial))
      (Actor|DestroyActor))))

(event Custom|LoadRender
  (params (CaptureAnimation :type Boolean) (Url :type String))
  ;[1 1 1] Load the avatar and set the Capture component to only record the actor components
  (Variables|Default|SetCaptureAnimation CaptureAnimation)
  (Class|ReadyPlayerMeComponent|LoadNewAvatar (Variables|Default|GetReadyPlayerMe) Url (delegate Custom|OnLoadCompleted))
  (Rendering|SceneCapture|ShowOnlyActorComponents (Variables|Default|GetSceneCaptureComponent2D) self false))

(fn ConstructionScript)