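; Multiplayer player controller for Ready Player Me that syncs each player's avatar URL to their character and manages the avatar loader panel.
; On possession, the authority asks the local client for the URL stored in the game instance, then sets it server-side on the character's RepNotify variable.
; A session setup widget submits new URLs through the same path.
; Q toggles the widget, switching pawn input, input mode and cursor.
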(event Custom|OnCloseLoader
  ;[1 1 1] Bind Panel Close Button Event
  (CallFunction|ToggleLoader))

(event Custom|CallAvatarLoadServer
  (params (Url :type String))
  ;[1 1 1] Bind Load Button Event To RPM Character Load Avatar Server
  (CallFunction|SetNewAvatarUrl Url))

(event Custom|SetAvatarLocal
  ;[1 1 1] From The Local Client Get The Avatar Id From The Game Instance And Set The Avatar In In The Server
  (bind _asgi_rpm_instance (Utilities|Casting|CastToGI_RPM_Instance (Game|GetGameInstance)))
  (CallFunction|SetAvatarServer (Variables|/Game/ReadyPlayerMe/Multiplayer/Blueprints/GI_RPM_Instance.GI_RPM_Instance_C|GetAvatarUrl _asgi_rpm_instance)))

(event Custom|SetAvatarServer
  (params (Url :type String))
  ;[1 1 1] When The Avatar Url Is Set In The Server Set The Avatar Url RepNotify Parameter Of The Character
  (bind _asbp_rpm_multiplayer_character (Utilities|Casting|CastToBP_RPM_MultiplayerCharacter (Pawn|GetControlledPawn)))
  (Variables|/Game/ReadyPlayerMe/Multiplayer/Blueprints/BP_RPM_MultiplayerCharacter.BP_RPM_MultiplayerCharacter_C|SetAvatarUrl _asbp_rpm_multiplayer_character Url))

(event EventBeginPlay
  (Utilities|FlowControl|Sequence
    (:then_0
      ;[1 1 1] Create Loader Widget
      (bind _returnvalue (UserInterface|CreateWidget "/Game/ReadyPlayerMe/Multiplayer/Widgets/WBP_SessionSetup.WBP_SessionSetup_C" (Game|GetPlayerController 0)))
      (bind _output_get (Variables|Default|SetAvatarLoaderWidget _returnvalue))
      (UserInterface|Viewport|AddtoViewport _output_get 0)
      (Default|SetLoaderVisibility (Variables|Default|GetAvatarLoaderWidget) "Hidden"))
    (:then_1
      ;[1 1 1] Bind Load Button Event To RPM Character Load Avatar Server
      (EventDispatchers|BindEventtoOnLoadUrl (Variables|Default|GetAvatarLoaderWidget) (delegate Custom|CallAvatarLoadServer))
      ;[1 1 1] Bind Panel Close Button Event
      (EventDispatchers|BindEventtoOnCloseLoaderPanel (Variables|Default|GetAvatarLoaderWidget) (delegate Custom|OnCloseLoader)))))

(event EventPossess
  (params (PossessedPawn :type Pawn%20Object%20Reference))
  ;[1 1 1] When OnPossess Is Called On The Server Load The Avatar On The Local Client
  (Networking|SwitchHasAuthority
    (:Authority
      (CallFunction|SetAvatarLocal))))

(event Input|KeyboardEvents|Q
  (params (Key :type Key%20Structure))
  ;[1 1 1] Input to toggle loader panel
  (:Pressed
    (CallFunction|ToggleLoader)))

(fn ConstructionScript)

(fn ToggleLoader
  (bind _returnvalue (Pawn|GetControlledPawn))
  (bind _self self)
  (bind _avatarloaderwidget (Variables|Default|GetAvatarLoaderWidget))
  (bind _avatarloaderwidget_2 (Variables|Default|GetAvatarLoaderWidget))
  ;[1 1 1] Set Panel Visibility
  (Utilities|IsValid _avatarloaderwidget
    (:Is%20Valid
      (if (Utilities|Enum|Equal(Enum) (Widget|GetVisibility (Variables|/Game/ReadyPlayerMe/Multiplayer/Widgets/WBP_SessionSetup.WBP_SessionSetup_C|GetSessionsBorder _avatarloaderwidget)) "Visible")
        (Default|SetLoaderVisibility _avatarloaderwidget_2 "Hidden")
        ;[1 1 1] Set Input Mode and Cursor
        (Input|EnableInput _returnvalue _self)
        (Input|SetInputModeGameOnly _self false)
        (Variables|Default|SetbShowMouseCursor false)
        (else
          (Default|SetLoaderVisibility _avatarloaderwidget_2 "Visible")
          (Input|DisableInput _returnvalue _self)
          (Input|SetInputModeGameandUI _self (Variables|Default|GetAvatarLoaderWidget) "DoNotLock" true false)
          (Variables|Default|SetbShowMouseCursor true))))))

(fn SetNewAvatarUrl
  (params (AvatarUrl :type String))
  (bind _asgi_rpm_instance (Utilities|Casting|CastToGI_RPM_Instance (Game|GetGameInstance)))
  (bind _output_get (Variables|/Game/ReadyPlayerMe/Multiplayer/Blueprints/GI_RPM_Instance.GI_RPM_Instance_C|SetAvatarUrl _asgi_rpm_instance AvatarUrl))
  (CallFunction|SetAvatarServer _output_get))