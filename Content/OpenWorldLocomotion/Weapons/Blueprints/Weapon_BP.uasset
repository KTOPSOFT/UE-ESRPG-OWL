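; Weapon actor for the locomotion system that builds its visuals from an overlay data asset and attaches to a socket on a parent mesh.
; The construction script adds collision-free static and skeletal mesh components using the data's meshes and transforms.
; BeginPlay attaches it and caches whether the instigator is locally controlled.
; For local, aimable weapons, Tick interpolates WeaponRotation from the look-at between AimTarget and the Arrow, for screen-center aiming.
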(event EventBeginPlay
  (bind _returnvalue (Game|GetInstigator))
  (Transformation|AttachComponentToComponent (Variables|Default|GetParentMesh) (Variables|Variables|GetSocket%20Name) "SnapToTarget" "SnapToTarget" "SnapToTarget" false)
  (Utilities|IsValid _returnvalue
    (:Is%20Valid
      (Variables|DoNotModify|SetLocalyControlled (Pawn|IsLocallyControlled _returnvalue)))))

(event EventTick
  (params (DeltaSeconds :type Float%20%28single-precision%29))
  ;[1 1 1] Logic used to point your weapon at the location in the middle of the screen
  (if (and (Variables|DoNotModify|GetLocalyControlled) (Variables|DoNotModify|GetCanBeAimed))
    (Variables|DoNotModify|SetWeaponRotation (Math|Interpolation|RInterpTo (Variables|DoNotModify|GetWeaponRotation) (Math|Rotator|FindLookatRotation (Variables|Variables|GetAimTarget) (Transformation|GetWorldLocation (Variables|Default|GetArrow))) (Utilities|Time|GetWorldDeltaSeconds) 5e+01))))

(fn ConstructionScript
  (Variables|Default|GetOverlayData
    (:then
      (Utilities|FlowControl|Sequence
        (:then_0
          (if (Variables|/Game/OpenWorldLocomotion/Data/DataAsset/AnimOverlay_PDA.AnimOverlay_PDA_C|GetAddStaticMesh (Variables|Default|GetOverlayData))
            (for (_array_element _array_index) (Variables|/Game/OpenWorldLocomotion/Data/DataAsset/AnimOverlay_PDA.AnimOverlay_PDA_C|GetStaticMesh (Variables|Default|GetOverlayData))
              (bind _returnvalue (AddComponent|AddStaticMeshComponent false (Utilities|Array|Get(acopy) (Variables|/Game/OpenWorldLocomotion/Data/DataAsset/AnimOverlay_PDA.AnimOverlay_PDA_C|GetStaticMeshTransform (Variables|Default|GetOverlayData)) _array_index)))
              (Components|StaticMesh|SetStaticMesh _returnvalue _array_element)
              (Collision|SetCollisionEnabled _returnvalue "NoCollision"))))
        (:then_1
          (if (Variables|/Game/OpenWorldLocomotion/Data/DataAsset/AnimOverlay_PDA.AnimOverlay_PDA_C|GetAddSkeletalMesh (Variables|Default|GetOverlayData))
            (for (_array_element_2 _array_index_2) (Variables|/Game/OpenWorldLocomotion/Data/DataAsset/AnimOverlay_PDA.AnimOverlay_PDA_C|GetSkeletalMesh (Variables|Default|GetOverlayData))
              (bind _returnvalue_2 (AddComponent|AddSkeletalMeshComponent false (Utilities|Array|Get(acopy) (Variables|/Game/OpenWorldLocomotion/Data/DataAsset/AnimOverlay_PDA.AnimOverlay_PDA_C|GetSkeletalMeshTransform (Variables|Default|GetOverlayData)) _array_index_2)))
              (Components|SkinnedMesh|SetSkinnedAssetandUpdate _returnvalue_2 _array_element_2 true)
              (Collision|SetCollisionEnabled _returnvalue_2 "NoCollision"))))))
    (:else)))