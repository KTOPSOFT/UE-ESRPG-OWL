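; Player character for the Open World Locomotion system, adding example weapon overlays, camera switching, a pause menu and HUD prompts.
; Switching weapons cycles animation overlays, whose enable event spawns or destroys the weapon and starts or stops hand IK.
; Timelines act as update loops for hand IK and the screen-center aim trace that feeds the weapon's target.
; Tick eases the camera back while sprinting and refreshes climb and vault prompts.
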(event Custom|SwitchWeapon
  ;[1 0 1] Switch weapon (example)
  (bind _output_get (Variables|Variables|SetCurrentOverlay (Utilities|Array|Get(acopy) (Variables|Default|GetWeapons) (Math|Integer|SelectInt (+ (Utilities|Array|FindItem (Variables|Default|GetWeapons) (Variables|Variables|GetCurrentOverlay)) 1) 0 (Utilities|Array|IsValidIndex (Variables|Default|GetWeapons) (+ (Utilities|Array|FindItem (Variables|Default|GetWeapons) (Variables|Variables|GetCurrentOverlay)) 1))))))
  (CallFunction|BPISwitchOverlay _output_get))

(event Input|EnhancedActionEvents|EnhancedInputActionIA_ChangeCamera
  (params (ActionValue :type Boolean) (ElapsedSeconds :type Float%20%28double-precision%29) (TriggeredSeconds :type Float%20%28double-precision%29) (InputAction :type Input%20Action%20Object%20Reference :default "/Game/OpenWorldLocomotion/Data/Inputs/IA_ChangeCamera.IA_ChangeCamera"))
  ;[1 1 1] ChangeCamera
  (:Triggered
    (switch Utilities|FlowControl|Switch|SwitchonE_CameraType (Variables|/Game/OpenWorldLocomotion/CharacterComponents/OWL_BaseComponent_BP.OWL_BaseComponent_BP_C|GetCameraType (Variables|Default|GetOWL_BaseComponent_BP))
      (:NewEnumerator0
        (Components|Activation|Deactivate (Variables|Default|GetFPC))
        (Components|Activation|Activate (Variables|Default|GetTPC) true))
      (:NewEnumerator1
        (Components|Activation|Deactivate (Variables|Default|GetTPC))
        (Components|Activation|Activate (Variables|Default|GetFPC) true)))))

(event Input|EnhancedActionEvents|EnhancedInputActionIA_Menu
  (params (ActionValue :type Boolean) (ElapsedSeconds :type Float%20%28double-precision%29) (TriggeredSeconds :type Float%20%28double-precision%29) (InputAction :type Input%20Action%20Object%20Reference :default "/Game/OpenWorldLocomotion/Data/Inputs/IA_Menu.IA_Menu"))
  ;[1 1 1] HUD
  (:Triggered
    (bind _menu (Variables|HUD|GetMenu)
      (:then
        (Widget|RemovefromParent _menu)
        (Variables|HUD|SetMenu 0)
        (Variables|/Script/Engine.PlayerController|SetbShowMouseCursor (Game|GetPlayerController 0) false)
        (Game|SetGamePaused false))
      (:else
        (bind _returnvalue (UserInterface|CreateWidget "/Game/OpenWorldLocomotion/HUD/Menu_Widget.Menu_Widget_C"))
        (bind _output_get (Variables|HUD|SetMenu _returnvalue))
        (UserInterface|Viewport|AddtoViewport _output_get 0)
        (Variables|/Script/Engine.PlayerController|SetbShowMouseCursor (Game|GetPlayerController 0) true)
        (Game|SetGamePaused true)))))

(event Input|EnhancedActionEvents|EnhancedInputActionIA_SwitchWeapon
  (params (ActionValue :type Boolean) (ElapsedSeconds :type Float%20%28double-precision%29) (TriggeredSeconds :type Float%20%28double-precision%29) (InputAction :type Input%20Action%20Object%20Reference :default "/Game/OpenWorldLocomotion/Data/Inputs/IA_SwitchWeapon.IA_SwitchWeapon"))
  ;[1 0 1] Switch weapon (example)
  (:Triggered
    (CallFunction|SwitchWeapon)))

(event EventBPIonOverlayEnabled
  (params (Enable :type Boolean))
  ;[1 0 1] Spawning a weapon (example)
  (|CallParentFunction Enable)
  (|Spawn/DespawnWeapon_Graph Enable))

(event EventBPIIsAiming
  (params (Aiming :type Boolean))
  ;[1 0 1] Aim weapon (example)
  (if Aiming
    (Components|Timeline|PlayfromStart (Variables|Default|GetAimingTrace_Timeline))
    (CallFunction|BPIModifyMovementSpeed true 1.5e+02 true)
    (else
      (Audio|Components|Audio|Stop (Variables|Default|GetAimingTrace_Timeline))
      (CallFunction|BPIModifyMovementSpeed false 0.0 false)
      (bind _currentweapon (Variables|Variables|GetCurrentWeapon)
        (:then
          (Variables|/Game/OpenWorldLocomotion/Weapons/Blueprints/Weapon_BP.Weapon_BP_C|SetUseAimTarget _currentweapon false))
        (:else)))))

(event EventTick
  (params (DeltaSeconds :type Float%20%28single-precision%29))
  ;[1 1 1] Tick event
  (|CallParentFunction DeltaSeconds)
  (Utilities|SprintCamera) ; Moves third person camera back when sprinting
  ;;[1 1 1] Screen Prompts (HUD)
  (|ManualClimbingScreenPrompt)
  (|VaultingScreenPrompt))

(event EventBeginPlay
  ;[1 1 1] Begin Play event
  (|CallParentFunction)
  (bind _foundwidgets (Widget|GetAllWidgetsOfClass "/Game/OpenWorldLocomotion/HUD/HUD_Widget.HUD_Widget_C" true))
  (Variables|HUD|SetHUD (Utilities|Array|Get(acopy) _foundwidgets))
  (CallFunction|SwitchWeapon))

(fn ConstructionScript
  (|CallParentFunction))