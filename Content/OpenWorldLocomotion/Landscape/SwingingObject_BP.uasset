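; Swinging obstacle actor whose static mesh rocks back and forth and ragdolls any Character that overlaps its capsule.
; On BeginPlay, a timeline with length set by Time eases the mesh's relative rotation between LocalMaxRotation and its negation.
; Each time the timeline finishes, it flips the Return flag and replays, swapping the endpoints for continuous pendulum motion.
; Capsule overlaps send a ragdoll interface message to the Character.
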(event OnComponentBeginOverlap(Capsule)
  (params (OverlappedComponent :type Primitive%20Component%20Object%20Reference) (OtherActor :type Actor%20Object%20Reference) (OtherComp :type Primitive%20Component%20Object%20Reference) (OtherBodyIndex :type Integer) (bFromSweep :type Boolean) (SweepResult :type Hit%20Result%20Structure%20%28by%20ref%29))
  (bind _ascharacter (Utilities|Casting|CastToCharacter OtherActor))
  (Class|OWLInterfaceBPI|BPIRagdoll(Message) _ascharacter true))

(event EventBeginPlay
  (bind _localmaxrotation (Variables|Default|GetLocalMaxRotation))
  (bind _timeline_0 (Variables|Default|GetTimeline_0))
  (bind _returnvalue (Class|KismetMathLibrary|NegateRotator _localmaxrotation))
  (Transformation|SetRelativeRotation (Variables|Default|GetStaticMesh) (Variables|Default|GetLocalMaxRotation) false false)
  (Components|Timeline|SetTimelineLength (Variables|Default|GetTimeline_0) (Variables|Default|GetTime))
  (Timeline|Timeline_0 PlayFromStart
    (:Update
      (Transformation|SetRelativeRotation (Variables|Default|GetStaticMesh) (Math|Interpolation|Ease "EaseInOut" (/ (Components|Timeline|GetPlaybackPosition _timeline_0) (Components|Timeline|GetTimelineLength _timeline_0)) (Math|Rotator|SelectRotator _localmaxrotation _returnvalue (Variables|Default|GetReturn)) (Math|Rotator|SelectRotator _returnvalue _localmaxrotation (Variables|Default|GetReturn)) true) false false))
    (:Finished
      (Variables|Default|SetReturn (not (Variables|Default|GetReturn)))
      (Timeline|Timeline_0 PlayFromStart))))

(fn ConstructionScript)