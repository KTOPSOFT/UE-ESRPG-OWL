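; Moving piston hazard that slides back and forth and ragdolls any Character that overlaps its box.
; After an initial delay, a timeline of configurable length eases the piston mesh along local Y by Distance with an ExpoIn curve.
; The Return flag swaps the endpoints on each finish, pausing only after the return stroke.
; Box overlaps send the ragdoll interface message to the Character.
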(event OnComponentBeginOverlap(Box)
  (params (OverlappedComponent :type Primitive%20Component%20Object%20Reference) (OtherActor :type Actor%20Object%20Reference) (OtherComp :type Primitive%20Component%20Object%20Reference) (OtherBodyIndex :type Integer) (bFromSweep :type Boolean) (SweepResult :type Hit%20Result%20Structure%20%28by%20ref%29))
  (bind _ascharacter (Utilities|Casting|CastToCharacter OtherActor))
  (Class|OWLInterfaceBPI|BPIRagdoll(Message) _ascharacter true))

(event EventBeginPlay
  (bind _distance (Variables|Default|GetDistance))
  (bind _timeline_0 (Variables|Default|GetTimeline_0))
  (Components|Timeline|SetTimelineLength (Variables|Default|GetTimeline_0) (Variables|Default|GetTime))
  (Utilities|FlowControl|Delay (Variables|Default|GetInitialDelay))
  (Timeline|Timeline_0 PlayFromStart
    (:Update
      (Transformation|SetRelativeLocation (Variables|Default|GetPiston) (Math|Interpolation|Ease "ExpoIn" (/ (Components|Timeline|GetPlaybackPosition _timeline_0) (Components|Timeline|GetTimelineLength _timeline_0)) (Math|Vector|SelectVector (Math|Vector|MakeVector 0.0 _distance 0.0) "0, 0, 0" (Variables|Default|GetReturn)) (Math|Vector|SelectVector "0, 0, 0" (Math|Vector|MakeVector 0.0 _distance 0.0) (Variables|Default|GetReturn))) false false))
    (:Finished
      (if (Variables|Default|GetReturn)
        (Variables|Default|SetReturn false)
        (Utilities|FlowControl|Delay (Variables|Default|GetDelay))
        (Timeline|Timeline_0 PlayFromStart)
        (else
          (Variables|Default|SetReturn true)
          (Timeline|Timeline_0 PlayFromStart))))))

(event Collision|EventActorBeginOverlap
  (params (OtherActor :type Actor%20Object%20Reference)))

(fn ConstructionScript)