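; Ladder actor that switches overlapping characters into a climbing mode through their OWL_Climbing_BP component.
; Its construction script stores a self reference in LadderData alongside the step height and first step height.
; On entering ClimbingModeVolume, a Character's climbing component receives that LadderData and a new ClimbingMode.
; Leaving the volume sets ClimbingMode back to the enum's first entry, without clearing the ladder data.
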(event OnComponentBeginOverlap(ClimbingModeVolume)
  (params (OverlappedComponent :type Primitive%20Component%20Object%20Reference) (OtherActor :type Actor%20Object%20Reference) (OtherComp :type Primitive%20Component%20Object%20Reference) (OtherBodyIndex :type Integer) (bFromSweep :type Boolean) (SweepResult :type Hit%20Result%20Structure%20%28by%20ref%29))
  (bind _ascharacter (Utilities|Casting|CastToCharacter OtherActor))
  (Variables|/Game/OpenWorldLocomotion/CharacterComponents/SystemComponents/OWL_Climbing_BP.OWL_Climbing_BP_C|SetLadderData (Actor|GetComponentbyClass _ascharacter "/Game/OpenWorldLocomotion/CharacterComponents/SystemComponents/OWL_Climbing_BP.OWL_Climbing_BP_C") (Variables|Default|GetLadderData))
  (Variables|/Game/OpenWorldLocomotion/CharacterComponents/SystemComponents/OWL_Climbing_BP.OWL_Climbing_BP_C|SetClimbingMode (Actor|GetComponentbyClass _ascharacter "/Game/OpenWorldLocomotion/CharacterComponents/SystemComponents/OWL_Climbing_BP.OWL_Climbing_BP_C") "NewEnumerator1"))

(event OnComponentEndOverlap(ClimbingModeVolume)
  (params (OverlappedComponent :type Primitive%20Component%20Object%20Reference) (OtherActor :type Actor%20Object%20Reference) (OtherComp :type Primitive%20Component%20Object%20Reference) (OtherBodyIndex :type Integer))
  (bind _ascharacter (Utilities|Casting|CastToCharacter OtherActor))
  (Variables|/Game/OpenWorldLocomotion/CharacterComponents/SystemComponents/OWL_Climbing_BP.OWL_Climbing_BP_C|SetClimbingMode (Actor|GetComponentbyClass _ascharacter "/Game/OpenWorldLocomotion/CharacterComponents/SystemComponents/OWL_Climbing_BP.OWL_Climbing_BP_C") "NewEnumerator0"))

(fn ConstructionScript
  (Variables|Default|SetLadderData (Utilities|Struct|MakeLadderData_Struct self (.stepheight (Variables|Default|GetLadderData)) (.firststepheight (Variables|Default|GetLadderData)))))