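; Kill box volume that relocates any Character overlapping its box instead of killing it.
; On overlap it sends the character a ragdoll interface message set to false, then fades the first player's camera to black.
; After a short delay it teleports the character to the Teleporter actor, or the first PlayerStart found if none is valid, and fades the view back in.
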(event OnComponentBeginOverlap(Box)
  (params (OverlappedComponent :type Primitive%20Component%20Object%20Reference) (OtherActor :type Actor%20Object%20Reference) (OtherComp :type Primitive%20Component%20Object%20Reference) (OtherBodyIndex :type Integer) (bFromSweep :type Boolean) (SweepResult :type Hit%20Result%20Structure%20%28by%20ref%29))
  (bind _ascharacter (Utilities|Casting|CastToCharacter (Components|GetOwner OtherComp)))
  (Class|OWLInterfaceBPI|BPIRagdoll(Message) _ascharacter false)
  (CameraFades|StartCameraFade :self (Game|GetPlayerCameraManager 0) :ToAlpha 1.0 :Duration 0.2 :bHoldWhenFinished true)
  (Utilities|FlowControl|Delay 0.2)
  (bind _teleporter (Variables|Default|GetTeleporter)
    (:then
      (Transformation|SetActorLocation _ascharacter (Transformation|GetActorLocation _teleporter) false true))
    (:else
      (bind _outactors (Actor|GetAllActorsOfClass "/Script/Engine.PlayerStart"))
      (Transformation|SetActorLocation _ascharacter (Transformation|GetActorLocation (Utilities|Array|Get(acopy) _outactors)) false true)))
  (CameraFades|StartCameraFade :self (Game|GetPlayerCameraManager 0) :FromAlpha 1.0 :Duration 0.5))

(event EventBeginPlay)

(event EventTick
  (params (DeltaSeconds :type Float%20%28single-precision%29)))

(fn ConstructionScript)