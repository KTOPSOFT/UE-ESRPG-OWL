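; Swimming component for the Open World Locomotion system, driving a character's speed, gait, diving and surfacing in the swimming locomotion state.
; State changes apply or restore movement settings, while Tick updates gait, keeps the character upright and checks depth and obstacles.
; Water height comes from an interface message or fallback line trace, switching buoyancy and rotation rate.
; Input vectors follow camera pitch for diving, honor surface-only mode and shrink on sphere-trace hits.
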(event EventBeginPlay
  ;[0 0 1] Initialize component
  (|CallParentFunction)
  (Initialization|Initialize))

(event EventTick
  (params (DeltaSeconds :type Float%20%28single-precision%29))
  (|CallParentFunction DeltaSeconds)
  (if (not (Variables|/Game/OpenWorldLocomotion/CharacterComponents/OWL_BaseComponent_BP.OWL_BaseComponent_BP_C|GetBlockLocomotionLogic (Variables|Default|GetBaseComponent)))
    (if (Utilities|Enum|Equal(Enum) (Variables|/Game/OpenWorldLocomotion/CharacterComponents/OWL_BaseComponent_BP.OWL_BaseComponent_BP_C|GetLocomotionState (Variables|Default|GetBaseComponent)) "NewEnumerator7")
      (|CanGetSurfaceData_Graph
        (:OutputPin
          (Swimming|SwimmingLogic)))
      (elif (Variables|/Script/Engine.PhysicsVolume|GetbWaterVolume (Class|MovementComponent|GetPhysicsVolume (Variables|Default|GetCharacterMovement)))
        (Swimming|CheckIsUnderwater)))))

(fn ChangeGait
  (if (not (Math|Vector|VectorIsZero (Transformation|GetVelocity (Variables|Default|GetCharacter))))
    (LocalVariables|SetPreviousGait_Loc (Variables|/Game/OpenWorldLocomotion/CharacterComponents/OWL_BaseComponent_BP.OWL_BaseComponent_BP_C|GetGait (Variables|Default|GetBaseComponent)))
    (Utilities|FlowControl|Sequence
      (:then_0
        ;[1 1 1] Change gait for swimming based on current velocity
        (if (Variables|/Game/OpenWorldLocomotion/CharacterComponents/OWL_BaseComponent_BP.OWL_BaseComponent_BP_C|GetIsSprinting (Variables|Default|GetBaseComponent))
          (if (> (Math|Vector|VectorLength (Transformation|GetVelocity (Variables|Default|GetCharacter))) (+ (Variables|Swimming|GetMaxSwimSpeed) 2.0))
            (Variables|/Game/OpenWorldLocomotion/CharacterComponents/OWL_BaseComponent_BP.OWL_BaseComponent_BP_C|SetGait (Variables|Default|GetBaseComponent) "NewEnumerator1")
            (else
              (Variables|/Game/OpenWorldLocomotion/CharacterComponents/OWL_BaseComponent_BP.OWL_BaseComponent_BP_C|SetGait (Variables|Default|GetBaseComponent) "NewEnumerator0")))
          (else
            (Variables|/Game/OpenWorldLocomotion/CharacterComponents/OWL_BaseComponent_BP.OWL_BaseComponent_BP_C|SetGait (Variables|Default|GetBaseComponent) "NewEnumerator0"))))
      (:then_1
        (if (Utilities|Enum|NotEqual(Enum) (LocalVariables|GetPreviousGait_Loc) (Variables|/Game/OpenWorldLocomotion/CharacterComponents/OWL_BaseComponent_BP.OWL_BaseComponent_BP_C|GetGait (Variables|Default|GetBaseComponent)))
          (Default|CallOnGaitChanged (Variables|Default|GetBaseComponent) (Variables|/Game/OpenWorldLocomotion/CharacterComponents/OWL_BaseComponent_BP.OWL_BaseComponent_BP_C|GetGait (Variables|Default|GetBaseComponent))))))))

(fn ChangeMaxSpeed
  (if (Utilities|Enum|Equal(Enum) (Variables|/Game/OpenWorldLocomotion/CharacterComponents/OWL_BaseComponent_BP.OWL_BaseComponent_BP_C|GetLocomotionState (Variables|Default|GetBaseComponent)) "NewEnumerator7")
    (Variables|/Script/Engine.CharacterMovementComponent|SetMaxSwimSpeed (Variables|Default|GetCharacterMovement) (Math|Float|SelectFloat (Variables|Swimming|GetMaxSwimSprintSpeed) (Variables|Swimming|GetMaxSwimSpeed) (Variables|/Game/OpenWorldLocomotion/CharacterComponents/OWL_BaseComponent_BP.OWL_BaseComponent_BP_C|GetIsSprinting (Variables|Default|GetBaseComponent))))))

(fn SwimmingLogic
  (Swimming|ChangeGait)
  (Transformation|SetActorRotation (Variables|Default|GetCharacter) (Math|Rotator|MakeRotator 0.0 0.0 (.yaw (Transformation|GetActorRotation (Variables|Default|GetCharacter)))))
  (Swimming|CheckIsUnderwater)
  (|CheckForCollisions))

(fn MovementVectorSwimming
  (bind _character (Variables|Default|GetCharacter))
  (bind _usecameratodive (Variables|Swimming|GetUseCameraToDive))
  (bind _basecomponent (Variables|Default|GetBaseComponent))
  (bind _surfaceonly (Variables|Swimming|GetSurfaceOnly))
  (bind _returnvalue (Pawn|GetControlRotation _character :!class /Script/Engine.Pawn))
  (bind _isunderwater (Variables|/Game/OpenWorldLocomotion/CharacterComponents/OWL_BaseComponent_BP.OWL_BaseComponent_BP_C|GetIsUnderwater _basecomponent))
  (bind _returnvalue_2 (Math|Boolean|NORBoolean _usecameratodive _isunderwater))
  (bind _yaw (Math|Rotator|BreakRotator _returnvalue))
  (bind _returnvalue_3 (Math|Rotator|MakeRotator 0.0 0.0 _yaw))
  (bind _returnvalue_4 (or _surfaceonly _returnvalue_2))
  (bind _returnvalue_5 (Math|Rotator|SelectRotator _returnvalue_3 _returnvalue _returnvalue_4))
  (bind _returnvalue_6 (Math|Vector|GetForwardVector _returnvalue_5))
  (bind _returnvalue_7 (Math|Vector|GetRightVector _returnvalue_5))
  (return (Math|Vector|SelectVector (* _returnvalue_6 0.1) _returnvalue_6 (Variables|SwimmingVariables|GetCollision)) (Math|Vector|SelectVector (* _returnvalue_7 0.1) _returnvalue_7 (Variables|SwimmingVariables|GetCollision))))

(fn InputSwimUpDown
  (params (Axis :type Float%20%28double-precision%29))
  (bind _surfaceonly (Variables|Swimming|GetSurfaceOnly))
  (if (and (!= Axis 0.0) (Utilities|Enum|Equal(Enum) (Variables|/Game/OpenWorldLocomotion/CharacterComponents/OWL_BaseComponent_BP.OWL_BaseComponent_BP_C|GetLocomotionState (Variables|Default|GetBaseComponent)) "NewEnumerator7"))
    (if (or (<= Axis 0.0) (Variables|/Game/OpenWorldLocomotion/CharacterComponents/OWL_BaseComponent_BP.OWL_BaseComponent_BP_C|GetIsUnderwater (Variables|Default|GetBaseComponent)))
      (if (or (and (> Axis 0.0) _surfaceonly) (not _surfaceonly))
        (Pawn|Input|AddMovementInput (Variables|Default|GetCharacter) (+ (* (Class|KismetMathLibrary|VectorNormal2D (Transformation|GetActorForwardVector (Variables|Default|GetCharacter)) 0.0001) (* Axis 0.001)) (Math|Vector|MakeVector 0.0 0.0 1.0)) Axis false)
        (if (< Axis 0.0)
          (Variables|/Script/Engine.CharacterMovementComponent|SetBuoyancy (Variables|Default|GetCharacterMovement) (Variables|Swimming|GetUnderwaterBuoyancy)))))))

(fn IsUnderwaterFunction
  (params (IsUnderwater :type Boolean))
  (if IsUnderwater
    (if (Variables|Swimming|GetSurfaceOnly)
      (Variables|/Script/Engine.CharacterMovementComponent|SetBuoyancy (Variables|Default|GetCharacterMovement) (Variables|Swimming|GetSurfaceBuoyancy))
      (Variables|/Script/Engine.CharacterMovementComponent|SetRotationRate (Variables|Default|GetCharacterMovement) (Variables|Swimming|GetSurfaceRotationRate))
      (Input|InputSwimUpDown 1.0)
      (else
        (Variables|/Script/Engine.CharacterMovementComponent|SetBuoyancy (Variables|Default|GetCharacterMovement) (Variables|Swimming|GetUnderwaterBuoyancy))
        (Variables|/Script/Engine.CharacterMovementComponent|SetRotationRate (Variables|Default|GetCharacterMovement) (Variables|Swimming|GetUnderwaterRotationRate))))
    (else
      (Variables|/Script/Engine.CharacterMovementComponent|SetBuoyancy (Variables|Default|GetCharacterMovement) (Variables|Swimming|GetSurfaceBuoyancy))
      (Variables|/Script/Engine.CharacterMovementComponent|SetRotationRate (Variables|Default|GetCharacterMovement) (Variables|Swimming|GetSurfaceRotationRate)))))

(fn CheckIsUnderwater
  (bind _character (Variables|Default|GetCharacter))
  (bind _character_2 (Variables|Default|GetCharacter))
  (bind _returnvalue (Transformation|GetActorLocation _character_2))
  (bind _capsulecomponent (Variables|/Script/Engine.Character|GetCapsuleComponent _character))
  (bind _capsulecomponent_2 (Variables|/Script/Engine.Character|GetCapsuleComponent _character_2))
  (bind _returnvalue_2 (Components|Capsule|GetScaledCapsuleHalfHeight _capsulecomponent))
  (bind _returnvalue_3 (Components|Capsule|GetScaledCapsuleHalfHeight _capsulecomponent_2))
  (Utilities|FlowControl|Sequence
    (:then_0
      (bind (_active _waterplanelocation _watersurfaceposition) (Class|OWLInterfaceBPI|BPIWaterSurfaceData(Message) (Variables|Default|GetCharacter)))
      (bind _output_get (Variables|SwimmingVariables|SetCanGetSurfaceData _active))
      (if (or _output_get (Variables|SwimmingVariables|GetGetSurfaceData))
        (Variables|SwimmingVariables|SetWaterPlaneHight (.z _waterplanelocation))
        (Variables|SwimmingVariables|SetWaterSurfaceHight (.z _watersurfaceposition))
        (else
          (bind _outhit (Collision|LineTraceForObjects (+ _returnvalue (Math|Vector|MakeVector 0.0 0.0 _returnvalue_3)) (- _returnvalue (Math|Vector|MakeVector 0.0 0.0 _returnvalue_3)) (Utilities|Array|MakeArray "ObjectTypeQuery1") false (Utilities|Array|MakeArray (Variables|Default|GetCharacter)) "None"))
          (bind _output_get_2 (Variables|SwimmingVariables|SetWaterPlaneHight (.Z (Math|Vector|BreakVector (.ImpactPoint (Collision|BreakHitResult _outhit))))))
          (Variables|SwimmingVariables|SetWaterSurfaceHight _output_get_2))))
    (:then_1
      (if (Math|Boolean|NotEqual(Boolean) (Variables|/Game/OpenWorldLocomotion/CharacterComponents/OWL_BaseComponent_BP.OWL_BaseComponent_BP_C|GetIsUnderwater (Variables|Default|GetBaseComponent)) (< (+ (Math|Float|Clamp(Float) (- _returnvalue_2 (Math|Float|Absolute(Float) (Variables|Swimming|GetUnderwaterCheckOffset))) 0.0 _returnvalue_2) (.z (Transformation|GetActorLocation (Variables|Default|GetCharacter)))) (Variables|SwimmingVariables|GetWaterPlaneHight)))
        (bind _output_get_3 (Variables|/Game/OpenWorldLocomotion/CharacterComponents/OWL_BaseComponent_BP.OWL_BaseComponent_BP_C|SetIsUnderwater (Variables|Default|GetBaseComponent) (< (+ (Math|Float|Clamp(Float) (- _returnvalue_2 (Math|Float|Absolute(Float) (Variables|Swimming|GetUnderwaterCheckOffset))) 0.0 _returnvalue_2) (.z (Transformation|GetActorLocation (Variables|Default|GetCharacter)))) (Variables|SwimmingVariables|GetWaterPlaneHight))))
        (Swimming|IsUnderwaterFunction _output_get_3)))))

(fn SprintingEvent
  (params (Sprinting :type Boolean))
  (if (Utilities|Enum|Equal(Enum) (Variables|/Game/OpenWorldLocomotion/CharacterComponents/OWL_BaseComponent_BP.OWL_BaseComponent_BP_C|GetLocomotionState (Variables|Default|GetBaseComponent)) "NewEnumerator7")
    (Swimming|ChangeMaxSpeed)))

(event Custom|ChangeLocomotionState_Event
  (params (NewLocomotionState :type E_LocomotionStates%20Enum :default "NewEnumerator0") (PrevLocomotionState :type E_LocomotionStates%20Enum :default "NewEnumerator0"))
  (bind _basecomponent (Variables|Default|GetBaseComponent))
  (bind _charactermovement (Variables|Default|GetCharacterMovement))
  (if (Utilities|Enum|Equal(Enum) NewLocomotionState "NewEnumerator7")
    ;[1 1 1] New
    (Character|UnCrouch (Variables|Default|GetCharacter))
    (bind _output_get (Variables|/Game/OpenWorldLocomotion/CharacterComponents/OWL_BaseComponent_BP.OWL_BaseComponent_BP_C|SetLocomotionState _basecomponent "NewEnumerator7"))
    (Variables|/Game/OpenWorldLocomotion/CharacterComponents/OWL_BaseComponent_BP.OWL_BaseComponent_BP_C|SetLocomotionStateNetworked _basecomponent _output_get)
    (Default|SetMovementMode (Variables|Default|GetBaseComponent))
    (Default|ResetSprinting (Variables|Default|GetBaseComponent))
    (Variables|/Script/Engine.CharacterMovementComponent|SetRotationRate (Variables|Default|GetCharacterMovement) (Variables|Swimming|GetSurfaceRotationRate))
    (Variables|/Script/Engine.CharacterMovementComponent|SetMaxAcceleration (Variables|Default|GetCharacterMovement) (Variables|Swimming|GetSwimmingMaxAcceleration))
    (Variables|/Script/Engine.CharacterMovementComponent|SetBrakingDecelerationSwimming (Variables|Default|GetCharacterMovement) (Variables|Swimming|GetBrakingDecelerationSwimming))
    (Swimming|ChangeMaxSpeed)
    (Variables|/Script/Engine.MovementComponent|SetVelocity _charactermovement (Math|Vector|MakeVector (/ (.x (Variables|/Script/Engine.MovementComponent|GetVelocity _charactermovement)) 2.0) (/ (.y (Variables|/Script/Engine.MovementComponent|GetVelocity _charactermovement)) 2.0) (.z (Variables|/Script/Engine.MovementComponent|GetVelocity _charactermovement))))
    (bind _active (Class|OWLInterfaceBPI|BPIWaterSurfaceData(Message) (Variables|Default|GetCharacter)))
    (bind _output_get_2 (Variables|SwimmingVariables|SetCanGetSurfaceData _active))
    (Variables|SwimmingVariables|SetGetSurfaceData _output_get_2)
    (Swimming|SwimmingLogic)
    (Swimming|IsUnderwaterFunction (Variables|/Game/OpenWorldLocomotion/CharacterComponents/OWL_BaseComponent_BP.OWL_BaseComponent_BP_C|GetIsUnderwater (Variables|Default|GetBaseComponent)))
    (elif (Utilities|Enum|Equal(Enum) PrevLocomotionState "NewEnumerator7")
      ;[1 1 1] Previous
      (Variables|/Script/Engine.CharacterMovementComponent|SetMaxAcceleration (Variables|Default|GetCharacterMovement) (Variables|DoNotModify|GetSaved_MaxAcceleration))
      (Default|ResetSprinting (Variables|Default|GetBaseComponent))
      (Variables|/Game/OpenWorldLocomotion/CharacterComponents/OWL_BaseComponent_BP.OWL_BaseComponent_BP_C|SetIsUnderwater (Variables|Default|GetBaseComponent) false))))