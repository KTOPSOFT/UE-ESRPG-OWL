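; Open World Locomotion component that adds gliding, toggled by jump while falling, with an optional floor-clearance trace.
; It follows the base component's locomotion state, swapping movement settings, spawning the glider and optionally simulating mesh bones, then reverting on exit.
; While gliding, gravity is zero and Tick drives velocity through LaunchCharacter, blending constant fall with timed external launches.
; Tick also tilts the character by acceleration and velocity and updates sprint-based gait.
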(event EventBeginPlay
  ;[0 1 1] Initialize component
  (|CallParentFunction)
  (Initialization|Initialize))

(event EventTick
  (params (DeltaSeconds :type Float%20%28single-precision%29))
  (|CallParentFunction DeltaSeconds)
  (if (not (Variables|/Game/OpenWorldLocomotion/CharacterComponents/OWL_BaseComponent_BP.OWL_BaseComponent_BP_C|GetBlockLocomotionLogic (Variables|Default|GetBaseComponent)))
    (if (Utilities|Enum|Equal(Enum) (Variables|/Game/OpenWorldLocomotion/CharacterComponents/OWL_BaseComponent_BP.OWL_BaseComponent_BP_C|GetLocomotionState (Variables|Default|GetBaseComponent)) "NewEnumerator4")
      (Gliding|GlidingLogic))))

(fn ChangeMaxSpeed
  (if (Utilities|Enum|Equal(Enum) (Variables|/Game/OpenWorldLocomotion/CharacterComponents/OWL_BaseComponent_BP.OWL_BaseComponent_BP_C|GetLocomotionState (Variables|Default|GetBaseComponent)) "NewEnumerator4")
    (Variables|/Script/Engine.CharacterMovementComponent|SetMaxWalkSpeed (Variables|Default|GetCharacterMovement) (Math|Float|SelectFloat (Variables|Gliding|GetGlidingMaxLateraSprintSpeed) (Variables|Gliding|GetGlidingMaxLateralSpeed) (Variables|/Game/OpenWorldLocomotion/CharacterComponents/OWL_BaseComponent_BP.OWL_BaseComponent_BP_C|GetIsSprinting (Variables|Default|GetBaseComponent))))))

(fn GlidingLogic
  (Base|ChangeGait)
  (Utilities|RotateActor true (Math|Rotator|MakeRotator (Math|Float|MapRangeClamped (.yaw (Math|Conversions|RotationFromXVector (Math|Vector|RotateVector (Class|KismetMathLibrary|VectorNormal2D (Pawn|Components|CharacterMovement|GetCurrentAcceleration (Variables|Default|GetCharacterMovement)) 0.0001) (Math|Rotator|MakeRotator 0.0 0.0 (.yaw (Class|KismetMathLibrary|NegateRotator (Transformation|GetActorRotation (Variables|Default|GetCharacter)))))))) -1.8e+02 1.8e+02 -3e+01 3e+01) (Math|Float|MapRangeClamped (.x (/ (Math|Vector|RotateVector (Transformation|GetVelocity (Variables|Default|GetCharacter)) (Math|Rotator|MakeRotator 0.0 0.0 (.yaw (Class|KismetMathLibrary|NegateRotator (Transformation|GetActorRotation (Variables|Default|GetCharacter)))))) (Class|MovementComponent|GetMaxSpeed (Variables|Default|GetCharacterMovement)))) -1.0 1.0 1e+01 -1e+01) (.yaw (Transformation|GetActorRotation (Variables|Default|GetCharacter)))) (Variables|Gliding|GetRotation_InterpSpeed))
  (Utilities|FlowControl|Sequence
    (:then_0
      (Variables|GlidingVariables|SetGlidingVelocity (|SetGlidingVelocity))
      (if (not (Variables|GlidingVariables|GetLaunchCharacter))
        (Variables|GlidingVariables|SetLaunchXYOverride false)
        (Variables|GlidingVariables|SetLaunchZOverride true)))
    (:then_1
      (if (|CorrectVelocity)
        ;[1 1 1] Add constatant fall speed to velocity vector
        (Character|LaunchCharacter (Variables|Default|GetCharacter) (Variables|GlidingVariables|GetGlidingVelocity) (Variables|GlidingVariables|GetLaunchXYOverride) (Variables|GlidingVariables|GetLaunchZOverride))))))

(fn CanGlide
  (bind _character (Variables|Default|GetCharacter))
  (bind _capsulecomponent (Variables|/Script/Engine.Character|GetCapsuleComponent _character))
  (bind _returnvalue (Components|Capsule|GetScaledCapsuleHalfHeight _capsulecomponent))
  (bind _returnvalue_2 (Transformation|GetWorldLocation _capsulecomponent))
  (bind _returnvalue_3 (- _returnvalue_2 (Math|Vector|MakeVector 0.0 0.0 _returnvalue)))
  (if (or (Variables|Gliding|GetDisableGliding) (Variables|GlidingVariables|GetDisableGliding_Override))
    (return false)
    (else
      ;[1 0 0] You can disable the floor check by setting the boolean. Usefull for wind up drafts
      (if (Variables|Gliding|GetGlidingStartFloorCheck)
        ;[1 1 1] Tarce down form the bottom edge of the capsule to check for a walkable floor. Prevent gliding form starting while jumping on a flat surface
        (bind (_outhit _returnvalue_4) (Class|KismetSystemLibrary|SphereTraceSinglebyProfile (+ _returnvalue_3 "0, 0,10.000000") (+ _returnvalue_3 (Math|Vector|MakeVector 0.0 0.0 (* -1 (Variables|Gliding|GetGlidingStartHight)))) (Components|Capsule|GetScaledCapsuleRadius (Variables|/Script/Engine.Character|GetCapsuleComponent (Variables|Default|GetCharacter))) "Pawn" false 0 "None" true "(R=1.000000,G=0.762658,B=0.000000,A=1.000000)" "(R=0.293873,G=1.000000,B=0.330127,A=1.000000)"))
        (if (and (Class|CharacterMovementComponent|IsWalkable (Variables|Default|GetCharacterMovement) _outhit) _returnvalue_4)
          (return false)
          (else
            (return true)))
        (else
          (return true))))))

(fn InputJump
  (if (not (Class|PawnMovementComponent|IsMoveInputIgnored (Variables|Default|GetCharacterMovement)))
    (switch Utilities|FlowControl|Switch|SwitchonE_LocomotionStates (Variables|/Game/OpenWorldLocomotion/CharacterComponents/OWL_BaseComponent_BP.OWL_BaseComponent_BP_C|GetLocomotionState (Variables|Default|GetBaseComponent))
      (:NewEnumerator2
        (bind _canglide (Gliding|CanGlide))
        (if _canglide
          (Default|ChangeMovementStateNetworking (Variables|Default|GetBaseComponent) "NewEnumerator4")))
      (:NewEnumerator4
        (Default|ChangeMovementStateNetworking (Variables|Default|GetBaseComponent) "NewEnumerator2")))))

(fn ChangeGait
  (if (not (Math|Vector|VectorIsZero (Transformation|GetVelocity (Variables|Default|GetCharacter))))
    (LocalVariables|SetPreviousGait_Loc (Variables|/Game/OpenWorldLocomotion/CharacterComponents/OWL_BaseComponent_BP.OWL_BaseComponent_BP_C|GetGait (Variables|Default|GetBaseComponent)))
    (Utilities|FlowControl|Sequence
      (:then_0
        ;[1 1 1] Change gait for gliding based on current velocity
        (if (Variables|/Game/OpenWorldLocomotion/CharacterComponents/OWL_BaseComponent_BP.OWL_BaseComponent_BP_C|GetIsSprinting (Variables|Default|GetBaseComponent))
          (if (> (Math|Vector|VectorLength (Transformation|GetVelocity (Variables|Default|GetCharacter))) (Variables|Gliding|GetGlidingMaxLateralSpeed))
            (Variables|/Game/OpenWorldLocomotion/CharacterComponents/OWL_BaseComponent_BP.OWL_BaseComponent_BP_C|SetGait (Variables|Default|GetBaseComponent) "NewEnumerator1")
            (else
              (Variables|/Game/OpenWorldLocomotion/CharacterComponents/OWL_BaseComponent_BP.OWL_BaseComponent_BP_C|SetGait (Variables|Default|GetBaseComponent) "NewEnumerator0")))
          (else
            (Variables|/Game/OpenWorldLocomotion/CharacterComponents/OWL_BaseComponent_BP.OWL_BaseComponent_BP_C|SetGait (Variables|Default|GetBaseComponent) "NewEnumerator0"))))
      (:then_1
        (if (Utilities|Enum|NotEqual(Enum) (LocalVariables|GetPreviousGait_Loc) (Variables|/Game/OpenWorldLocomotion/CharacterComponents/OWL_BaseComponent_BP.OWL_BaseComponent_BP_C|GetGait (Variables|Default|GetBaseComponent)))
          (Default|CallOnGaitChanged (Variables|Default|GetBaseComponent) (Variables|/Game/OpenWorldLocomotion/CharacterComponents/OWL_BaseComponent_BP.OWL_BaseComponent_BP_C|GetGait (Variables|Default|GetBaseComponent))))))))

(fn SprintingEvent
  (params (Sprinting :type Boolean))
  (if (Utilities|Enum|Equal(Enum) (Variables|/Game/OpenWorldLocomotion/CharacterComponents/OWL_BaseComponent_BP.OWL_BaseComponent_BP_C|GetLocomotionState (Variables|Default|GetBaseComponent)) "NewEnumerator4")
    (Base|ChangeMaxSpeed)))

(fn DisableGlidingOverrideEvent
  (params (DisableGliding :type Boolean))
  (Variables|GlidingVariables|SetDisableGliding_Override DisableGliding))

(event Custom|Gliding%20Launch%20Character
  (params (Duration :type Float%20%28double-precision%29) (LaunchVelocity :type Vector) (XYOverride :type Boolean) (ZOverride :type Boolean))
  (Variables|GlidingVariables|SetLaunchCharacter true)
  (Variables|GlidingVariables|SetLaunchDuration Duration)
  (Variables|GlidingVariables|SetLaunchVelocity LaunchVelocity)
  (Variables|GlidingVariables|SetLaunchXYOverride XYOverride)
  (Variables|GlidingVariables|SetLaunchZOverride ZOverride)
  (Utilities|FlowControl|RetriggerableDelay (Variables|GlidingVariables|GetLaunchDuration))
  (Variables|GlidingVariables|SetLaunchCharacter false))

(event Custom|CorrectRotation
  (params (Condition :type Boolean))
  (if Condition
    (Utilities|Timer 0.5 :!label _label
      (:Update
        (Utilities|RotateActor true (Math|Rotator|MakeRotator 0.0 0.0 (.yaw (Transformation|GetActorRotation (Variables|Default|GetCharacter)))) 1e+01)))
    (else
      (goto _label Stop))))

(event Custom|ChangeLocomotionState_Event
  (params (NewLocomotionState :type E_LocomotionStates%20Enum :default "NewEnumerator0") (PrevLocomotionState :type E_LocomotionStates%20Enum :default "NewEnumerator0"))
  (bind _basecomponent (Variables|Default|GetBaseComponent))
  (if (Utilities|Enum|Equal(Enum) NewLocomotionState "NewEnumerator4")
    (bind _output_get (Variables|/Game/OpenWorldLocomotion/CharacterComponents/OWL_BaseComponent_BP.OWL_BaseComponent_BP_C|SetLocomotionState _basecomponent "NewEnumerator4"))
    (Variables|/Game/OpenWorldLocomotion/CharacterComponents/OWL_BaseComponent_BP.OWL_BaseComponent_BP_C|SetLocomotionStateNetworked _basecomponent _output_get)
    (Default|ResetSprinting (Variables|Default|GetBaseComponent))
    (Base|ChangeMaxSpeed)
    (Utilities|FlowControl|Sequence
      (:then_0
        ;[1 1 1] Enable physics simulation
        (if (Variables|Physics|GetEnablePhysics)
          (if true
            (Collision|SetCollisionEnabled (Variables|/Script/Engine.Character|GetMesh (Variables|Default|GetCharacter)) "QueryAndPhysics")
            (bind _keys (Utilities|Map|Keys (Variables|Physics|GetPhysicsBoneNames)))
            (for _array_element _keys
              (if (Transformation|DoesSocketExist (Variables|/Script/Engine.Character|GetMesh (Variables|Default|GetCharacter)) _array_element)
                (Class|SkeletalMeshComponent|SetAllBodiesBelowSimulatePhysics (Variables|/Script/Engine.Character|GetMesh (Variables|Default|GetCharacter)) _array_element (.Value (Utilities|Map|Find (Variables|Physics|GetPhysicsBoneNames) _array_element)) true)
                (else
                  (Development|PrintString "Incorrect bone name. Change the PhysicsBoneName variable in the Gliding component to match the bone names in your skeleton or set EnablePhysics to false" true true "(R=1.000000,G=0.000000,B=0.000000,A=1.000000)" 2e+01))))
            (Class|SkeletalMeshComponent|SetAllBodiesBelowPhysicsBlendWeight (Variables|/Script/Engine.Character|GetMesh (Variables|Default|GetCharacter)) (Variables|/Game/OpenWorldLocomotion/CharacterComponents/OWL_BaseComponent_BP.OWL_BaseComponent_BP_C|GetPelvis%20Bone%20Name (Variables|Default|GetBaseComponent)) (Variables|Physics|GetPhysics%20Blend%20Weight) false false))))
      (:then_1
        ;[1 1 1] New
        (Default|SetMovementMode (Variables|Default|GetBaseComponent))
        (Variables|/Script/Engine.CharacterMovementComponent|SetAirControl (Variables|Default|GetCharacterMovement) (Variables|Gliding|GetGlidingAirControl))
        (Variables|/Script/Engine.CharacterMovementComponent|SetBrakingDecelerationFalling (Variables|Default|GetCharacterMovement) (Variables|Gliding|GetGlidingLateralDeceleration))
        (Variables|/Script/Engine.CharacterMovementComponent|SetRotationRate (Variables|Default|GetCharacterMovement) (Variables|Gliding|GetGlidingRotationRate))
        (Variables|/Script/Engine.CharacterMovementComponent|SetGravityScale (Variables|Default|GetCharacterMovement) 0.0)
        (CallFunction|CorrectRotation false))
      (:then_2
        ;[1 1 1] SpawnGlider
        (Utilities|FlowControl|RetriggerableDelay (Variables|Glider|GetGliderSpawnDelay))
        (if (Utilities|Enum|Equal(Enum) (Variables|/Game/OpenWorldLocomotion/CharacterComponents/OWL_BaseComponent_BP.OWL_BaseComponent_BP_C|GetLocomotionState (Variables|Default|GetBaseComponent)) "NewEnumerator4")
          (bind _returnvalue (Game|SpawnActorfromClass (Variables|Glider|GetGliderClass) (Math|Transform|MakeTransform "0, 0, 0" "0, 0, 0" "1.000000,1.000000,1.000000") "AlwaysSpawn" 0 0))
          (bind _output_get_2 (Variables|GlidingVariables|SetGlider _returnvalue))
          (Transformation|AttachComponentToComponent _output_get_2 (Variables|/Script/Engine.Character|GetMesh (Variables|Default|GetCharacter)) "GliderSocket" "KeepRelative" "KeepRelative" "KeepRelative" true))))
    (else
      ;[1 1 1] Previous
      (if (Utilities|Enum|Equal(Enum) PrevLocomotionState "NewEnumerator4")
        (Utilities|FlowControl|Sequence
          (:then_0
            (Variables|/Script/Engine.CharacterMovementComponent|SetGravityScale (Variables|Default|GetCharacterMovement) (Variables|DoNotModify|GetSaved_GravityScale))
            (Variables|/Script/Engine.CharacterMovementComponent|SetAirControl (Variables|Default|GetCharacterMovement) (Variables|DoNotModify|GetSaved_AirControl))
            (Variables|/Script/Engine.CharacterMovementComponent|SetBrakingDecelerationFalling (Variables|Default|GetCharacterMovement) (Variables|DoNotModify|GetSaved_BrakingDecelerationFalling))
            (Default|ResetSprinting (Variables|Default|GetBaseComponent))
            (Collision|SetCollisionEnabled (Variables|/Script/Engine.Character|GetMesh (Variables|Default|GetCharacter)) "QueryOnly")
            (Class|SkeletalMeshComponent|SetAllBodiesSimulatePhysics (Variables|/Script/Engine.Character|GetMesh (Variables|Default|GetCharacter)) false)
            (bind _glider (Variables|GlidingVariables|GetGlider)
              (:then
                (Actor|DestroyActor _glider))
              (:else)))
          (:then_1
            (if (Utilities|Enum|NotEqual(Enum) NewLocomotionState "NewEnumerator3")
              (CallFunction|CorrectRotation true))))))))