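; Blueprint function library of helpers for the advanced vehicle system, covering car paint, passenger checks and angle math.
; The color helper puts a random entry from a Colors array into the car's material array, then reapplies the materials.
; Passenger detection tests a valid pawn for the car passenger interface.
; Angle helpers return degrees between normalized vectors in 3D or 2D, with optional 2D sign from the cross product.
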(fn ApplyRandomColortoCar
  (params (inCar :type BP%20New%20Base%20Vehicle%20Object%20Reference))
  (Utilities|Array|SetArrayElem (Variables|/Game/DD_Vehicles_Advanced/Blueprints/Vehicles/BP_NewBaseVehicle.BP_NewBaseVehicle_C|GetMaterialsRef inCar) 0 (Utilities|Array|Get(acopy) (LocalVariables|GetColors) (Math|Random|RandomIntegerinRange 0 (- (Utilities|Array|Length (LocalVariables|GetColors)) 1))) true)
  (Default|SetMaterials inCar (Variables|/Game/DD_Vehicles_Advanced/Blueprints/Vehicles/BP_NewBaseVehicle.BP_NewBaseVehicle_C|GetMaterialsRef inCar)))

(fn GetAngleBetween
  (params (Vector1 :type Vector) (Vector2 :type Vector))
  (return (Class|KismetMathLibrary|DegAcos (Math|Vector|DotProduct (Math|Vector|Normalize Vector1) (Math|Vector|Normalize Vector2)))))

(fn IsPassenger
  (params (Pawn :type Pawn%20Object%20Reference))
  (Utilities|IsValid Pawn
    (:Is%20Valid
      (return (Utilities|DoesObjectImplementInterface Pawn "/Game/DD_Vehicles_Advanced/Blueprints/Passenger/BP_Interface_CarPassenger.BP_Interface_CarPassenger_C")))
    (:Is%20Not%20Valid
      (return false))))

(fn Get2DAngleBetween
  (params (Signed :type Boolean) (VectorA :type Vector%202D%20Structure) (VectorB :type Vector%202D%20Structure))
  (if Signed
    (return (* (Class|KismetMathLibrary|DegAcos (Math|Vector2D|DotProduct(2D) (Math|Vector2D|Normalize2D VectorA) (Math|Vector2D|Normalize2D VectorB))) (Math|Float|Sign(Float) (- (* (.y VectorB) (.x VectorA)) (* (.y VectorA) (.x VectorB))))))
    (else
      (return (Class|KismetMathLibrary|DegAcos (Math|Vector2D|DotProduct(2D) (Math|Vector2D|Normalize2D VectorA) (Math|Vector2D|Normalize2D VectorB)))))))