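; Arcade game mode that seats player 0 in a randomly chosen BP_NewBaseVehicle three seconds after BeginPlay.
; A Tick-fed gate also watches for the E key, closing while a manual entry attempt runs to block repeats.
; That attempt waits briefly, then enters another random car only if the controlled pawn is a SpectatorPawn, otherwise it reopens the gate.
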(event EventBeginPlay
  ;[0 1 0] Begin Play (Automatic entrance)
  (Utilities|FlowControl|Delay 3.0)
  ;[1 1 1] Enter car
  (bind _car (|Getrandomcar))
  (Default|CEEnterCar _car (Game|GetPlayerController 0) 0 false)
  ;[0 1 0] Event Tick (Manual entrance)
  (Utilities|FlowControl|Gate false) ; enters at Open
)

(event EventTick
  (params (DeltaSeconds :type Float%20%28single-precision%29))
  ;[0 1 0] Event Tick (Manual entrance)
  (Utilities|FlowControl|Gate false :!label _label
    (:Exit
      (|InputEisdown
        (:Start%20entrance
          (|Checkplayercanentercar
            (:true
              ;[1 1 1] Enter car
              (bind _car (|Getrandomcar))
              (Default|CEEnterCar _car (Game|GetPlayerController 0) 0 false)
              (goto _label Open))
            (:false
              (goto _label Open))))
        (:block%20manual%20entrance
          (goto _label Close))))))

(fn ConstructionScript)