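; Networked game state that monitors server frame rate, adapts client FPS limits to it, and shows clients a loading screen on start.
; After five seconds, server Tick measures FPS, toggles LowFPSOnServer below ServerFpsLimit, and updates MinServerFps after deviations persist 30 seconds.
; OnRep handlers show or hide the server-state warning widget and conditionally issue a client t.MaxFPS command derived from MinServerFps.
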(event EventBeginPlay
  ;[0 1 0] BeginPlay
  (if (not (Class|KismetSystemLibrary|IsStandalone))
    ;;[1 1 1] Loading screen on clients
    (Networking|SwitchHasAuthority
      (:Remote
        (bind _returnvalue (UserInterface|CreateWidget "/Game/DD_Vehicles_Advanced/Blueprints/Widgets/WBP_ClientLoadingScreen.WBP_ClientLoadingScreen_C"))
        (UserInterface|Viewport|AddtoViewport _returnvalue 0)))))

(event EventTick
  (params (DeltaSeconds :type Float%20%28single-precision%29))
  ;[0 1 0] EventTick
  (Networking|SwitchHasAuthority
    (:Authority
      (if (> (Utilities|Time|GetGameTimeinSeconds) 5.0)
        (Variables|FPSControl|SetCurrentServerFps (/ 1.0 DeltaSeconds))
        (Utilities|FlowControl|Sequence
          (:then_0
            (|EvaluateFPSadjustment))
          (:then_1
            (|Showserverstate)))))))

(fn ConstructionScript)

(fn OnRepMinServerFps
  (bind _minserverfps (Variables|FPSControl|GetMinServerFps))
  (Networking|SwitchHasAuthority
    (:Remote
      (if (< (- (Variables|FPSControl|GetServerFpsLimit) 1e+01) _minserverfps)
        (Development|ExecuteConsoleCommand (Utilities|String|Append "t.MaxFPS " (Utilities|String|ToString(Float) (- _minserverfps 1e+01))) (Game|GetPlayerController 0))))))

(fn OnRepLowFPSonServer
  (if (Variables|FPSControl|GetLowFPSOnServer)
    (Variables|FPSControl|GetServerStateWidget
      (:then
        _)
      (:else
        (bind _returnvalue (UserInterface|CreateWidget "/Game/DD_Vehicles_Advanced/Blueprints/Widgets/WBP_UI_ServerState.WBP_UI_ServerState_C"))
        (bind _output_get (Variables|FPSControl|SetServerStateWidget _returnvalue))))
    (if (not (UserInterface|Viewport|IsinViewport _output_get))
      (UserInterface|Viewport|AddtoViewport _output_get 1))
    (else
      (bind _serverstatewidget (Variables|FPSControl|GetServerStateWidget)
        (:then
          (if (UserInterface|Viewport|IsinViewport _serverstatewidget)
            (Widget|RemovefromParent _serverstatewidget)))
        (:else)))))