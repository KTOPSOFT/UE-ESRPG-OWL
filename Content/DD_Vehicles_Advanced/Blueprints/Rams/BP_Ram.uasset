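; BP_Ram is a ram actor with an optional target and wedge head that reacts to hits from BP_NewBaseVehicle.
; Construction toggles the target decal and wedge head collision; BeginPlay spawns a linked BP_RamTarget at the decal when enabled.
; Vehicle hits tell the target to stop, then a once-gated delayed overlap check looks up BP_ResetRams actors without using the result.
; ce_Reset resets the target and re-arms the gate.
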(event OnComponentHit(Mesh)
  (params (HitComponent :type Primitive%20Component%20Object%20Reference) (OtherActor :type Actor%20Object%20Reference) (OtherComp :type Primitive%20Component%20Object%20Reference) (NormalImpulse :type Vector :default "0, 0, 0") (Hit :type Hit%20Result%20Structure%20%28by%20ref%29))
  (bind _asbp_new_base_vehicle (Utilities|Casting|CastToBP_NewBaseVehicle OtherActor))
  (Variables|Default|SethitActor _asbp_new_base_vehicle)
  (Default|CeStopRam (Variables|Default|GetramTarget))
  (Utilities|FlowControl|DoOnce false
    (:Completed
      (Utilities|FlowControl|Delay 0.2)
      (if (Collision|IsOverlappingActor (Variables|Default|GethitActor) :!class /Script/Engine.Actor)
        (bind _outactors (Actor|GetAllActorsOfClass "/Game/DD_Vehicles_Advanced/Blueprints/Rams/BP_ResetRams.BP_ResetRams_C"))))))

(event Custom|ce_Reset
  (Default|CeResetRam (Variables|Default|GetramTarget))
  (Utilities|FlowControl|DoOnce false) ; enters at Reset
)

(event EventBeginPlay
  (Collision|IgnoreActorwhenMoving (Variables|Default|GetBlockHead) self true)
  (if (Variables|Default|GetuseTarget)
    (bind _returnvalue (Game|SpawnActorfromClass "/Game/DD_Vehicles_Advanced/Blueprints/Rams/BP_RamTarget.BP_RamTarget_C" (Transformation|GetWorldTransform (Variables|Default|GetDecal)) "Undefined" 0 0))
    (Variables|Default|SetramTarget _returnvalue)
    (Variables|/Game/DD_Vehicles_Advanced/Blueprints/Rams/BP_RamTarget.BP_RamTarget_C|Setram (Variables|Default|GetramTarget) self)))

(fn ConstructionScript
  (bind _wedgehead (Variables|Default|GetWedgeHead))
  (Rendering|SetVisibility (Variables|Default|GetDecal) (Variables|Default|GetuseTarget) false)
  (Rendering|SetVisibility (Variables|Default|GetWedgeHead) (Variables|Default|GetuseWedgeHead) false)
  (if (Variables|Default|GetuseWedgeHead)
    (Collision|SetCollisionEnabled _wedgehead "QueryAndPhysics")
    (else
      (Collision|SetCollisionEnabled _wedgehead "NoCollision"))))