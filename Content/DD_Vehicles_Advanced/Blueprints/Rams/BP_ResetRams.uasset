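; Trigger podium that resets every BP_Ram vehicle in the level to its starting transform.
; BeginPlay caches all rams and their initial transforms.
; A character or skeletal mesh overlap, or the ce_reset event, makes the server zero throttle, reset and teleport each ram after a short delay.
; Multi feedback events play podium color, teleport sound and particle effects; ending overlap restores yellow.
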(event OnComponentBeginOverlap(trigger)
  (params (OverlappedComponent :type Primitive%20Component%20Object%20Reference) (OtherActor :type Actor%20Object%20Reference) (OtherComp :type Primitive%20Component%20Object%20Reference) (OtherBodyIndex :type Integer) (bFromSweep :type Boolean) (SweepResult :type Hit%20Result%20Structure%20%28by%20ref%29))
  ;[1 1 1] Begin Overlap
  (Utilities|Casting|CastToSkeletalMeshComponent OtherComp
    (:then
      _)
    (:CastFailed
      (Utilities|Casting|CastToCharacter OtherActor)))
  (Networking|SwitchHasAuthority
    (:Authority
      (CallFunction|CEMultiOverlapFeedbacks true)
      (Utilities|FlowControl|Delay 0.4)
      (for (_array_element _array_index) (Variables|Default|GetRams)
        (Class|ChaosVehicleMovementComponent|SetThrottleInput (Variables|/Script/ChaosVehicles.WheeledVehiclePawn|GetVehicleMovementComponent _array_element) 0.0)
        (Default|CeReset _array_element)
        (CallFunction|CEMultiRepositionFeedbacks (Transformation|GetActorLocation _array_element))
        (Transformation|SetActorTransform _array_element (Utilities|Array|Get(acopy) (Variables|Default|GetramsIntitialTransform) _array_index) false true)))))

(event Custom|ce_reset
  ;[1 1 1] Begin Overlap
  (Networking|SwitchHasAuthority
    (:Authority
      (CallFunction|CEMultiOverlapFeedbacks true)
      (Utilities|FlowControl|Delay 0.4)
      (for (_array_element _array_index) (Variables|Default|GetRams)
        (Class|ChaosVehicleMovementComponent|SetThrottleInput (Variables|/Script/ChaosVehicles.WheeledVehiclePawn|GetVehicleMovementComponent _array_element) 0.0)
        (Default|CeReset _array_element)
        (CallFunction|CEMultiRepositionFeedbacks (Transformation|GetActorLocation _array_element))
        (Transformation|SetActorTransform _array_element (Utilities|Array|Get(acopy) (Variables|Default|GetramsIntitialTransform) _array_index) false true)))))

(event Custom|CE_Multi_RepositionFeedbacks
  (params (Location :type Vector))
  ;[1 1 1] Feedbacks (Multiplayer)
  (Effects|SpawnEmitteratLocation "/Game/DD_Vehicles_Advanced/Particles/PS_Teleport.PS_Teleport" Location))

(event Custom|CE_Multi_OverlapFeedbacks
  (params (Active :type Boolean))
  ;[1 1 1] Feedbacks (Multiplayer)
  (if Active
    (Rendering|Material|SetMaterial (Variables|Default|Getpodium) 0 "/Game/DD_Vehicles_Advanced/Materials/Material_Instances/garage/MI_emissive_blue.MI_emissive_blue")
    (Audio|PlaySoundatLocation "/Game/DD_Vehicles_Advanced/Sound/cues/general/SC_teleport.SC_teleport" (Transformation|GetActorLocation) "0, 0, 0" 1.0 1.0 0.0 0 0 0 0)
    (else
      (Rendering|Material|SetMaterial (Variables|Default|Getpodium) 0 "/Game/DD_Vehicles_Advanced/Materials/Material_Instances/TestArea/MI_emissive_yellow.MI_emissive_yellow"))))

(event EventBeginPlay
  ;[0 1 0] Begin Play
  (bind _outactors (Actor|GetAllActorsOfClass "/Game/DD_Vehicles_Advanced/Blueprints/Rams/BP_Ram.BP_Ram_C"))
  (bind _output_get (Variables|Default|SetRams _outactors))
  (for _array_element _output_get
    (Utilities|Array|Add (Variables|Default|GetramsIntitialTransform) (Transformation|GetActorTransform _array_element))))

(event Collision|EventActorEndOverlap
  (params (OtherActor :type Actor%20Object%20Reference))
  ;[1 1 1] End Overlap
  (CallFunction|CEMultiOverlapFeedbacks false))

(fn ConstructionScript)