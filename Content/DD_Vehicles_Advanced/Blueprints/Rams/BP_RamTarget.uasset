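; Trigger actor that launches its referenced Ram vehicle when another advanced-vehicle actor drives into its trigger.
; A skeletal-mesh overlap from a BP_NewBaseVehicle that is not a BP_Ram applies throttle after a short delay, gated by a DoOnce until ce_resetRam re-arms it.
; The Ram leaving the trigger, or ce_StopRam, cuts throttle and applies full brake through SetThrottle.
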(event OnComponentEndOverlap(trigger)
  (params (OverlappedComponent :type Primitive%20Component%20Object%20Reference) (OtherActor :type Actor%20Object%20Reference) (OtherComp :type Primitive%20Component%20Object%20Reference) (OtherBodyIndex :type Integer))
  (if (== OtherActor (Variables|Default|Getram))
    (CallFunction|SetThrottle 0.0)))

(event OnComponentBeginOverlap(trigger)
  (params (OverlappedComponent :type Primitive%20Component%20Object%20Reference) (OtherActor :type Actor%20Object%20Reference) (OtherComp :type Primitive%20Component%20Object%20Reference) (OtherBodyIndex :type Integer) (bFromSweep :type Boolean) (SweepResult :type Hit%20Result%20Structure%20%28by%20ref%29))
  (Utilities|Casting|CastToSkeletalMeshComponent OtherComp)
  (Utilities|Casting|CastToBP_NewBaseVehicle OtherActor)
  (Utilities|FlowControl|Delay 0.1)
  (if (not (== (Utilities|GetClass OtherActor) "/Game/DD_Vehicles_Advanced/Blueprints/Rams/BP_Ram.BP_Ram_C"))
    (Utilities|FlowControl|DoOnce false
      (:Completed
        (CallFunction|SetThrottle 1e+02)))))

(event Custom|ce_StopRam
  (CallFunction|SetThrottle 0.0))

(event Custom|ce_resetRam
  (Utilities|FlowControl|DoOnce false) ; enters at Reset
)

(fn ConstructionScript)

(fn SetThrottle
  (params (Throttle :type Float%20%28double-precision%29))
  (bind _ram (Variables|Default|Getram))
  (bind _ram_2 (Variables|Default|Getram))
  (bind _vehiclemovementcomponent (Variables|/Script/ChaosVehicles.WheeledVehiclePawn|GetVehicleMovementComponent _ram))
  (bind _vehiclemovementcomponent_2 (Variables|/Script/ChaosVehicles.WheeledVehiclePawn|GetVehicleMovementComponent _ram_2))
  (Utilities|IsValid (Variables|Default|Getram)
    (:Is%20Valid
      (if (== Throttle 0.0)
        (Class|ChaosVehicleMovementComponent|SetBrakeInput _vehiclemovementcomponent_2 1.0)
        (Class|ChaosVehicleMovementComponent|SetThrottleInput _vehiclemovementcomponent_2 0.0)
        (else
          (Class|ChaosVehicleMovementComponent|SetBrakeInput _vehiclemovementcomponent 0.0)
          (Class|ChaosVehicleMovementComponent|SetThrottleInput _vehiclemovementcomponent Throttle))))))