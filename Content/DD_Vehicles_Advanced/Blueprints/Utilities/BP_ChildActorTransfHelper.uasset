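; Transform marker helper actor for the vehicle assets, showing a named point in the editor and, by its name, intended for use as a child actor.
; Construction draws a cone (directional) or small sphere labeled with TransformName.
; BeginPlay either destroys the actor or removes the label and hides the mesh.
; UpdateTransformReference teleports it to a given location and rotation in world space, relative space, or offset from a supplied parent component.
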(event EventBeginPlay
  (if (Variables|Default|GetDestroyOnPlay)
    (Actor|DestroyActor)
    (else
      (Components|DestroyComponent (Variables|Default|GetTransformTitle))
      (Development|SetHiddeninGame (Variables|Default|GetHelper) true false))))

(fn ConstructionScript
  (Components|StaticMesh|SetStaticMesh (Variables|Default|GetHelper) (select (Variables|Default|GetShowDirection) "/Engine/BasicShapes/Cone.Cone" "/Engine/EngineMeshes/Sphere.Sphere"))
  (Transformation|SetRelativeScale3D (Variables|Default|GetHelper) (select (Variables|Default|GetShowDirection) "0.100000,0.100000,0.100000" "0.050000,0.050000,0.050000"))
  (Rendering|Components|TextRender|SetText (Variables|Default|GetTransformTitle) (Variables|Default|GetTransformName)))

(fn UpdateTransformReference
  (params (TransformReference :type Transform) (Relative :type Boolean) (UseAsParent :type Primitive%20Component%20Object%20Reference))
  (if Relative
    (Utilities|IsValid UseAsParent
      (:Is%20Valid
        (Transformation|SetActorTransform (Transformation|GetWorldTransform UseAsParent) false true)
        (Transformation|AddActorLocalOffset (.location TransformReference) false true)
        (Transformation|AddActorLocalRotation (.rotation TransformReference) false true))
      (:Is%20Not%20Valid
        (Transformation|SetActorRelativeTransform (Math|Transform|MakeTransform (.location TransformReference) (.rotation TransformReference) "1.000000,1.000000,1.000000") false true)))
    (else
      (Transformation|SetActorTransform (Math|Transform|MakeTransform (.location TransformReference) (.rotation TransformReference) "1.000000,1.000000,1.000000") false true))))