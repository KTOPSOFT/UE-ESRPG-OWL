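; Vehicle backfire effect actor, spawned under a BP_NewBaseVehicle, that plays an exhaust pop sound and particle when CE_Backfire is called.
; Volume and pitch scale with RPM, in-car state and the vehicle's volume modifier, while a randomized delay gate limits overlapping pops.
; It listens for constraint breaks on tag-matched destructible pieces, switching the particle's origin from the piece position to the vehicle position once one disconnects.
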(event Custom|CE_Backfire
  (params (delayBetweenPops :type Float%20%28double-precision%29) (RPM :type Float%20%28double-precision%29) (InCar :type Boolean))
  (bind _pieceposition (Variables|Default|GetPiecePosition))
  (bind _disconnectedpiece (Variables|Default|GetDisconnectedPiece))
  (bind _vehicleposition (Variables|Default|GetVehiclePosition))
  (bind _returnvalue (select _disconnectedpiece _vehicleposition _pieceposition))
  (bind _returnvalue_2 (Transformation|GetWorldTransform _returnvalue))
  ;[0 0 0] Backfire
  (if (Variables|Default|GetCanPop)
    (Variables|Default|SetDelayBetweenPops delayBetweenPops)
    (Variables|Default|SetCanPop false)
    (Utilities|FlowControl|Delay (Math|Random|RandomFloatinRange 0.01 0.02))
    (Audio|PlaySoundatLocation "/Game/DD_Vehicles_Advanced/Sound/Metasounds/MS_Backfire.MS_Backfire" (Transformation|GetActorLocation self) "0, 0, 0" (* (Math|Float|MapRangeClamped RPM 0.0 1e+04 0.5 (Math|Float|SelectFloat 0.25 0.5 InCar)) (Variables|Default|GetVolumeMultiplier)) (Math|Float|MapRangeClamped RPM 0.0 1e+04 -1.0 (Math|Float|SelectFloat 0.8 1.0 InCar)) 0.0 "/Game/DD_Vehicles_Advanced/Sound/Engine_Att.Engine_Att" 0 0 0)
    ;;[0 0 0] Spawn particle
    (Effects|SpawnEmitterAttached "/Game/DD_Vehicles_Advanced/Particles/P_Backfire.P_Backfire" (Variables|Default|GetVehiclePosition) "None" (.location _returnvalue_2) (.rotation _returnvalue_2) (.scale _returnvalue_2) "KeepWorldPosition")
    ;[0 0 0] Avoid many backfires at the same time
    (Utilities|FlowControl|Delay (Math|Random|RandomFloatinRange (/ (Variables|Default|GetDelayBetweenPops) 1.1) (Variables|Default|GetDelayBetweenPops)))
    (Variables|Default|SetCanPop true)))

(event Custom|CE_ContraintBroken
  ;[0 0.6042 0.02386] Begin Play
  (Variables|Default|SetDisconnectedPiece true))

(event EventBeginPlay
  (bind _returnvalue (Actor|GetParentActor))
  ;[0 0.6042 0.02386] Begin Play
  (bind _asbp_new_base_vehicle (Utilities|Casting|CastToBP_NewBaseVehicle _returnvalue))
  (bind _output_get (Variables|Default|SetParentVehicle _asbp_new_base_vehicle))
  (Variables|Default|SetVolumeMultiplier (Variables|/Game/DD_Vehicles_Advanced/Blueprints/Vehicles/BP_NewBaseVehicle.BP_NewBaseVehicle_C|GetBackfireVolumeModifier _output_get))
  (for _array_element (Actor|GetAllChildActors _returnvalue true)
    (bind _asbp_destructible_piece (Utilities|Casting|CastToBP_DestructiblePiece _array_element))
    (if (> (Utilities|Array|Length (Variables|Actor|GetTags)) 0)
      (if (Actor|ActorHasTag _asbp_destructible_piece (Utilities|Array|Get(acopy) (Variables|Actor|GetTags)))
        (EventDispatchers|BindEventtoConstraintBrokenDispatcher _asbp_destructible_piece (delegate Custom|CE_ContraintBroken))))))

(fn ConstructionScript
  (Transformation|SetRelativeTransform (Variables|Default|GetPiecePosition) (Variables|Default|GetPositionOnPiece) false true))