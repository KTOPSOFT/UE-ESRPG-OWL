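; BP_siren is a vehicle prop for an orange rotating warning beacon that can be switched on and off, burnt or blown off.
; Lights toggles four spotlights, swaps reflector and housing materials, and starts or stops a timeline that spins the two light meshes.
; Burn stops rotation, deactivates the spotlights and chars every housing material.
; Explode does the same, also detaching the actor and enabling physics on the housing.
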(event Custom|CE_Burn
  (bind _sm_siren (Variables|Default|Getsm_siren))
  ;[1 1 1] Damage
  (CallFunction|CeStopLights)
  (Components|Activation|Deactivate (Variables|Default|GetSpotLight1))
  (for (_ _array_index) (Rendering|Material|GetMaterials _sm_siren)
    (Rendering|Material|SetMaterial _sm_siren _array_index "/Game/DD_Vehicles_Advanced/Materials/Material_Instances/Misc/MI_Burnt.MI_Burnt")))

(event Custom|CE_Explode
  (bind _sm_siren (Variables|Default|Getsm_siren))
  (bind _sm_siren_2 (Variables|Default|Getsm_siren))
  ;[1 1 1] Damage
  (CallFunction|CeStopLights)
  (Components|Activation|Deactivate (Variables|Default|GetSpotLight1))
  (Transformation|DetachFromActor self "KeepWorld" "KeepWorld" "KeepWorld")
  (Physics|SetSimulatePhysics _sm_siren true)
  (Physics|SetEnableGravity _sm_siren true)
  (for (_ _array_index) (Rendering|Material|GetMaterials _sm_siren_2)
    (Rendering|Material|SetMaterial _sm_siren_2 _array_index "/Game/DD_Vehicles_Advanced/Materials/Material_Instances/Misc/MI_Burnt.MI_Burnt")))

(event Custom|Ce_stopLights
  ;[1 1 1] Lights
  (bind _rotationrate (Timeline|lightsTurn Stop)
    (:Update
      (Transformation|AddLocalRotation (Variables|Default|Getsm_light2) (Math|Rotator|MakeRotator 0.0 0.0 _rotationrate) false false))))

(event Custom|ce_RotateLights
  ;[1 1 1] Lights
  (bind _rotationrate (Timeline|lightsTurn Play)
    (:Update
      (Transformation|AddLocalRotation (Variables|Default|Getsm_light2) (Math|Rotator|MakeRotator 0.0 0.0 _rotationrate) false false))))

(fn ConstructionScript)

(fn Lights
  (params (lightsOn :type Boolean))
  (bind _sm_siren (Variables|Default|Getsm_siren))
  (Rendering|SetVisibility (Variables|Default|GetSpotLight2) lightsOn false)
  (if lightsOn
    (CallFunction|CeRotateLights)
    (Rendering|Material|SetMaterial (Variables|Default|Getsm_light2) 0 "/Game/DD_Vehicles_Advanced/Materials/Material_Instances/Reflectors/MI_Reflector_Orange_Emissive.MI_Reflector_Orange_Emissive")
    (Rendering|Material|SetMaterial _sm_siren 0 "/Game/DD_Vehicles_Advanced/Materials/Material_Instances/Reflectors/MI_Reflector_orange_TranslucentEmissive.MI_Reflector_orange_TranslucentEmissive")
    (else
      (CallFunction|CeStopLights)
      (Rendering|Material|SetMaterial (Variables|Default|Getsm_light) 0 "/Game/DD_Vehicles_Advanced/Materials/Material_Instances/Reflectors/MI_Reflector_Grey.MI_Reflector_Grey")
      (Rendering|Material|SetMaterial _sm_siren 0 "/Game/DD_Vehicles_Advanced/Materials/Material_Instances/Reflectors/MI_Reflector_orange_Translucent3.MI_Reflector_orange_Translucent3"))))