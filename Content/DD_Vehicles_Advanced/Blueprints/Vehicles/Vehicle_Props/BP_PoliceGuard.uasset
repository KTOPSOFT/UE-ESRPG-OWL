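; Police guard vehicle prop with flashing red and blue lights that the possessing player cycles through off, normal and double-speed modes.
; On possession, it toggles input and the siren mapping context; the horn action advances a replicated counter via a server event.
; A timeline animates dynamic light materials and a spotlight, after waiting for those materials to exist.
; Breaking the constraint shuts lights off, while burning or exploding applies a burnt material.
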(event Custom|ce_ParentPossessed
  (params (Controller :type Controller%20Object%20Reference) (Possessed :type Boolean))
  ;[1 1 1] bindings
  (CallFunction|CEMultiParentPossessed Controller Possessed))

(event Custom|CE_Multi_ParentPossessed
  (params (Controller :type Controller%20Object%20Reference) (Possessed :type Boolean))
  ;[1 1 1] bindings
  (|activate/deactivateInput Controller Possessed))

(event Custom|CE_Server_ActiveSiren
  ;[1 1 1] activate siren
  (Variables|Default|SetsirenCounter (Math|Integer|%(Integer) (+ (Variables|Default|GetsirenCounter) 1) 3))
  (switch int (Variables|Default|GetsirenCounter)
    (:0
      (Utilities|FlowControl|Sequence
        (:then_0
          (Utilities|FlowControl|Delay 0.1)
          (Rendering|Material|SetVectorParameterValue :self (Variables|Default|GetRedLights) :ParameterName "brightness" :!class /Script/Engine.MaterialInstanceDynamic)
          (Rendering|Material|SetVectorParameterValue :self (Variables|Default|GetBlueLights) :ParameterName "brightness" :!class /Script/Engine.MaterialInstanceDynamic)
          (Rendering|SetVisibility (Variables|Default|GetSpotLight) false false))
        (:then_1
          (goto _label Stop))))
    (:1
      (Components|Timeline|SetPlayRate (Variables|Default|GetTimeline_0) 1.0)
      (Rendering|SetVisibility (Variables|Default|GetSpotLight) true false)
      (|flashlights :!label _label))
    (:2
      (Components|Timeline|SetPlayRate (Variables|Default|GetTimeline_0) 2.0))))

(event Custom|CE_Burn
  (bind _self self)
  (bind _deformablemesh (Variables|Default|GetDeformableMesh _self))
  ;[1 1 1] Damage
  (Components|Activation|Deactivate (Variables|Default|GetSpotLight))
  (for (_ _array_index) (Rendering|Material|GetMaterials _deformablemesh)
    (Rendering|Material|SetMaterial _deformablemesh _array_index "/Game/DD_Vehicles_Advanced/Materials/Material_Instances/Misc/MI_Burnt.MI_Burnt")))

(event Custom|CE_OnRepSirenCounter
  ;[1 1 1] activate siren
  (|WheSirenisready
    (:Is%20Ready
      (switch int (Variables|Default|GetsirenCounter)
        (:0
          (Utilities|FlowControl|Sequence
            (:then_0
              (Utilities|FlowControl|Delay 0.1)
              (Rendering|Material|SetVectorParameterValue :self (Variables|Default|GetRedLights) :ParameterName "brightness" :!class /Script/Engine.MaterialInstanceDynamic)
              (Rendering|Material|SetVectorParameterValue :self (Variables|Default|GetBlueLights) :ParameterName "brightness" :!class /Script/Engine.MaterialInstanceDynamic)
              (Rendering|SetVisibility (Variables|Default|GetSpotLight) false false))
            (:then_1
              (goto _label Stop))))
        (:1
          (Components|Timeline|SetPlayRate (Variables|Default|GetTimeline_0) 1.0)
          (Rendering|SetVisibility (Variables|Default|GetSpotLight) true false)
          (|flashlights :!label _label))
        (:2
          (Components|Timeline|SetPlayRate (Variables|Default|GetTimeline_0) 2.0))))))

(event Custom|CE_Explode
  (bind _self self)
  (bind _collisionmesh (Variables|Default|GetCollisionMesh))
  (bind _deformablemesh (Variables|Default|GetDeformableMesh _self))
  ;[1 1 1] Damage
  (Components|Activation|Deactivate (Variables|Default|GetSpotLight))
  (Physics|SetSimulatePhysics _collisionmesh true)
  (Physics|SetEnableGravity _collisionmesh true)
  (for (_ _array_index) (Rendering|Material|GetMaterials _deformablemesh)
    (Rendering|Material|SetMaterial _deformablemesh _array_index "/Game/DD_Vehicles_Advanced/Materials/Material_Instances/Misc/MI_Burnt.MI_Burnt")))

(event Input|EnhancedActionEvents|EnhancedInputActionIA_Horn
  (params (ActionValue :type Boolean) (ElapsedSeconds :type Float%20%28double-precision%29) (TriggeredSeconds :type Float%20%28double-precision%29) (InputAction :type Input%20Action%20Object%20Reference :default "/Game/DD_Vehicles_Advanced/Blueprints/Vehicles/Input/Actions/IA_Horn.IA_Horn"))
  ;[1 1 1] activate siren
  (:Started
    (CallFunction|CEServerActiveSiren)))

(event EventCEonSynchComplete
  (bind _deformablemesh (Variables|Default|GetDeformableMesh))
  (bind _deformablemesh_2 (Variables|Default|GetDeformableMesh))
  ;[1 1 1] bindings
  (|CallParentFunction)
  (EventDispatchers|BindEventtoOnPossessed (Variables|Default|GetcarReference) (delegate Custom|ce_ParentPossessed))
  ;[1 1 1] create lights material instances
  (bind _returnvalue (Rendering|Material|CreateDynamicMaterialInstance _deformablemesh_2 2 (Rendering|Material|GetMaterial _deformablemesh_2 2) "None" :!class /Script/Engine.PrimitiveComponent))
  (Variables|Default|SetBlueLights _returnvalue)
  (bind _returnvalue_2 (Rendering|Material|CreateDynamicMaterialInstance _deformablemesh 1 (Rendering|Material|GetMaterial _deformablemesh 1) "None" :!class /Script/Engine.PrimitiveComponent))
  (Variables|Default|SetRedLights _returnvalue_2))

(event EventOnConstraintBroken
  ;[1 1 1] activate siren
  ;;[1 1 1] disconnect
  (|CallParentFunction)
  (Input|DisableInput (Game|GetPlayerController 0))
  (Utilities|FlowControl|Sequence
    (:then_0
      (Utilities|FlowControl|Delay 0.1)
      (Rendering|Material|SetVectorParameterValue :self (Variables|Default|GetRedLights) :ParameterName "brightness" :!class /Script/Engine.MaterialInstanceDynamic)
      (Rendering|Material|SetVectorParameterValue :self (Variables|Default|GetBlueLights) :ParameterName "brightness" :!class /Script/Engine.MaterialInstanceDynamic)
      (Rendering|SetVisibility (Variables|Default|GetSpotLight) false false))
    (:then_1
      (|flashlights) ; enters at Stop
    )))

(fn ConstructionScript
  (|CallParentFunction))

(fn OnRepSirenCounter
  (CallFunction|CEonRepSirenCounter))