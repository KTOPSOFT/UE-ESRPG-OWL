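; Police siren prop for vehicles, with horn-input control, flashing red/blue lights, breakable glass and burn/explode damage states.
; It physics-constrains itself to the parent car or a tag-matched destructible piece, with clients waiting to align using a server-computed relative transform.
; Possession toggles its Enhanced Input context; a counter with OnRep cycles off, on and faster flashing with alternate sound.
; Piece disconnection disables input and turns it off; explosion detaches it with physics and fire.
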(event OnComponentHit(sm_sirenGlass1)
  (params (HitComponent :type Primitive%20Component%20Object%20Reference) (OtherActor :type Actor%20Object%20Reference) (OtherComp :type Primitive%20Component%20Object%20Reference) (NormalImpulse :type Vector :default "0, 0, 0") (Hit :type Hit%20Result%20Structure%20%28by%20ref%29))
  ;[1 1 1] break glasses
  (if (> (Math|Vector|VectorLength NormalImpulse) 1e+02)
    (Utilities|FlowControl|DoOnce false
      (:Completed
        (CallFunction|BreakSirenGlass HitComponent Hit)))))

(event OnComponentHit(sm_sirenGlass2)
  (params (HitComponent :type Primitive%20Component%20Object%20Reference) (OtherActor :type Actor%20Object%20Reference) (OtherComp :type Primitive%20Component%20Object%20Reference) (NormalImpulse :type Vector :default "0, 0, 0") (Hit :type Hit%20Result%20Structure%20%28by%20ref%29))
  ;[1 1 1] break glasses
  (if (> (Math|Vector|VectorLength NormalImpulse) 1e+02)
    (Utilities|FlowControl|DoOnce false
      (:Completed
        (CallFunction|BreakSirenGlass HitComponent Hit)))))

(event Custom|CE_ReattachSiren
  (bind _oncarpossessed (|Oncarpossessedevents))
  ;[1 1 1] Reattach
  ;[0 1 0] begin play
  (Networking|SwitchHasAuthority
    (:Authority
      (|Getbindedcar)
      (|Gettransformadjustmentonserver))
    (:Remote
      (|Whenclientreadytoattachsiren
        (:IsReady
          _))))
  (|Carbindings _oncarpossessed)
  (|Generatematerialinstancies)
  (|Defineactortoattach
    (:DestructiblePiece
      (|TrytoattachtodestructiblePiece _oncarpossessed
        (:DestruciblePieceNotValid
          _)))
    (:Car
      _))
  (|Attachtocar))

(event Custom|CE_Burn
  ;[1 1 1] Damage
  (CallFunction|CETurnOff)
  (Rendering|Material|SetMaterial (Variables|Default|Getsm_sirenBase) 0 "/Game/DD_Vehicles_Advanced/Materials/Material_Instances/Misc/MI_Burnt.MI_Burnt")
  (bind _returnvalue (Game|SpawnActorfromClass "/Game/DD_Vehicles_Advanced/Blueprints/TestArea/BP_Fire.BP_Fire_C" (Transformation|GetWorldTransform (Variables|Default|Getsm_sirenBase)) "AlwaysSpawn" 0 0))
  (Utilities|Array|Add (Variables|/Game/DD_Vehicles_Advanced/Blueprints/Vehicles/BP_NewBaseVehicle.BP_NewBaseVehicle_C|GetSpawnedFires (Variables|Default|GetCar)) _returnvalue)
  (Default|CEAttach _returnvalue 0.0 (Variables|Default|Getsm_sirenBase) 1.0))

(event Custom|CE_Server_ActiveSiren
  ;[1 1 1] activate siren
  (Variables|Default|SetsirenCounter (Math|Integer|%(Integer) (+ (Variables|Default|GetsirenCounter) 1) 3)))

(event Custom|CE_TurnOff
  ;[1 1 1] activate siren
  (Components|Activation|Deactivate (Variables|Default|GetAudio))
  (Audio|Components|Audio|SetSound (Variables|Default|GetAudio) "/Game/DD_Vehicles_Advanced/Sound/cues/general/PoliceSirenBase_Cue.PoliceSirenBase_Cue")
  (Components|Timeline|SetPlayRate (Variables|Default|Getred/blue%20lights) 1.0)
  (Utilities|FlowControl|Sequence
    (:then_0
      (|flashlights) ; enters at Stop
    )
    (:then_1
      (Utilities|FlowControl|Delay 0.1)
      (Rendering|SetVisibility (Variables|Default|GetRedSpotLight) false false)
      (Rendering|Material|SetVectorParameterValue :self (Variables|Default|GetRedLights) :ParameterName "brightness" :!class /Script/Engine.MaterialInstanceDynamic)
      (Rendering|Material|SetVectorParameterValue :self (Variables|Default|GetBlueLights) :ParameterName "brightness" :!class /Script/Engine.MaterialInstanceDynamic))))

(event Custom|CE_OnRepSirenCounter
  ;[1 1 1] activate siren
  (|WheSirenisready
    (:Is%20Ready
      (switch int (Variables|Default|GetsirenCounter)
        (:0
          (Components|Activation|Deactivate (Variables|Default|GetAudio))
          (Audio|Components|Audio|SetSound (Variables|Default|GetAudio) "/Game/DD_Vehicles_Advanced/Sound/cues/general/PoliceSirenBase_Cue.PoliceSirenBase_Cue")
          (Components|Timeline|SetPlayRate (Variables|Default|Getred/blue%20lights) 1.0)
          (Utilities|FlowControl|Sequence
            (:then_0
              (goto _label Stop))
            (:then_1
              (Utilities|FlowControl|Delay 0.1)
              (Rendering|SetVisibility (Variables|Default|GetRedSpotLight) false false)
              (Rendering|Material|SetVectorParameterValue :self (Variables|Default|GetRedLights) :ParameterName "brightness" :!class /Script/Engine.MaterialInstanceDynamic)
              (Rendering|Material|SetVectorParameterValue :self (Variables|Default|GetBlueLights) :ParameterName "brightness" :!class /Script/Engine.MaterialInstanceDynamic))))
        (:1
          (Components|Activation|Activate (Variables|Default|GetAudio) false)
          (Rendering|SetVisibility (Variables|Default|GetRedSpotLight) true false)
          (|flashlights :!label _label))
        (:2
          (Audio|Components|Audio|SetSound (Variables|Default|GetAudio) "/Game/DD_Vehicles_Advanced/Sound/cues/general/PoliceSiren2_cue.PoliceSiren2_cue")
          (Components|Timeline|SetPlayRate (Variables|Default|Getred/blue%20lights) 2.0))))))

(event Custom|CE_Explode
  (bind _sm_sirenbase (Variables|Default|Getsm_sirenBase))
  ;[1 1 1] Damage
  (Transformation|DetachFromActor self "KeepWorld" "KeepWorld" "KeepWorld")
  (Physics|SetSimulatePhysics _sm_sirenbase true)
  (Physics|SetEnableGravity _sm_sirenbase true)
  (CallFunction|CETurnOff)
  (Rendering|Material|SetMaterial (Variables|Default|Getsm_sirenBase) 0 "/Game/DD_Vehicles_Advanced/Materials/Material_Instances/Misc/MI_Burnt.MI_Burnt")
  (bind _returnvalue (Game|SpawnActorfromClass "/Game/DD_Vehicles_Advanced/Blueprints/TestArea/BP_Fire.BP_Fire_C" (Transformation|GetWorldTransform (Variables|Default|Getsm_sirenBase)) "AlwaysSpawn" 0 0))
  (Utilities|Array|Add (Variables|/Game/DD_Vehicles_Advanced/Blueprints/Vehicles/BP_NewBaseVehicle.BP_NewBaseVehicle_C|GetSpawnedFires (Variables|Default|GetCar)) _returnvalue)
  (Default|CEAttach _returnvalue 0.0 (Variables|Default|Getsm_sirenBase) 1.0))

(event Input|EnhancedActionEvents|EnhancedInputActionIA_Horn
  (params (ActionValue :type Boolean) (ElapsedSeconds :type Float%20%28double-precision%29) (TriggeredSeconds :type Float%20%28double-precision%29) (InputAction :type Input%20Action%20Object%20Reference :default "/Game/DD_Vehicles_Advanced/Blueprints/Vehicles/Input/Actions/IA_Horn.IA_Horn"))
  ;[1 1 1] activate siren
  (:Started
    (if (not (Variables|/Game/DD_Vehicles_Advanced/Blueprints/Vehicles/BP_NewBaseVehicle.BP_NewBaseVehicle_C|GetExploded (Variables|Default|GetCar)))
      (CallFunction|CEServerActiveSiren))))

(event EventBeginPlay
  (bind _oncarpossessed (|Oncarpossessedevents))
  ;[0 1 0] begin play
  (Networking|SwitchHasAuthority
    (:Authority
      (|Getbindedcar)
      (|Gettransformadjustmentonserver))
    (:Remote
      (|Whenclientreadytoattachsiren
        (:IsReady
          _))))
  (|Carbindings _oncarpossessed)
  (|Generatematerialinstancies)
  (|Defineactortoattach
    (:DestructiblePiece
      (|TrytoattachtodestructiblePiece _oncarpossessed
        (:DestruciblePieceNotValid
          _)))
    (:Car
      _))
  (|Attachtocar))

(fn ConstructionScript)

(fn BreakSirenGlass
  (params (HitComponent :type Primitive%20Component%20Object%20Reference) (Hit :type Hit%20Result%20Structure%20%28by%20ref%29))
  (bind _returnvalue (Rendering|Material|CreateDynamicMaterialInstance HitComponent 0 (Rendering|Material|GetMaterial HitComponent 0) "None" :!class /Script/Engine.PrimitiveComponent))
  (Rendering|Material|SetTextureParameterValue _returnvalue "ImpactMask" 0)
  (Rendering|Material|SetScalarParameterValue _returnvalue "opacity" 5.0 :!class /Script/Engine.MaterialInstanceDynamic)
  (Rendering|Material|SetScalarParameterValue _returnvalue "BreakTreshold" 0.1 :!class /Script/Engine.MaterialInstanceDynamic)
  (Audio|PlaySoundatLocation "/Game/DD_Vehicles_Advanced/Sound/cues/impacts/broken_glass_Cue.broken_glass_Cue" (Transformation|GetActorLocation) "0, 0, 0" 1.0 1.0 0.0 0 0 0 0)
  (Effects|SpawnEmitteratLocation "/Game/DD_Vehicles_Advanced/Particles/P_glassImpact1.P_glassImpact1" (|impactpoint Hit)))

(fn OnRepSirenCounter
  (CallFunction|CEonRepSirenCounter))

(event Custom|CE_OnSirenConnectedToDP
  (Utilities|FlowControl|Gate false) ; enters at Close
)

(event Custom|CE_UnbindInputActivation
  ;[1 1 1] If destructible piece has siren attached and is disconnected...
  (EventDispatchers|UnbindEventfromOnPossessed (Variables|Default|GetCar) (stale _oncarpossessed))
  (CallFunction|CEMultiDisableSirenInteraction)
  (CallFunction|CETurnOff))

(event Custom|CE_Multi_DisableSirenInteraction
  ;[1 1 1] If destructible piece has siren attached and is disconnected...
  (Input|DisableInput 0))

(event Custom|ce_ParentPossessed
  (params (Controller :type Controller%20Object%20Reference) (Possessed :type Boolean))
  (CallFunction|CEMultiParentPossessed Controller Possessed))

(event Custom|CE_Multi_ParentPossessed
  (params (Controller :type Controller%20Object%20Reference) (Possessed :type Boolean))
  (|activate/deactivateInput_2 Controller Possessed))