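; Base Blueprint template for supercar vehicles, extending a parent vehicle class with a digital dashboard widget.
; On BeginPlay it casts the DigitalDashboard component's widget to WBP_DigitalDashboard and assigns itself as that widget's vehicle.
; When the car explodes, it runs the parent explosion logic and then hides the dashboard and its children.
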(event EventBeginPlay
  (|CallParentFunction)
  (bind _aswbp_digital_dashboard (Utilities|Casting|CastToWBP_DigitalDashboard (UserInterface|GetWidget (Variables|Default|GetDigital_Dashboard))))
  (Variables|/Game/DD_Vehicles_Advanced/Blueprints/Widgets/WBP_DigitalDashboard.WBP_DigitalDashboard_C|SetVehicle _aswbp_digital_dashboard self))

(event EventExplode
  (|CallParentFunction)
  (Development|SetHiddeninGame (Variables|Default|GetDigital_Dashboard) true true))

(fn ConstructionScript
  (|CallParentFunction))