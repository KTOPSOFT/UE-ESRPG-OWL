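; Cargo truck vehicle template with box body B, adding destructible box and door pieces that block pawns and a beeper that sounds when reversing.
; After polling until pieces and seats initialize, it can match cargo material to the cabin's through a data table, defaulting to the cabin material.
; Cargo material goes onto eligible destructible pieces at construction and BeginPlay, and is copied to the respawned truck.
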(event EventBeginPlay
  (bind _self self)
  (bind _returnvalue (Utilities|GetClass _self))
  (|CallParentFunction)
  ;[0 0 0] Set collision Box - Pawn
  (for _array_element (Utilities|Array|MakeArray (Variables|Default|GetDP_BoxB) (Variables|Default|GetDP_BoxBRightDoor) (Variables|Default|GetDP_BoxBRearDoor) (Variables|Default|GetDP_BoxBLeftDoor))
    (bind _asbp_destructible_piece (Utilities|Casting|CastToBP_DestructiblePiece (Variables|/Script/Engine.ChildActorComponent|GetChildActor _array_element)))
    (Collision|SetCollisionResponsetoChannel (Variables|/Game/DD_Vehicles_Advanced/Blueprints/Vehicles/BP_DestructiblePiece.BP_DestructiblePiece_C|GetCollisionMesh _asbp_destructible_piece) "ECC_Pawn" "ECR_Block"))
  (|Waitnetworksynchro)
  (Utilities|FlowControl|Delay 1.0)
  (if (Variables|Material|GetuseMaterialDataTable)
    ;[1 1 1] CARGO MATERIAL FOR CUSTOMIZER
    ;;[0.3498 0.3198 1] if cabin material is on the custom materials list, apply corresponding material to cargo. If not, apply same material than cabin
    ;;;[1 1 1] get row data
    (bind _outrownames (DataTable|GetDataTableRowNames "/Game/DD_Vehicles_Advanced/Blueprints/Structs/DT_CargoTruck/DT_CargoTruckMats.DT_CargoTruckMats"))
    (for _array_element_2 _outrownames
      (bind _returnvalue_2 (Utilities|GetDataTableRow "/Game/DD_Vehicles_Advanced/Blueprints/Structs/DT_CargoTruck/DT_CargoTruckMats.DT_CargoTruckMats" _array_element_2)
        (:then
          (if (or (Utilities|ClassIsChildOf _returnvalue (.CargoTruckType (Utilities|Struct|BreakBPS_CargoTruckMats _returnvalue_2))) (== (.CargoTruckType (Utilities|Struct|BreakBPS_CargoTruckMats _returnvalue_2)) _returnvalue))
            (if (== (.CabinMaterial (Utilities|Struct|BreakBPS_CargoTruckMats _returnvalue_2)) (Utilities|Array|Get(acopy) (Variables|Default|GetMaterialsRef)))
              (Variables|Material|SetCargoMaterial (.CargoMaterial (Utilities|Struct|BreakBPS_CargoTruckMats _returnvalue_2)))
              (goto _label Close))))))
    (Utilities|FlowControl|Sequence
      (:then_0
        ;;;[1 1 1] Cargo Material = Cabin Material
        (Utilities|FlowControl|Gate false :!label _label
          (:Exit
            (Variables|Material|SetCargoMaterial (Utilities|Array|Get(acopy) (Variables|Default|GetMaterialsRef))))))
      (:then_1
        ;;[1 1 1] apply cargo material on correct parts
        (Utilities|FlowControl|Delay 0.2)
        (for _array_element_3 (CallFunction|GetDestructiblePieces)
          (if (not (Variables|/Game/DD_Vehicles_Advanced/Blueprints/Vehicles/BP_DestructiblePiece.BP_DestructiblePiece_C|GetinheritParentMainMat _array_element_3))
            (if (Variables|/Game/DD_Vehicles_Advanced/Blueprints/Vehicles/BP_DestructiblePiece.BP_DestructiblePiece_C|GethasCustomMaterial _array_element_3)
              (Rendering|Material|SetMaterial (Variables|/Game/DD_Vehicles_Advanced/Blueprints/Vehicles/BP_DestructiblePiece.BP_DestructiblePiece_C|GetDeformableMesh _array_element_3) 0 (Variables|Material|GetCargoMaterial)))))))
    (else
      ;[0 0 0] set cargo  Material
      (for _array_element_4 (CallFunction|GetDestructiblePieces)
        (if (not (Variables|/Game/DD_Vehicles_Advanced/Blueprints/Vehicles/BP_DestructiblePiece.BP_DestructiblePiece_C|GetinheritParentMainMat _array_element_4))
          (if (Variables|/Game/DD_Vehicles_Advanced/Blueprints/Vehicles/BP_DestructiblePiece.BP_DestructiblePiece_C|GethasCustomMaterial _array_element_4)
            (Rendering|Material|SetMaterial (Variables|/Game/DD_Vehicles_Advanced/Blueprints/Vehicles/BP_DestructiblePiece.BP_DestructiblePiece_C|GetDeformableMesh _array_element_4) 0 (Variables|Material|GetCargoMaterial))))))))

(event Collision|EventActorBeginOverlap
  (params (OtherActor :type Actor%20Object%20Reference))
  (|CallParentFunction OtherActor) ; This node is disabled and will not be called.\nDrag off pins to build functionality.
)

(event EventCEMultiSetMatRefonRespawnedCar
  (params (RespCar :type BP%20New%20Base%20Vehicle%20Object%20Reference))
  ;[0 0 0] Respawn witrh same material
  (|CallParentFunction RespCar)
  (bind _asbp_cargo_truck_template_box_b (Utilities|Casting|CastToBP_CargoTruck_Template_BoxB RespCar))
  (Variables|BP_CargoTruck_Template_BoxB_C|SetCargoMaterial _asbp_cargo_truck_template_box_b (Variables|Material|GetCargoMaterial)))

(event EventTick
  (params (DeltaSeconds :type Float%20%28single-precision%29))
  (bind _vehiclemovementcomponent (Variables|Default|GetVehicleMovementComponent))
  ;[0 0 0] beep sound on rear gear
  (|CallParentFunction 0.0)
  (if (and (< (Vehicle|GetForwardSpeed _vehiclemovementcomponent) 0.0) (== (Class|ChaosVehicleMovementComponent|GetCurrentGear _vehiclemovementcomponent) -1))
    (Components|Activation|Activate (Variables|Default|GetBeepSound) false)
    (else
      (Components|Activation|Deactivate (Variables|Default|GetBeepSound)))))

(fn ConstructionScript
  (|CallParentFunction)
  (for _array_element (CallFunction|GetDestructiblePieces)
    (if (not (Variables|/Game/DD_Vehicles_Advanced/Blueprints/Vehicles/BP_DestructiblePiece.BP_DestructiblePiece_C|GetinheritParentMainMat _array_element))
      (if (Variables|/Game/DD_Vehicles_Advanced/Blueprints/Vehicles/BP_DestructiblePiece.BP_DestructiblePiece_C|GethasCustomMaterial _array_element)
        (Rendering|Material|SetMaterial (Variables|/Game/DD_Vehicles_Advanced/Blueprints/Vehicles/BP_DestructiblePiece.BP_DestructiblePiece_C|GetDeformableMesh _array_element) 0 (Variables|Material|GetCargoMaterial))))))