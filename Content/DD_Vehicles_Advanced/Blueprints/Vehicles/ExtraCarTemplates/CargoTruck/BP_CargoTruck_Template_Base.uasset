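; Base Blueprint template for a cargo truck vehicle that adds a reversing beep on top of its parent vehicle class.
; On Tick, after calling the parent, it activates BeepSound while forward speed is negative and the movement component is in reverse gear, and deactivates it otherwise.
; The construction script only calls the parent, and BeginPlay and overlap events are disabled stubs.
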(event EventBeginPlay
  (|CallParentFunction) ; This node is disabled and will not be called.\nDrag off pins to build functionality.
)

(event Collision|EventActorBeginOverlap
  (params (OtherActor :type Actor%20Object%20Reference))
  (|CallParentFunction OtherActor) ; This node is disabled and will not be called.\nDrag off pins to build functionality.
)

(event EventTick
  (params (DeltaSeconds :type Float%20%28single-precision%29))
  (bind _vehiclemovementcomponent (Variables|Default|GetVehicleMovementComponent))
  ;[0 0 0] beep sound on rear gear
  (|CallParentFunction 0.0)
  (if (and (< (Vehicle|GetForwardSpeed _vehiclemovementcomponent) 0.0) (== (Class|ChaosVehicleMovementComponent|GetCurrentGear _vehiclemovementcomponent) -1))
    (Components|Activation|Activate (Variables|Default|GetBeepSound) false)
    (else
      (Components|Activation|Deactivate (Variables|Default|GetBeepSound)))))

(fn ConstructionScript
  (|CallParentFunction))