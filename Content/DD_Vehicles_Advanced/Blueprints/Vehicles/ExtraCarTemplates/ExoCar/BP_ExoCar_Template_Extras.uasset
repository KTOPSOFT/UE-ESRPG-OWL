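; ExoCar vehicle template Blueprint that sets a secondary material on the car mesh to match its primary material.
; It looks up the first MaterialsRef entry in a Materials map and applies the paired material to slot 4, falling back to black carbon fiber.
; The same logic runs in the Construction Script and again shortly after BeginPlay, each following the parent's implementation.
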(event EventBeginPlay
  (|CallParentFunction)
  (Utilities|FlowControl|Delay 0.2)
  (bind _asmaterial_instance (Utilities|Casting|CastToMaterialInstance (Utilities|Array|Get(acopy) (Variables|Default|GetMaterialsRef))))
  (if (.ReturnValue (Utilities|Map|Find (Variables|Default|GetMaterials) _asmaterial_instance))
    (Rendering|Material|SetMaterial (Variables|Character|GetMesh) 4 (.Value (Utilities|Map|Find (Variables|Default|GetMaterials) _asmaterial_instance)))
    (else
      (Rendering|Material|SetMaterial (Variables|Character|GetMesh) 4 "/Game/DD_Vehicles_Advanced/Materials/Material_Instances/Cars/CarPaint/exoCarAdvanced/MI_ExoCar_CustomCarbonBlackFiber.MI_ExoCar_CustomCarbonBlackFiber"))))

(fn ConstructionScript
  (|CallParentFunction)
  (bind _asmaterial_instance (Utilities|Casting|CastToMaterialInstance (Utilities|Array|Get(acopy) (Variables|Default|GetMaterialsRef))))
  (if (.ReturnValue (Utilities|Map|Find (Variables|Default|GetMaterials) _asmaterial_instance))
    (Rendering|Material|SetMaterial (Variables|Character|GetMesh) 4 (.Value (Utilities|Map|Find (Variables|Default|GetMaterials) _asmaterial_instance)))
    (else
      (Rendering|Material|SetMaterial (Variables|Character|GetMesh) 4 "/Game/DD_Vehicles_Advanced/Materials/Material_Instances/Cars/CarPaint/exoCarAdvanced/MI_ExoCar_CustomCarbonBlackFiber.MI_ExoCar_CustomCarbonBlackFiber"))))