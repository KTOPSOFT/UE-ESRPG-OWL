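; BP_BaseCar is a base car Blueprint that can save and apply its configuration through a template.
; SaveCarConfiguration and ApplyCarConfiguration pass the car and its ConfigTemplate to get and set helpers, after checking that the template is valid.
; Tick and the construction script only call the parent, and BeginPlay is disabled, so the Blueprint adds no runtime driving logic in its graphs.
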(event EventBeginPlay
  (|CallParentFunction) ; This node is disabled and will not be called.\nDrag off pins to build functionality.
)

(event Collision|EventActorBeginOverlap
  (params (OtherActor :type Actor%20Object%20Reference)))

(event EventTick
  (params (DeltaSeconds :type Float%20%28single-precision%29))
  (|CallParentFunction DeltaSeconds))

(event EventApplyCarConfiguration
  ;[0 0.09483 1] Car Template
  (Utilities|IsValid (Variables|Default|GetConfigTemplate)
    (:Is%20Valid
      (CallFunction|SetCarConfigto self (Variables|Default|GetConfigTemplate)))))

(event EventSaveCarConfiguration
  ;[0 0.09483 1] Car Template
  (Utilities|IsValid (Variables|Default|GetConfigTemplate)
    (:Is%20Valid
      (CallFunction|GetCarConfigfrom self (Variables|Default|GetConfigTemplate)))))

(fn ConstructionScript
  (|CallParentFunction))