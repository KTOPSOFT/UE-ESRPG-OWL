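; Replicated physics vehicle door with animated open/close, configured from the car's per-door template matched by tag.
; A timeline interpolates keyframed transforms on a bone-attached animation root, while a server-side physics handle drags the simulated door toward that moving reference.
; Opening releases a tagged locking constraint; closing relocks it, and a hit while opening can block seat access and trigger closing.
; Handle transforms, passenger hold blending and VR grab-based seat trigger toggling are supported.
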(event Custom|CE_Server_SetCurrentHandle
  (params (CurrentHandle :type E_DoorHandle%20Enum :default "NewEnumerator0"))
  ;[1 1 1] RPCs
  (Variables|Animation|SetCurrentHandle CurrentHandle))

(event Custom|CE_StartDoorRelease
  ;[1 0.4397 0] Animation Notify Calls
  ;;[0 0 0] Passenger Releasing Doors
  (Networking|SwitchHasAuthority
    (:Authority
      (CallFunction|CEMultiStartDoorRelease))))

(event Custom|CE_Multi_SetCurrentHandle
  (params (CurrentHandle :type E_DoorHandle%20Enum :default "NewEnumerator0"))
  ;[1 1 1] RPCs
  (Variables|Animation|SetCurrentHandle CurrentHandle))

(event Custom|CE_Multi_SetLockingConstraintState
  (params (ConstraintType :type Byte))
  ;[1 1 1] RPCs
  (CallFunction|SetLockingConstraintState ConstraintType))

(event Custom|CE_StartDoorHold
  ;[1 0.4397 0] Animation Notify Calls
  ;;[0 0 0] Passenger Releasing Doors
  (Networking|SwitchHasAuthority
    (:Authority
      (CallFunction|CEMultiStartDoorHold))))

(event Custom|CE_CloseDoor
  ;[1 0.4397 0] Animation Notify Calls
  ;;[0 0 0] Door Open/Close animation
  (Networking|SwitchHasAuthority
    (:Authority
      (Utilities|PreconfDoorAnim "Backward"
        (:HasAnimData
          (CallFunction|CEMultiPlayCloseFeedbacks)
          (CallFunction|GrabDoor)
          (Physics|SetSimulatePhysics (Variables|Default|GetCollisionMesh) true)
          (bind (_direction _alpha) (Timeline|DoorAnim ReverseFromEnd)
            (:Update
              (Utilities|FlowControl|Sequence
                (:then_0
                  (|Updateanimindex _direction _alpha))
                (:then_1
                  (|Updateanimmovement _direction _alpha))))
            (:Finished
              (Variables|Animation|SetMovingDoor false)
              (if (not (Utilities|Enum|Equal(Enum) _direction "Forward"))
                (|Lockdoor)))))))))

(event Custom|CE_SetCurrentHandle
  (params (CurrentHandle :type E_DoorHandle%20Enum :default "NewEnumerator0"))
  ;[1 1 1] RPCs
  (Networking|SwitchHasAuthority
    (:Authority
      (CallFunction|CEMultiSetCurrentHandle CurrentHandle))
    (:Remote
      (CallFunction|CEServerSetCurrentHandle CurrentHandle))))

(event Custom|CE_OpenDoor
  ;[1 0.4397 0] Animation Notify Calls
  ;;[0 0 0] Door Open/Close animation
  (Networking|SwitchHasAuthority
    (:Authority
      (Utilities|PreconfDoorAnim "Forward"
        (:HasAnimData
          (|Unlockdoor)
          (CallFunction|GrabDoor)
          (Physics|SetSimulatePhysics (Variables|Default|GetCollisionMesh) true)
          (bind (_direction _alpha) (Timeline|DoorAnim PlayFromStart)
            (:Update
              (Utilities|FlowControl|Sequence
                (:then_0
                  (|Updateanimindex _direction _alpha))
                (:then_1
                  (|Updateanimmovement _direction _alpha))))
            (:Finished
              (Variables|Animation|SetMovingDoor false)
              (if (not (Utilities|Enum|Equal(Enum) _direction "Forward"))
                (|Lockdoor)))))))))

(event Custom|CE_StopDoorAnim
  ;[1 0.4397 0] Animation Notify Calls
  ;;[0 0 0] Door Open/Close animation
  (CallFunction|DropDoor)
  (bind (_direction _alpha) (Timeline|DoorAnim Stop)
    (:Update
      (Utilities|FlowControl|Sequence
        (:then_0
          (|Updateanimindex _direction _alpha))
        (:then_1
          (|Updateanimmovement _direction _alpha))))
    (:Finished
      (Variables|Animation|SetMovingDoor false)
      (if (not (Utilities|Enum|Equal(Enum) _direction "Forward"))
        (|Lockdoor)))))

(event Custom|CE_Multi_StartDoorHold
  ;[1 0.4397 0] Animation Notify Calls
  ;;[0 0 0] Passenger Releasing Doors
  (bind _animationblend (Timeline|TL_DoorHoldingBlend PlayFromStart)
    (:Update
      (Variables|Animation|SetHoldingDoorWeight _animationblend))))

(event Custom|CE_Multi_StartDoorRelease
  ;[1 0.4397 0] Animation Notify Calls
  ;;[0 0 0] Passenger Releasing Doors
  (bind _animationblend (Timeline|TL_DoorHoldingBlend ReverseFromEnd)
    (:Update
      (Variables|Animation|SetHoldingDoorWeight _animationblend))))

(event EventTick
  (params (DeltaSeconds :type Float%20%28single-precision%29))
  ;[0 1 0] Event Tick
  (|CallParentFunction DeltaSeconds)
  (Networking|SwitchHasAuthority
    (:Authority
      (|GrabIKupdate))))

(event EventCEonConstruction
  ;[0 1 0] Construction
  (|CallParentFunction)
  (if (Variables|Default|GetOverrideCarTemplate)
    _
    (else
      (|SetDoortemplate)))
  (|Sethandlestransforms)
  (|Setanimationvalues))

(event EventCEonSynchComplete
  ;[0 1 0] Begin Play
  (|CallParentFunction)
  (Utilities|FlowControl|Sequence
    (:then_0
      (|Sethandlestransforms(OnCompìlations))
      (|Dooranimationprecofigurations))
    (:then_1
      (|AdvancedVRconfiguration))))

(event EventOnDisplacementThresholdReached
  (params (Greater :type Boolean))
  ;[1 1 1] VR Grabbable
  (Collision|SetCollisionEnabled (Variables|/Game/DD_Vehicles_Advanced/Blueprints/Vehicles/BP_Seat.BP_Seat_C|GetTrigger (Variables|Advanced|GetSeat)) (select Greater "QueryOnly" "NoCollision"))
  (Variables|Advanced|SetLocked Greater))

(fn ConstructionScript
  (|CallParentFunction))

(fn GetHandleTrns
  (params (Type :type E_DoorHandle%20Enum :default "NewEnumerator0"))
  (return (Utilities|Select :Index Type :NewEnumerator0 (Transformation|GetActorTransform (Variables|/Script/Engine.ChildActorComponent|GetChildActor (Variables|Default|GetOuterHandle))) :NewEnumerator1 (Transformation|GetActorTransform (Variables|/Script/Engine.ChildActorComponent|GetChildActor (Variables|Default|GetInnerHandle))) :NewEnumerator2 (Transformation|GetActorTransform (Variables|/Script/Engine.ChildActorComponent|GetChildActor (Variables|Default|GetOuterClosingPoint))))))

(fn GrabDoor
  (Class|PhysicsHandleComponent|GrabComponentatLocation (Variables|Default|GetDoorAnimHandle) (Variables|Default|GetCollisionMesh) "None" (Transformation|GetWorldLocation (Variables|/Script/Engine.Actor|GetRootComponent (Variables|/Script/Engine.ChildActorComponent|GetChildActor (Variables|Default|GetOuterHandle)))))
  (Variables|Animation|SetSmoothingOutGrab true)
  (Variables|Animation|SetMovingDoor true))

(fn DropDoor
  (Physics|Components|PhysicsHandle|ReleaseComponent (Variables|Default|GetDoorAnimHandle))
  (Variables|Animation|SetMovingDoor false))

(event Custom|CE_StopOpening
  ;[0 0 0] On door Hit Bind
  (|Stopopeninganimationifrequired))

(event Custom|CE_ResetBlockCheking
  ;[0 0 0] Stop Passenger Out With Door
  (Variables|/Game/DD_Vehicles_Advanced/Blueprints/Vehicles/BP_Seat.BP_Seat_C|SetAccessBlocked (Variables|Advanced|GetSeat) false)
  (Utilities|FlowControl|DoOnce false) ; enters at Reset
)