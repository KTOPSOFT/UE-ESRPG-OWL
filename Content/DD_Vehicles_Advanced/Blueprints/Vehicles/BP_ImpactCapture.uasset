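; BP_ImpactCapture is an actor that paints impact damage into a car's render target mask.
; SetRenderTarget binds car and pieces to the scene capture, feeding the mask into dynamic car paint and glass materials.
; Each hit briefly swaps in an unwrap material and captures that brush stroke into a paint or glass channel.
; Busy or delayed requests queue in ToPaint; glass hits spawn shards and requeue a later pass into another channel.
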(event Custom|CE_StartPainting
  (params (Piece :type BP%20Destructible%20Piece%20Object%20Reference) (MatIndex :type Integer) (HitLocation :type Vector) (BrushBounds :type Vector) (BrushDirection :type Vector) (ImpactHardness :type Float%20%28double-precision%29) (ImpactIntensity :type Float%20%28double-precision%29))
  ;[1 0.9948 0.9948] Recursive Paint
  ;;[0 0 0] Start Paint Request
  (Utilities|MPaintMask Piece MatIndex HitLocation BrushBounds BrushDirection ImpactHardness ImpactIntensity 0.0))

(event Custom|CE_ContinuePainting
  (bind _topaint (Variables|RecursivePaint|GetToPaint))
  ;[1 0.9948 0.9948] Recursive Paint
  ;;[0 0 0] Paint From Request List
  (Utilities|FlowControl|Delay 0.0)
  (if (> (Utilities|Array|Length _topaint) 0)
    (Variables|Default|SetCurrentPaintData (Utilities|Array|Get(acopy) _topaint))
    (Utilities|Array|RemoveIndex _topaint)
    (Utilities|MPaintMask (.piecetopaint (Variables|Default|GetCurrentPaintData)) (.matindextopaint (Variables|Default|GetCurrentPaintData)) (.hitlocation (Variables|Default|GetCurrentPaintData)) (.impactbounds (Variables|Default|GetCurrentPaintData)) (.brushdirection (Variables|Default|GetCurrentPaintData)) (.impacthardness (Variables|Default|GetCurrentPaintData)) (.impactintensity (Variables|Default|GetCurrentPaintData)) (.timetopaint (Variables|Default|GetCurrentPaintData)))))

(event EventBeginPlay
  ;[0.04519 0.4735 0] Begin Play
  ;;[0 0 0] Initialize Unwrap Material
  (bind _returnvalue (Rendering|Material|CreateDynamicMaterialInstance "/Game/DD_Vehicles_Advanced/Materials/Masters/M_Unwrap.M_Unwrap" "None" "None" :!class /Script/Engine.KismetMaterialLibrary))
  (Variables|Default|SetUnwrapMaterial _returnvalue)
  ;;[0 0 0] Reset Impact Capturer Pos
  (Transformation|SetWorldLocation (Variables|Default|GetDefaultSceneRoot) (Variables|Default|GetCapturerDisabledLocation) false false)
  (Utilities|MInitializeParameters))

(fn ConstructionScript)

(fn SetRenderTarget
  (params (carReference :type BP%20New%20Base%20Vehicle%20Object%20Reference))
  (Variables|Default|SetCarBinded carReference)
  ;[1 1 1] Include car and its destructiblePiece actors to capture component visibility list
  (bind _output_get (Variables|/Script/Engine.SceneCaptureComponent|SetShowOnlyActors (Variables|Default|GetGlobalImpacts%20Capture) (Default|GetDestructiblePieces carReference)))
  (Utilities|Array|Add _output_get carReference)
  (Utilities|Array|Add _output_get self)
  ;[1 1 1] Set Texture Targets
  (Variables|/Script/Engine.SceneCaptureComponent2D|SetTextureTarget (Variables|Default|GetGlobalImpacts%20Capture) (Variables|/Game/DD_Vehicles_Advanced/Blueprints/Vehicles/BP_NewBaseVehicle.BP_NewBaseVehicle_C|GetImpactRenderTarget carReference))
  ;[1 1 1] Set target Render texture as mask on destructible materials
  (for _array_element (Default|GetDestructiblePieces carReference)
    ;;[1 1 1] dynamic Car Paint material from mesh material
    (LocalVariables|SetCurrentPiece _array_element)
    (Utilities|Array|Clear (Variables|/Game/DD_Vehicles_Advanced/Blueprints/Vehicles/BP_DestructiblePiece.BP_DestructiblePiece_C|GetImpactMatIDs _array_element))
    (LocalVariables|SetMeshToPaint (Variables|/Game/DD_Vehicles_Advanced/Blueprints/Vehicles/BP_DestructiblePiece.BP_DestructiblePiece_C|GetDeformableMesh _array_element))
    (for (_array_element_2 _array_index) (Variables|/Game/DD_Vehicles_Advanced/Blueprints/Vehicles/BP_DestructiblePiece.BP_DestructiblePiece_C|GetMaterialsRef (LocalVariables|GetCurrentPiece))
      (Utilities|IsValid _array_element_2
        (:Is%20Valid
          ;;;[0 0 0] Check Destructible Parent Reference
          (bind _returnvalue (Rendering|Material|GetBaseMaterial _array_element_2))
          (if (== _returnvalue "/Game/DD_Vehicles_Advanced/Materials/Masters/M_Carpaint.M_Carpaint")
            (Variables|/Game/DD_Vehicles_Advanced/Blueprints/Vehicles/BP_DestructiblePiece.BP_DestructiblePiece_C|SethasImpactMaterial (LocalVariables|GetCurrentPiece) true)
            (Utilities|Array|Add (Variables|/Game/DD_Vehicles_Advanced/Blueprints/Vehicles/BP_DestructiblePiece.BP_DestructiblePiece_C|GetImpactMatIDs (LocalVariables|GetCurrentPiece)) _array_index)
            (bind _returnvalue_2 (Rendering|Material|CreateDynamicMaterialInstance _array_element_2 "None" "None" :!class /Script/Engine.KismetMaterialLibrary))
            (Rendering|Material|SetTextureParameterValue _returnvalue_2 "ImpactMask" (Variables|/Script/Engine.SceneCaptureComponent2D|GetTextureTarget (Variables|Default|GetGlobalImpacts%20Capture)))
            (Rendering|Material|SetMaterial (LocalVariables|GetMeshToPaint) _array_index _returnvalue_2)))))
    (CallFunction|InitializeGlassMaterials (LocalVariables|GetCurrentPiece)))
  ;[1 1 1] Set target Render texture as mask on bodywork
  ;;[1 1 1] dynamic Car Paint material from mesh material
  (Utilities|Array|Clear (Variables|/Game/DD_Vehicles_Advanced/Blueprints/Vehicles/BP_NewBaseVehicle.BP_NewBaseVehicle_C|GetImpactMatIDs (Variables|Default|GetCarBinded)))
  (for (_array_element_3 _array_index_2) (Variables|/Game/DD_Vehicles_Advanced/Blueprints/Vehicles/BP_NewBaseVehicle.BP_NewBaseVehicle_C|GetMaterialsRef (Variables|Default|GetCarBinded))
    (Utilities|IsValid _array_element_3
      (:Is%20Valid
        ;;;[0 0 0] Check Destructible Parent Reference
        (bind _returnvalue_3 (Rendering|Material|GetBaseMaterial _array_element_3))
        (if (== _returnvalue_3 "/Game/DD_Vehicles_Advanced/Materials/Masters/M_Carpaint.M_Carpaint")
          (Variables|/Game/DD_Vehicles_Advanced/Blueprints/Vehicles/BP_NewBaseVehicle.BP_NewBaseVehicle_C|SetHasImpactMaterial carReference true)
          (Utilities|Array|Add (Variables|/Game/DD_Vehicles_Advanced/Blueprints/Vehicles/BP_NewBaseVehicle.BP_NewBaseVehicle_C|GetImpactMatIDs (Variables|Default|GetCarBinded)) _array_index_2)
          (bind _returnvalue_4 (Rendering|Material|CreateDynamicMaterialInstance _array_element_3 "None" "None" :!class /Script/Engine.KismetMaterialLibrary))
          (Rendering|Material|SetTextureParameterValue _returnvalue_4 "ImpactMask" (Variables|/Script/Engine.SceneCaptureComponent2D|GetTextureTarget (Variables|Default|GetGlobalImpacts%20Capture)))
          (Rendering|Material|SetMaterial (Variables|/Script/ChaosVehicles.WheeledVehiclePawn|GetMesh (Variables|Default|GetCarBinded)) _array_index_2 _returnvalue_4)))))
  (CallFunction|InitializeGlassMaterials carReference)
  ;[1 1 1] Clear Render Targets
  (Rendering|ClearRenderTarget2D (Variables|/Script/Engine.SceneCaptureComponent2D|GetTextureTarget (Variables|Default|GetGlobalImpacts%20Capture))))

(fn InitializeGlassMaterials
  (params (DestructibleActor :type Actor%20Object%20Reference))
  (bind _asbp_new_base_vehicle (Utilities|Casting|CastToBP_NewBaseVehicle DestructibleActor)
    (:then
      (LocalVariables|SetCarReference _asbp_new_base_vehicle)
      (bind _outrownames (DataTable|GetDataTableRowNames (Variables|/Game/DD_Vehicles_Advanced/Blueprints/Vehicles/BP_NewBaseVehicle.BP_NewBaseVehicle_C|GetMorphBinds (LocalVariables|GetCarReference))))
      (for _array_element _outrownames
        (bind _returnvalue (Utilities|GetDataTableRow (Variables|/Game/DD_Vehicles_Advanced/Blueprints/Vehicles/BP_NewBaseVehicle.BP_NewBaseVehicle_C|GetMorphBinds (LocalVariables|GetCarReference)) _array_element)
          (:then
            (bind _array_element_2 (Utilities|Array|ForEachLoopwithBreak (.ConectedGlass (Utilities|Struct|BreakBPS_MophsBinds _returnvalue)))
              (:LoopBody
                (if (not (Utilities|Array|ContainsItem (LocalVariables|GetInitializedIndex) (.MaterialIndex (Utilities|Struct|BreakBPS_BindGlassData _array_element_2))))
                  (Utilities|Array|Add (LocalVariables|GetInitializedIndex) (.MaterialIndex (Utilities|Struct|BreakBPS_BindGlassData _array_element_2)))
                  ;[1 1 1] Create Dynamic Material from Index on mesh
                  (if (Utilities|Array|IsValidIndex (Variables|/Game/DD_Vehicles_Advanced/Blueprints/Vehicles/BP_NewBaseVehicle.BP_NewBaseVehicle_C|GetMaterialsRef (LocalVariables|GetCarReference)) (.MaterialIndex (Utilities|Struct|BreakBPS_BindGlassData _array_element_2)))
                    (bind _returnvalue_2 (Rendering|Material|CreateDynamicMaterialInstance (Utilities|Array|Get(acopy) (Variables|/Game/DD_Vehicles_Advanced/Blueprints/Vehicles/BP_NewBaseVehicle.BP_NewBaseVehicle_C|GetMaterialsRef (LocalVariables|GetCarReference)) (.MaterialIndex (Utilities|Struct|BreakBPS_BindGlassData _array_element_2))) "None" "None" :!class /Script/Engine.KismetMaterialLibrary))
                    ;[1 1 1] Set Impact Render Texture
                    (Rendering|Material|SetTextureParameterValue _returnvalue_2 "ImpactMask" (Variables|/Script/Engine.SceneCaptureComponent2D|GetTextureTarget (Variables|Default|GetGlobalImpacts%20Capture)))
                    ;[1 1 1] Crack Border Mask
                    (Rendering|Material|SetTextureParameterValue _returnvalue_2 "CrackBorder" (Variables|/Game/DD_Vehicles_Advanced/Blueprints/Vehicles/BP_NewBaseVehicle.BP_NewBaseVehicle_C|GetCrackBorderMask (Variables|Default|GetCarBinded)))
                    (Rendering|Material|SetMaterial (Variables|/Script/ChaosVehicles.WheeledVehiclePawn|GetMesh (LocalVariables|GetCarReference)) (.MaterialIndex (Utilities|Struct|BreakBPS_BindGlassData _array_element_2)) _returnvalue_2)))))))))
    (:CastFailed
      (bind _asbp_destructible_piece (Utilities|Casting|CastToBP_DestructiblePiece DestructibleActor))
      (LocalVariables|SetDestructilbePieceReference _asbp_destructible_piece)
      (bind _outrownames_2 (DataTable|GetDataTableRowNames (Variables|/Game/DD_Vehicles_Advanced/Blueprints/Vehicles/BP_DestructiblePiece.BP_DestructiblePiece_C|GetmorphBinds (LocalVariables|GetDestructilbePieceReference))))
      (for _array_element_3 _outrownames_2
        (bind _returnvalue_3 (Utilities|GetDataTableRow (Variables|/Game/DD_Vehicles_Advanced/Blueprints/Vehicles/BP_DestructiblePiece.BP_DestructiblePiece_C|GetmorphBinds (LocalVariables|GetDestructilbePieceReference)) _array_element_3)
          (:then
            (bind _array_element_4 (Utilities|Array|ForEachLoopwithBreak (.ConectedGlass (Utilities|Struct|BreakBPS_MophsBinds _returnvalue_3)))
              (:LoopBody
                (if (not (Utilities|Array|ContainsItem (LocalVariables|GetInitializedIndex) (.MaterialIndex (Utilities|Struct|BreakBPS_BindGlassData _array_element_4))))
                  (Utilities|Array|Add (LocalVariables|GetInitializedIndex) (.MaterialIndex (Utilities|Struct|BreakBPS_BindGlassData _array_element_4)))
                  ;[1 1 1] Create Dynamic Material from Index on mesh
                  (if (Utilities|Array|IsValidIndex (Variables|/Game/DD_Vehicles_Advanced/Blueprints/Vehicles/BP_DestructiblePiece.BP_DestructiblePiece_C|GetMaterialsRef (LocalVariables|GetDestructilbePieceReference)) (.MaterialIndex (Utilities|Struct|BreakBPS_BindGlassData _array_element_4)))
                    (bind _returnvalue_4 (Rendering|Material|CreateDynamicMaterialInstance (Utilities|Array|Get(acopy) (Variables|/Game/DD_Vehicles_Advanced/Blueprints/Vehicles/BP_DestructiblePiece.BP_DestructiblePiece_C|GetMaterialsRef (LocalVariables|GetDestructilbePieceReference)) (.MaterialIndex (Utilities|Struct|BreakBPS_BindGlassData _array_element_4))) "None" "None" :!class /Script/Engine.KismetMaterialLibrary))
                    ;[1 1 1] Set Impact Render Texture
                    (Utilities|IsValid _returnvalue_4
                      (:Is%20Valid
                        (Rendering|Material|SetTextureParameterValue _returnvalue_4 "ImpactMask" (Variables|/Script/Engine.SceneCaptureComponent2D|GetTextureTarget (Variables|Default|GetGlobalImpacts%20Capture)))
                        ;[1 1 1] Crack Border Mask
                        (Rendering|Material|SetTextureParameterValue _returnvalue_4 "CrackBorder" (Variables|/Game/DD_Vehicles_Advanced/Blueprints/Vehicles/BP_NewBaseVehicle.BP_NewBaseVehicle_C|GetCrackBorderMask (Variables|Default|GetCarBinded)))
                        (Rendering|Material|SetMaterial (Variables|/Game/DD_Vehicles_Advanced/Blueprints/Vehicles/BP_DestructiblePiece.BP_DestructiblePiece_C|GetDeformableMesh (LocalVariables|GetDestructilbePieceReference)) (.MaterialIndex (Utilities|Struct|BreakBPS_BindGlassData _array_element_4)) _returnvalue_4)))))))))))))