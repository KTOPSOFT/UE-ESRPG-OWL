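; A collision component for BP_NewBaseVehicle actors that marks a damageable area able to set the vehicle on fire or blow it up.
; Damage arrives through the ITakeDamage interface or from overlaps with explosion-tagged actors or components, lowering the area's resistance.
; With a valid linked particle system, low resistance asks the vehicle to start a fire there, and depleted resistance triggers its explosion, each gated by flags.
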(event Custom|OnComponentBeginOverlap_Event_0
  (params (OverlappedComponent :type Primitive%20Component%20Object%20Reference) (OtherActor :type Actor%20Object%20Reference) (OtherComp :type Primitive%20Component%20Object%20Reference) (OtherBodyIndex :type Integer) (bFromSweep :type Boolean) (SweepResult :type Hit%20Result%20Structure%20%28by%20ref%29))
  (bind _explosiontag (Variables|Default|GetExplosionTag))
  (if (or (Actor|ActorHasTag OtherActor _explosiontag) (Components|ComponentHasTag OtherComp _explosiontag))
    (if (Variables|Default|GetCanBeDamaged)
      (CallFunction|TakeDamage (Variables|Default|GetDefaultDamage)))))

(event EventBeginPlay
  (Collision|SetCollisionEnabled "QueryOnly")
  (bind _asbp_new_base_vehicle (Utilities|Casting|CastToBP_NewBaseVehicle (Components|GetOwner))
    (:then
      (Variables|Default|SetVehicle _asbp_new_base_vehicle)
      (Variables|Default|SetCurrentResistance (Variables|Default|GetExplosionResistance))
      (Collision|AssignOnComponentBeginOverlap (delegate Custom|OnComponentBeginOverlap_Event_0)))
    (:CastFailed
      (|WarningMessage))))

(event EventITakeDamage
  (params (Damage :type Float%20%28double-precision%29) (Location :type Vector :default "0, 0, 0") (Direction :type Vector :default "0, 0, 0"))
  (CallFunction|TakeDamage Damage))

(fn TakeDamage
  (params (Damage :type Float%20%28double-precision%29))
  ;[0 0 0] Subtract damage to resistance
  (bind _output_get (Variables|Default|SetCurrentResistance (- (Variables|Default|GetCurrentResistance) Damage)))
  ;[0 0 0] Check if has to start fire
  (Utilities|IsValid (Variables|Default|GetLinkedVehicleParticleSystem)
    (:Is%20Valid
      (if (Math|Boolean|ANDBoolean (<= _output_get (Variables|Default|GetResistance%20to%20start%20fire)) (not (Components|Activation|IsActive (Variables|Default|GetLinkedVehicleParticleSystem))) (Variables|Default|GetCanCatchFire))
        (Default|CEStartFire (Variables|Default|GetVehicle) (Variables|Default|GetLinkedVehicleParticleSystem) self))
      ;[0 0 0] Check if has to explode
      (if (and (<= (Variables|Default|GetCurrentResistance) 0.0) (Variables|Default|GetCanExplode))
        (Default|Explode (Variables|Default|GetVehicle))))))