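; Base bike Blueprint for the advanced vehicle system that marks itself as not a car and serves as a minimal parent for specific bikes.
; It declares empty hooks for rider ejection, sidestand and anim updates, plus stub getters for lift locations and relative velocity.
; A macro gates input while airborne unless air control is enabled.
; Each tick, a billboard macro yaws a text render toward the player pawn.
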(event Custom|CE_ActivateSidestand
  (params (Active :type Boolean))
  ;[1 0 0] Minimun necessary
)

(event Custom|CE_StopBikeAfterEjected
  ;[1 0 0] Minimun necessary
)

(event Custom|CE_RiderEjected
  ;[1 0 0] Minimun necessary
)

(event Custom|CE_UpdateDataOnAnimBP
  (params (FrontWheel :type Boolean))
  ;[1 0 0] Minimun necessary
)

(event EventBeginPlay
  ;[1 0 0] Minimun necessary
  (Variables|Default|SetIsCar false))

(event EventTick
  (params (DeltaSeconds :type Float%20%28single-precision%29))
  ;[1 0 0] Minimun necessary
  (|Billboard))

(event EventActiveSideStand
  (params (Active :type Boolean))
  ;[1 1 1] Bike Interface
)

(fn ConstructionScript
  (|CallParentFunction))

(fn GetCenterOfMass
  (return (Variables|Default|GetCenterOffMassOffset)))

(fn GetLiftLocations
  (return "" ""))

(fn GetRelativeVelocity
  (return "0, 0, 0"))