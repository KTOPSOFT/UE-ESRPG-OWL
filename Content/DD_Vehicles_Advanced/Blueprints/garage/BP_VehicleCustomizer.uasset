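; Garage customizer podium that lets a player reconfigure a vehicle overlapping it.
; Server-side overlaps track the user, who becomes the actor's owner, and the vehicle, driving multicast podium feedback, an Enhanced Input mapping and a client-side menu.
; Opening the menu locks the car against interaction.
; Configuration requests go through a server event to a multicast that spawns the new vehicle class, copies materials, moves seated controllers across and destroys the old car.
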(event Custom|CE_Multi_InteractionFeedbacks
  (params (Active :type Boolean))
  ;[1 1 1] RPCs
  ;;[0 0 0] Feedbacks
  ;;;[1 1 1] activate podium
  (Audio|PlaySoundatLocation (select Active "/Game/DD_Vehicles_Advanced/Sound/cues/general/SC_alarm_2.SC_alarm_2" "/Game/DD_Vehicles_Advanced/Sound/cues/general/SC_Click_on_Button.SC_Click_on_Button") (Transformation|GetActorLocation) "0, 0, 0" 1.0 1.0 0.0 0 0 0 0)
  (Rendering|Material|SetMaterial (Variables|Default|Getpodium) 0 (select Active (Variables|Default|Getmaterial_on) (Variables|Default|Getmaterial_off)))
  ;;;[1 1 1] spotlight
  (Rendering|SetVisibility (Variables|Default|GetRectLight) Active false)
  ;;;[1 1 1] Texts
  (if (not Active)
    (CallFunction|SetTextsVisibility true)))

(event Custom|CE_Server_ConfigurationRequest
  (params (NewCarClass :type Actor%20Class%20Reference) (NewMainMat :type Material%20Interface%20Object%20Reference) (DamageAffectEngine :type Boolean))
  ;[1 1 1] RPCs
  ;;[0 0 0] Create new vehicle
  (CallFunction|CEMultiCreateNewVehicle NewCarClass NewMainMat DamageAffectEngine))

(event Custom|CE_MultiCreateNewVehicle
  (params (NewCarClass :type Actor%20Class%20Reference) (NewMainMaterial :type Material%20Interface%20Object%20Reference) (DamageAffectEngine :type Boolean))
  ;[1 1 1] RPCs
  ;;[0 0 0] Create new vehicle
  (Variables|Default|SetNew%20Main%20Mat NewMainMaterial)
  ;;;[1 1 1] update old vehicle ref
  (bind _output_get (Variables|Default|SetOldVehicle (Variables|Default|GetVehicle)))
  (Variables|/Game/DD_Vehicles_Advanced/Blueprints/Vehicles/BP_NewBaseVehicle.BP_NewBaseVehicle_C|SetInteractionLocked _output_get true)
  ;;;[1 1 1] disable collision
  (Variables|Default|SetVehicle 0)
  (Collision|SetActorEnableCollision (Variables|Default|GetOldVehicle) false)
  ;;;[1 1 1] get location from old vehicle
  (Variables|Default|SetcarTransfrom (Transformation|GetActorTransform (Variables|Default|GetOldVehicle)))
  ;;;[1 1 1] spawn vehicle
  (bind _returnvalue (Game|SpawnActorfromClass NewCarClass (|relocatecarabovefloor) "Undefined" 0 0))
  (bind _output_get_2 (Variables|Default|SetNewVehicle (.AsBP%20New%20Base%20Vehicle (Utilities|Casting|CastToBP_NewBaseVehicle _returnvalue))))
  (Variables|/Game/DD_Vehicles_Advanced/Blueprints/Vehicles/BP_NewBaseVehicle.BP_NewBaseVehicle_C|SetInteractionLocked _output_get_2 true)
  ;;;[0 0 0] SetMaterialsInSpawnedCar
  (|SetOldVehicleMatsOnNewVehicle (Variables|Default|GetOldVehicle))
  (Default|CEMultiSetMatRefonRespawnedCar (Variables|Default|GetNewVehicle) (Variables|Default|GetNewVehicle))
  (|Movecontrollerstonewcar (Variables|Default|GetNewVehicle))
  ;;;[1 1 1] destroy old vehicle
  (Actor|DestroyActor (Variables|Default|GetOldVehicle))
  (Variables|/Game/DD_Vehicles_Advanced/Blueprints/Vehicles/BP_NewBaseVehicle.BP_NewBaseVehicle_C|SetdamageAffectSpeed (Variables|Default|GetNewVehicle) DamageAffectEngine)
  (Variables|Default|SetVehicle (Variables|Default|GetNewVehicle)))

(event Custom|CE_Client_ShowCustomizerUI
  (bind _config_menu (Variables|Default|Getconfig_menu))
  ;[1 1 1] RPCs
  ;;[0 0 0] Show Widget
  (|Setcustomizerreferencetomenu)
  (Utilities|FlowControl|Sequence
    (:then_0
      (Utilities|FlowControl|Delay 1.0)
      (Utilities|FlowControl|Gate true :!label _label
        (:Exit
          (Input|EnableInput (Game|GetPlayerController 0))
          (CallFunction|SetTextsVisibility false)
          (Utilities|IsValid (Variables|Default|GetVehicle)
            (:Is%20Valid
              (Default|CeShowConfigurator _config_menu true))
            (:Is%20Not%20Valid
              (Default|CeShowConfigurator _config_menu false))))))
    (:then_1
      (goto _label Open))))

(event Custom|CE_Client_HideCustomizerUI
  (bind _returnvalue (Game|GetPlayerController 0))
  (bind _config_menu (Variables|Default|Getconfig_menu))
  ;[1 1 1] RPCs
  ;;[0 0 0] Hide Widget
  (Utilities|IsValid _config_menu
    (:Is%20Valid
      (Default|CeShowConfigurator _config_menu false)
      (Widget|RemovefromParent _config_menu)
      (Input|DisableInput _returnvalue)
      (Variables|/Script/Engine.PlayerController|SetbShowMouseCursor _returnvalue false)
      (Input|SetInputModeGameOnly _returnvalue false))))

(event Custom|CE_Server_TurnOffCustomizer
  ;[1 1 1] RPCs
  ;;[0 0 0] Turn off customizer
  (Variables|Default|SetCurrentUser 0)
  ;;;[1 1 1] Feedbacks
  (CallFunction|CEMultiInteractionFeedbacks false))

(event Custom|CE_StopCustomizerInitialization
  (bind _config_menu (Variables|Default|Getconfig_menu))
  ;[1 1 1] RPCs
  ;;[0 0 0] Show Widget
  (Utilities|FlowControl|Gate true) ; enters at Close
)

(event Custom|CE_Client_UpdateCustomizerUI
  (params (CanWork :type Boolean))
  ;[1 1 1] RPCs
  ;;[0 0 0] Update Widget
  (Utilities|IsValid (Variables|Default|Getconfig_menu)
    (:Is%20Valid
      (Default|CeShowConfigurator (Variables|Default|Getconfig_menu) CanWork))))

(event Custom|CE_Server_LockCar
  (params (Lock :type Boolean))
  (bind _vehicle (Variables|Default|GetVehicle))
  ;[1 1 1] RPCs
  ;;[0 0 0] Update Widget
  (Utilities|IsValid _vehicle
    (:Is%20Valid
      (Variables|/Game/DD_Vehicles_Advanced/Blueprints/Vehicles/BP_NewBaseVehicle.BP_NewBaseVehicle_C|SetInteractionLocked _vehicle Lock))))

(event Custom|CE_RemoveInputs
  ;[0.141 0 1] enhanced inputs
  (|RemoveInputMapping) ; enhanced inputs
)

(event Custom|CE_AddInputs
  (params (Pawn :type Actor%20Object%20Reference))
  ;[0.141 0 1] enhanced inputs
  (|AddInputMapping Pawn) ; enhanced inputs
)

(event Input|EnhancedActionEvents|EnhancedInputActionIA_Interact
  (params (ActionValue :type Boolean) (ElapsedSeconds :type Float%20%28double-precision%29) (TriggeredSeconds :type Float%20%28double-precision%29) (InputAction :type Input%20Action%20Object%20Reference :default "/Game/DD_Vehicles_Advanced/Blueprints/Passenger/Input/Actions/IA_Interact.IA_Interact"))
  ;[1 1 1] Customizer Off
  ;;[0 0 0] Input Interact
  (:Started
    (CallFunction|CEClientHideCustomizerUI)
    (CallFunction|CEServerTurnOffCustomizer)
    (CallFunction|CEServerLockCar false)))

(event Input|EnhancedActionEvents|EnhancedInputActionIA_CustomizeCar
  (params (ActionValue :type Boolean) (ElapsedSeconds :type Float%20%28double-precision%29) (TriggeredSeconds :type Float%20%28double-precision%29) (InputAction :type Input%20Action%20Object%20Reference :default "/Game/DD_Vehicles_Advanced/Blueprints/GeneralInputs/Actions/IA_CustomizeCar.IA_CustomizeCar"))
  (bind _returnvalue (Game|GetPlayerController 0))
  (bind _config_menu (Variables|Default|Getconfig_menu))
  ;[1 1 1] Customizer Interaction
  (:Started
    ;;[0 0 0] add / remove widget
    (if (UserInterface|Viewport|IsinViewport _config_menu)
      (Widget|RemovefromParent _config_menu)
      (CallFunction|SetTextsVisibility false)
      ;;[0 0 0] set input mode
      (Variables|/Script/Engine.PlayerController|SetbShowMouseCursor _returnvalue false)
      (Input|SetInputModeGameOnly _returnvalue false)
      ;;[0 0 0] feedbacks
      (Audio|PlaySoundatLocation "/Game/DD_Vehicles_Advanced/Sound/cues/general/SC_Click_on_Button.SC_Click_on_Button" (Transformation|GetActorLocation) "0, 0, 0" 1.0 1.0 0.0 0 0 0 0)
      (CallFunction|CEServerLockCar false)
      (else
        (UserInterface|Viewport|AddtoViewport _config_menu 0)
        (CallFunction|SetTextsVisibility true)
        (Input|SetInputModeGameandUI (Game|GetPlayerController 0) 0 "DoNotLock" true false)
        (Variables|/Script/Engine.PlayerController|SetbShowMouseCursor (Game|GetPlayerController 0) true)
        (Audio|PlaySoundatLocation "/Game/DD_Vehicles_Advanced/Sound/cues/general/SC_alarm_2.SC_alarm_2" (Transformation|GetActorLocation) "0, 0, 0" 1.0 1.0 0.0 0 0 0 0)
        (CallFunction|CEServerLockCar true)))))

(event Collision|EventActorBeginOverlap
  (params (OtherActor :type Actor%20Object%20Reference))
  ;[1 1 1] begin overlap
  (Networking|SwitchHasAuthority
    (:Authority
      (Utilities|IsValid (Variables|Default|GetCurrentUser)
        (:Is%20Valid
          ;;[0 0 0] vehicle overlap
          (if (and (not (Utilities|IsValid (Variables|Default|GetVehicle))) (not (Utilities|IsValid (Variables|Default|GetOldVehicle)))) :!label _label
            (bind _asbp_new_base_vehicle (Utilities|Casting|CastToBP_NewBaseVehicle OtherActor))
            (Variables|Default|SetVehicle _asbp_new_base_vehicle)
            (CallFunction|CEClientUpdateCustomizerUI true)))
        (:Is%20Not%20Valid
          ;;[0 0 0] character overlap
          (if (or (Utilities|DoesObjectImplementInterface OtherActor "/Game/DD_Vehicles_Advanced/Blueprints/Passenger/BP_Interface_CarPassenger.BP_Interface_CarPassenger_C") (== (Utilities|GetClass OtherActor) "/Game/DD_Vehicles_Advanced/Blueprints/FirstPersonBP/BP_FirstPersonCharacter.BP_FirstPersonCharacter_C"))
            ;;;[0 0 0] assign controller this blueprint
            (bind _aspawn (Utilities|Casting|CastToPawn OtherActor))
            (bind _asplayer_controller (Utilities|Casting|CastToPlayerController (Pawn|GetController _aspawn)))
            (Variables|Default|SetCurrentController _asplayer_controller)
            (bind _output_get (Variables|Default|SetCurrentUser _aspawn))
            (Actor|SetOwner _output_get)
            ;;;[1 1 1] Feedbacks
            (CallFunction|CEMultiInteractionFeedbacks true)
            ;;;[1 1 1] Create widget on client
            (CallFunction|CEClientShowCustomizerUI)
            (CallFunction|CEAddInputs _output_get)
            (else
              (goto _label))))))))

(event Collision|EventActorEndOverlap
  (params (OtherActor :type Actor%20Object%20Reference))
  ;[1 1 1] Customizer Off
  ;;[0 0 0] End overlap (only player)
  (Networking|SwitchHasAuthority
    (:Authority
      (if (== (Variables|Default|GetCurrentUser) OtherActor)
        (CallFunction|CEStopCustomizerInitialization)
        (Utilities|FlowControl|Sequence
          (:then_0
            (CallFunction|CERemoveInputs))
          (:then_1
            ;;[0 0 0] Input Interact
            (CallFunction|CEClientHideCustomizerUI)
            (CallFunction|CEServerTurnOffCustomizer)
            (CallFunction|CEServerLockCar false)))
        (elif (== (Variables|Default|GetVehicle) OtherActor)
          (Variables|Default|SetVehicle 0)
          (CallFunction|CEClientUpdateCustomizerUI false)
          (Variables|Default|SetPurchaseFeedbacksActive false))))))

(fn ConstructionScript
  ;[1 1 1] get original off material
  (Variables|Default|Setmaterial_off (Rendering|Material|GetMaterial (Variables|Default|Getpodium) 0)))

(fn SetTextsVisibility
  (params (Hidden :type Boolean))
  (Development|SetHiddeninGame (Variables|Default|Getscreen) Hidden false))

(fn OnRepPurchaseFeedbacksActive)