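; Garage sliding double door that opens automatically and shatters as breakable glass.
; A main trigger box plays or reverses a timeline, with audio, sliding both panels in opposite directions for characters and static or skeletal mesh components.
; Each panel has a one-shot box that, on mesh overlap, swaps it for a physics-simulated Geometry Collection.
; Chaos break events play smash sounds at volume scaled by fragment mass.
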(event OnChaosBreakEvent(GC_SlidingDoor2)
  (params (BreakEvent :type Chaos%20Break%20Event%20Structure%20%28by%20ref%29))
  (bind (_component _location _velocity _angularvelocity _mass) (Utilities|Struct|BreakChaosBreakEvent BreakEvent))
  ;[0 0 0] Broken glass sound
  (Audio|PlaySoundatLocation "/Game/DD_Vehicles_Advanced/Sound/cues/general/glass_smash_Cue.glass_smash_Cue" _location "0, 0, 0" (/ _mass 1e+03) 1.0 0.0 "/Game/DD_Vehicles_Advanced/Sound/Impacts_Att.Impacts_Att" 0 0 0))

(event OnComponentBeginOverlap(Box)
  (params (OverlappedComponent :type Primitive%20Component%20Object%20Reference) (OtherActor :type Actor%20Object%20Reference) (OtherComp :type Primitive%20Component%20Object%20Reference) (OtherBodyIndex :type Integer) (bFromSweep :type Boolean) (SweepResult :type Hit%20Result%20Structure%20%28by%20ref%29))
  ;[0 0 0] Door Open/Close Motion and Sound
  (Utilities|Casting|CastToCharacter OtherActor
    (:then
      _)
    (:CastFailed
      (Utilities|Casting|CastToStaticMeshComponent OtherComp
        (:then
          _)
        (:CastFailed
          (Utilities|Casting|CastToSkeletalMeshComponent OtherComp)))))
  (Audio|Components|Audio|Play (Variables|Default|GetAudio) 0.0)
  (bind _doormovement (Timeline|Timeline_0 Play)
    (:Update
      (Transformation|SetRelativeLocation (Variables|Default|Getsm_slidingDoor1) (Math|Vector|MakeVector 0.0 _doormovement 0.0) false false)
      (Transformation|SetRelativeLocation (Variables|Default|Getsm_slidingDoor2) (* (Math|Vector|MakeVector 0.0 _doormovement 0.0) -1.0) false false))
    (:Finished
      (Audio|Components|Audio|Stop (Variables|Default|GetAudio)))))

(event OnComponentEndOverlap(Box)
  (params (OverlappedComponent :type Primitive%20Component%20Object%20Reference) (OtherActor :type Actor%20Object%20Reference) (OtherComp :type Primitive%20Component%20Object%20Reference) (OtherBodyIndex :type Integer))
  ;[0 0 0] Door Open/Close Motion and Sound
  (Utilities|Casting|CastToCharacter OtherActor
    (:then
      _)
    (:CastFailed
      (Utilities|Casting|CastToStaticMeshComponent OtherComp
        (:then
          _)
        (:CastFailed
          (Utilities|Casting|CastToSkeletalMeshComponent OtherComp)))))
  (Audio|Components|Audio|Play (Variables|Default|GetAudio) 0.0)
  (bind _doormovement (Timeline|Timeline_0 Reverse)
    (:Update
      (Transformation|SetRelativeLocation (Variables|Default|Getsm_slidingDoor1) (Math|Vector|MakeVector 0.0 _doormovement 0.0) false false)
      (Transformation|SetRelativeLocation (Variables|Default|Getsm_slidingDoor2) (* (Math|Vector|MakeVector 0.0 _doormovement 0.0) -1.0) false false))
    (:Finished
      (Audio|Components|Audio|Stop (Variables|Default|GetAudio)))))

(event OnComponentBeginOverlap(Box1)
  (params (OverlappedComponent :type Primitive%20Component%20Object%20Reference) (OtherActor :type Actor%20Object%20Reference) (OtherComp :type Primitive%20Component%20Object%20Reference) (OtherBodyIndex :type Integer) (bFromSweep :type Boolean) (SweepResult :type Hit%20Result%20Structure%20%28by%20ref%29))
  (bind _box1 (Variables|Default|GetBox1))
  ;[0 0 0] Hide regular mesh and show destructible mesh
  (Utilities|Casting|CastToStaticMeshComponent OtherComp
    (:then
      _)
    (:CastFailed
      (Utilities|Casting|CastToSkeletalMeshComponent OtherComp)))
  (Utilities|IsValid _box1
    (:Is%20Valid
      (Components|DestroyComponent _box1)
      (Rendering|SetVisibility (Variables|Default|Getsm_slidingDoor1) false false)
      (Development|SetHiddeninGame (Variables|Default|Getsm_slidingDoor1) true false)
      (Rendering|SetVisibility (Variables|Default|GetGC_SlidingDoor1) true false)
      (Development|SetHiddeninGame (Variables|Default|GetGC_SlidingDoor1) false false)
      (Physics|SetSimulatePhysics (Variables|Default|GetGC_SlidingDoor1) true))))

(event OnComponentBeginOverlap(Box2)
  (params (OverlappedComponent :type Primitive%20Component%20Object%20Reference) (OtherActor :type Actor%20Object%20Reference) (OtherComp :type Primitive%20Component%20Object%20Reference) (OtherBodyIndex :type Integer) (bFromSweep :type Boolean) (SweepResult :type Hit%20Result%20Structure%20%28by%20ref%29))
  (bind _box2 (Variables|Default|GetBox2))
  ;[0 0 0] Hide regular mesh and show destructible mesh
  (Utilities|Casting|CastToStaticMeshComponent OtherComp
    (:then
      _)
    (:CastFailed
      (Utilities|Casting|CastToSkeletalMeshComponent OtherComp)))
  (Utilities|IsValid _box2
    (:Is%20Valid
      (Components|DestroyComponent _box2)
      (Rendering|SetVisibility (Variables|Default|Getsm_slidingDoor2) false false)
      (Development|SetHiddeninGame (Variables|Default|Getsm_slidingDoor2) true false)
      (Rendering|SetVisibility (Variables|Default|GetGC_SlidingDoor2) true false)
      (Development|SetHiddeninGame (Variables|Default|GetGC_SlidingDoor2) false false)
      (Physics|SetSimulatePhysics (Variables|Default|GetGC_SlidingDoor2) true))))

(event OnChaosBreakEvent(GC_SlidingDoor1)
  (params (BreakEvent :type Chaos%20Break%20Event%20Structure%20%28by%20ref%29))
  (bind (_component _location _velocity _angularvelocity _mass) (Utilities|Struct|BreakChaosBreakEvent BreakEvent))
  ;[0 0 0] Broken glass sound
  (Audio|PlaySoundatLocation "/Game/DD_Vehicles_Advanced/Sound/cues/general/glass_smash_Cue.glass_smash_Cue" _location "0, 0, 0" (/ _mass 1e+03) 1.0 0.0 "/Game/DD_Vehicles_Advanced/Sound/Impacts_Att.Impacts_Att" 0 0 0))

(fn ConstructionScript)