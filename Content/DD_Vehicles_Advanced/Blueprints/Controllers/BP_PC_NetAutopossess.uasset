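; Player controller that lets a player hop into a random vehicle in the level by pressing O, apparently for networked possession.
; A DoOnce with a one-second reset throttles the key before calling the server seat event.
; That event frees any seat currently held, as driver or passenger, then requests seat 0, without forcing entry, on a randomly picked BP_NewBaseVehicle actor.
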(event Custom|CE_Server_PlaceOnSeat
  ;[1 1 1] Possess/Unpossess random car in level
  (|Checkplayercanentercar)
  (bind _car (|Getrandomcar))
  (Default|PlaceonSeat _car self 0 false))

(event Custom|CE_PossessRandomCar
  ;[1 1 1] Possess/Unpossess random car in level
  (Utilities|FlowControl|DoOnce false :!label _label
    (:Completed
      (Utilities|FlowControl|Sequence
        (:then_0
          (CallFunction|CEServerPlaceonSeat))
        (:then_1
          (Utilities|FlowControl|Delay 1.0)
          (goto _label Reset))))))

(event Input|KeyboardEvents|O
  (params (Key :type Key%20Structure))
  (:Pressed
    ;[1 1 1] Possess/Unpossess random car in level
    (Utilities|FlowControl|DoOnce false :!label _label
      (:Completed
        (Utilities|FlowControl|Sequence
          (:then_0
            (CallFunction|CEServerPlaceonSeat))
          (:then_1
            (Utilities|FlowControl|Delay 1.0)
            (goto _label Reset)))))))

(fn ConstructionScript)