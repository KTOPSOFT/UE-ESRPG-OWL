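; Blueprint interface for characters that act as car passengers in the advanced vehicle system.
; It declares seat events and references, entrance and exit checks, and accessors for car state, driving, seat changing, door opening and movement.
; It also covers collision response to cars, impact notifications with a hard-impact threshold, and full-ragdoll recovery state such as facing, standing up and hip location.
; All functions are empty declarations for implementers to fill.
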(fn OnSeatTaken)

(fn OnSeatLeft)

(fn SetSeatReference
  (params (Seat :type BP%20Seat%20Object%20Reference)))

(fn GetSeatReference
  (return 0))

(fn SetCarState
  (params (State :type E_PassengerStates%20Enum :default "NewEnumerator0")))

(fn GetCarState
  (return "NewEnumerator0"))

(fn SetOpeningwithDoor
  (params (NewValue :type Boolean)))

(fn GetOpeningwithDoor
  (return false))

(fn SetDriving
  (params (NewValue :type Boolean)))

(fn GetDriving
  (return false))

(fn SetChangingSeat
  (params (NewValue :type Boolean)))

(fn GetChangingSeat
  (return false))

(fn SetEnableMovement
  (params (NewValue :type Boolean)))

(fn GetEnableMovement
  (return false))

(fn SetResponsetoCars
  (params (Response :type ECollisionResponse%20Enum :default "ECR_Ignore")))

(fn OnEntranceCheck
  (params (ValidEntrance :type Boolean)))

(fn OnExitCheck
  (params (ValidExit :type Boolean)))

(fn SetRunningEntranceExit
  (params (Running :type Boolean)))

(fn GetRunningEntranceExit
  (return false))

(fn OnImpactReceived
  (params (Impact :type Vector) (HardImpactThreshold :type Float%20%28single-precision%29) (ForceType :type E_RagdollForce%20Enum :default "NewEnumerator0")))

(fn GetIsRestoringFullRagdoll
  (return false false false "0, 0, 0"))

(fn SetIsRestoringFullRagdoll
  (params (RestoringRagdoll :type Boolean) (StandUp :type Boolean))
  (return))