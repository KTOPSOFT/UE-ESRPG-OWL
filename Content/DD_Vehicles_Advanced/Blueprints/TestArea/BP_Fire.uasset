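; BP_Fire is a fire actor that damages overlapped BP_FullDestructionArea components every tick and notifies owning vehicles.
; It burns indefinitely or follows a duration-scaled timeline driving sound, named particle emitter parameters and optional flickering light, later destroying itself.
; CE_Attach pins it to a static mesh component, deriving scale and, if unspecified, duration from mesh bounds.
; Tick also keeps the overlap capsule upright.
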(event OnComponentBeginOverlap(Capsule)
  (params (OverlappedComponent :type Primitive%20Component%20Object%20Reference) (OtherActor :type Actor%20Object%20Reference) (OtherComp :type Primitive%20Component%20Object%20Reference) (OtherBodyIndex :type Integer) (bFromSweep :type Boolean) (SweepResult :type Hit%20Result%20Structure%20%28by%20ref%29))
  ;[0 0 0 1 30] Overlapping
  (bind _asbp_full_destruction_area (Utilities|Casting|CastToBP_FullDestructionArea OtherComp))
  (Variables|Default|SetDamageableArea _asbp_full_destruction_area)
  (Variables|Default|SetIsBurningSomething true)
  ;;[0 0 0] Interaction with vehicles
  (bind _asbp_new_base_vehicle (Utilities|Casting|CastToBP_NewBaseVehicle (Components|GetOwner (Variables|Default|GetDamageableArea))))
  (Default|CEReceiveFire _asbp_new_base_vehicle self (Variables|Default|GetDamageableArea)))

(event OnComponentEndOverlap(Capsule)
  (params (OverlappedComponent :type Primitive%20Component%20Object%20Reference) (OtherActor :type Actor%20Object%20Reference) (OtherComp :type Primitive%20Component%20Object%20Reference) (OtherBodyIndex :type Integer))
  ;[0 0 0 1 30] Overlapping
  (bind _asbp_full_destruction_area (Utilities|Casting|CastToBP_FullDestructionArea OtherComp))
  (if (== _asbp_full_destruction_area (Variables|Default|GetDamageableArea))
    (Variables|Default|SetIsBurningSomething false)))

(event Custom|CE_Attach
  (params (Fire%20duration%20%280%20to%20auto-calculation%29 :type Float%20%28double-precision%29) (SM%20Component%20to%20attach%20fire :type Static%20Mesh%20Component%20Object%20Reference) (Scale%20Multiplier :type Float%20%28double-precision%29))
  (bind _staticmesh (Variables|/Script/Engine.StaticMeshComponent|GetStaticMesh SM%20Component%20to%20attach%20fire))
  ;[0 0 0 1 30] Attach fire to SM Component and set scale according to bounds
  (Variables|Default|SetFireDuration Fire%20duration%20%280%20to%20auto-calculation%29)
  (Utilities|IsValid SM%20Component%20to%20attach%20fire
    (:Is%20Valid
      (Transformation|AttachComponentToComponent SM%20Component%20to%20attach%20fire "None" "KeepWorld" "KeepWorld" "KeepWorld" true)
      (Utilities|IsValid _staticmesh
        (:Is%20Valid
          (CallFunction|SetScaleandDuration (.sphereradius (StaticMesh|GetBounds _staticmesh)) Scale%20Multiplier))))))

(event EventBeginPlay
  ;[0 0 0 1 30] Begin  Play
  (if (Variables|Default|GetHasLight)
    _
    (else
      (Components|DestroyComponent (Variables|Default|GetPointLight))))
  (if (Variables|Default|GetInfiniteBurning)
    ;;[0 0 0] Infinite fire
    (Audio|Components|Audio|AdjustVolume (Variables|Default|GetFireSound) 0.0 1.0 "Linear" :!class /Script/Engine.AudioComponent)
    (Audio|Components|Audio|AdjustVolume (Variables|Default|GetFireSound) 0.0 1.0 "Linear" :!class /Script/Engine.AudioComponent)
    (CallFunction|EmitterParametersModification (Variables|Default|GetFireParticleSystem) 1.0 0.0 "BigFlames")
    (CallFunction|EmitterParametersModification (Variables|Default|GetFireParticleSystem) 1.0 0.0 "SmallFlames")
    (CallFunction|EmitterParametersModification (Variables|Default|GetFireParticleSystem) 1.0 0.0 "Smoke")
    (else
      ;;[0 0 0] Set up fire duration
      (Components|Timeline|SetPlayRate (Variables|Default|GetTimeline_0) (/ 1.0 (Variables|Default|GetFireDuration)))
      (bind _intensity (Timeline|Timeline_0 Play)
        (:Update
          (Audio|Components|Audio|AdjustVolume (Variables|Default|GetFireSound) 0.0 _intensity "Linear" :!class /Script/Engine.AudioComponent)
          (CallFunction|EmitterParametersModification (Variables|Default|GetFireParticleSystem) _intensity 0.3 "BigFlames")
          (CallFunction|EmitterParametersModification (Variables|Default|GetFireParticleSystem) _intensity 0.1 "SmallFlames")
          (CallFunction|EmitterParametersModification (Variables|Default|GetFireParticleSystem) _intensity 0.0 "Smoke")
          (if (Variables|Default|GetHasLight)
            (Rendering|Components|Light|SetIntensity (Variables|Default|GetPointLight) (* _intensity (Math|Random|RandomFloatinRange 1.5e+03 2.5e+03)))))
        (:Finished
          (Utilities|FlowControl|Delay (Variables|Default|GetFireDuration))
          (Actor|DestroyActor))))))

(event EventTick
  (params (DeltaSeconds :type Float%20%28single-precision%29))
  ;[0 0 0 1 30] Event Tick
  ;;[0 0 0] Force vertical orientation
  (Transformation|SetWorldRotation (Variables|Default|GetCapsule) "0, 0, 0" false false)
  (if (Variables|Default|GetIsBurningSomething)
    ;;[0 0 0] Damage to damageable areas
    (Default|TakeDamage (Variables|Default|GetDamageableArea) (Variables|Default|GetDamageByFrame))))

(fn ConstructionScript)

(fn EmitterParametersModification
  (params (ParticleSystem :type Particle%20System%20Component%20Object%20Reference) (ParamValue :type Float%20%28double-precision%29) (ParamAtenuation :type Float%20%28double-precision%29) (EmitterName :type Name))
  (LocalVariables|SetParam (- ParamValue ParamAtenuation))
  (Effects|Components|ParticleSystem|SetFloatParameter ParticleSystem (Utilities|String|StringToName (Utilities|String|Append (Utilities|String|ToString(Name) EmitterName) "Spawn")) (LocalVariables|GetParam))
  (Effects|Components|ParticleSystem|SetFloatParameter ParticleSystem (Utilities|String|StringToName (Utilities|String|Append (Utilities|String|ToString(Name) EmitterName) "Life")) (LocalVariables|GetParam)))

(fn SetScaleandDuration
  (params (BoundsRadius :type Float%20%28double-precision%29) (ScaleMultiplier :type Float%20%28double-precision%29))
  (bind _capsule (Variables|Default|GetCapsule))
  (bind _capsuleradius (Variables|/Script/Engine.CapsuleComponent|GetCapsuleRadius _capsule))
  (bind _returnvalue (/ BoundsRadius _capsuleradius))
  (bind _returnvalue_2 (* _returnvalue ScaleMultiplier))
  (Transformation|SetWorldScale3D (Variables|Default|GetDefaultSceneRoot) (Math|Vector|MakeVector _returnvalue_2 _returnvalue_2 _returnvalue_2))
  (if (<= (Variables|Default|GetFireDuration) 0.0)
    ;[0 0 0] Set duration based on scale
    (Variables|Default|SetFireDuration (* BoundsRadius (Math|Random|RandomFloatinRange 0.666 1.333))))
  ;[0 0 0] Set specified duration
  (Components|Timeline|SetPlayRate (Variables|Default|GetTimeline_0) (/ 1.0 (Variables|Default|GetFireDuration))))