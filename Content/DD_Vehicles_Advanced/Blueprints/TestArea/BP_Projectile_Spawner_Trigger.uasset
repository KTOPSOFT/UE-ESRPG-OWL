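; Server-authoritative test-area trigger that makes random BP_ProjectileSpawner actors fire while an actor is inside its box.
; Overlap starts an alarm and light timeline; if the actor remains after five seconds, machine sound and a gated, random-delay shooting loop start.
; Ending overlap closes the gate and stops the effects, which are driven through multicast events.
; The platform rotation node is disconnected, so only the light animates.
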(event OnComponentBeginOverlap(Box)
  (params (OverlappedComponent :type Primitive%20Component%20Object%20Reference) (OtherActor :type Actor%20Object%20Reference) (OtherComp :type Primitive%20Component%20Object%20Reference) (OtherBodyIndex :type Integer) (bFromSweep :type Boolean) (SweepResult :type Hit%20Result%20Structure%20%28by%20ref%29))
  (Networking|SwitchHasAuthority
    (:Authority
      (CallFunction|CEMultiActiveAlarm true)
      (Utilities|FlowControl|Sequence
        (:then_0
          (Utilities|FlowControl|Delay 5.0)
          (if (Collision|IsOverlappingActor OtherActor :!class /Script/Engine.Actor)
            (Variables|Default|Setrotate true)
            (CallFunction|CEMultiActiveMachine true)
            (Utilities|FlowControl|Delay (Math|Random|RandomFloatinRange (Variables|Default|Getmin_time) (Variables|Default|Getmax_time)) :!label _label)
            (Utilities|FlowControl|Gate true :!label _label_2
              (:Exit
                (Default|CeShoot (Utilities|Array|Get(acopy) (Variables|Default|Getspawners) (Math|Random|RandomIntegerinRange 0 (Variables|Default|GettotalSpawners))))
                (goto _label)))))
        (:then_1
          (goto _label_2 Open))
        (:then_2
          (CallFunction|CEMultiStartPlatformRotation))))))

(event OnComponentEndOverlap(Box)
  (params (OverlappedComponent :type Primitive%20Component%20Object%20Reference) (OtherActor :type Actor%20Object%20Reference) (OtherComp :type Primitive%20Component%20Object%20Reference) (OtherBodyIndex :type Integer))
  (Networking|SwitchHasAuthority
    (:Authority
      (Variables|Default|Setrotate false)
      (CallFunction|CEMultiActiveMachine false)
      (CallFunction|CEMultiActiveAlarm false)
      (Utilities|FlowControl|Sequence
        (:then_0
          (Utilities|FlowControl|Gate true) ; enters at Close
        )
        (:then_1
          (CallFunction|CEMultiStopPlatformRotation))))))

(event Custom|CE_Multi_ActiveMachine
  (params (Active :type Boolean))
  ;[1 1 1] Sounds (RPCs)
  (Components|Activation|SetActive (Variables|Default|Getmachine) Active false))

(event Custom|CE_Multi_ActiveAlarm
  (params (Active :type Boolean))
  ;[1 1 1] Sounds (RPCs)
  (Components|Activation|SetActive (Variables|Default|Getalarm) Active false))

(event Custom|CE_Multi_StartPlatformRotation
  ;[1 1 1] Platform Feedbacks
  (Rendering|SetVisibility (Variables|Default|GetPointLight) true false)
  (bind (_direction _light _podium) (Timeline|Timeline_0 Play)
    (:Update
      (Rendering|Components|Light|SetIntensity (Variables|Default|GetPointLight) _light)
      (Networking|SwitchHasAuthority
        (:Authority
          (if (Variables|Default|Getrotate)
            _))))))

(event Custom|CE_Multi_StopPlatformRotation
  ;[1 1 1] Platform Feedbacks
  (Rendering|SetVisibility (Variables|Default|GetPointLight) false false)
  (bind (_direction _light _podium) (Timeline|Timeline_0 Stop)
    (:Update
      (Rendering|Components|Light|SetIntensity (Variables|Default|GetPointLight) _light)
      (Networking|SwitchHasAuthority
        (:Authority
          (if (Variables|Default|Getrotate)
            _))))))

(event EventBeginPlay
  (Networking|SwitchHasAuthority
    (:Authority
      (bind _outactors (Actor|GetAllActorsOfClass "/Game/DD_Vehicles_Advanced/Blueprints/TestArea/BP_ProjectileSpawner.BP_ProjectileSpawner_C"))
      (bind _output_get (Variables|Default|Setspawners _outactors))
      (Variables|Default|SettotalSpawners (- (Utilities|Array|Length _output_get) 1)))))

(fn ConstructionScript)