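; BP_VehicleDestroyer is a test-area trigger that removes vehicles parked inside it, handling one vehicle at a time on the server.
; If the vehicle still overlaps after a short delay, it stops the car, ejects occupants and locks interaction.
; After a longer wait, a Gate cancels destruction if any seat is still occupied, unlocking the car and restarting it for a driver.
; Otherwise it plays multiplayer teleport effects and destroys the vehicle.
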(event OnComponentBeginOverlap(Vehicle_touch)
  (params (OverlappedComponent :type Primitive%20Component%20Object%20Reference) (OtherActor :type Actor%20Object%20Reference) (OtherComp :type Primitive%20Component%20Object%20Reference) (OtherBodyIndex :type Integer) (bFromSweep :type Boolean) (SweepResult :type Hit%20Result%20Structure%20%28by%20ref%29))
  ;[1 1 1] Begin Overlap
  (Networking|SwitchHasAuthority
    (:Authority
      (Utilities|IsValid (Variables|Default|Getvehicle)
        (:Is%20Not%20Valid
          (bind _asbp_new_base_vehicle (Utilities|Casting|CastToBP_NewBaseVehicle OtherActor))
          (Variables|Default|Setvehicle _asbp_new_base_vehicle)
          (Utilities|FlowControl|Delay 3.0)
          (if (Collision|IsOverlappingActor (Variables|Default|Getvehicle) :!class /Script/Engine.Actor)
            (Default|CEStopCar (Variables|Default|Getvehicle))
            (for _array_element (Variables|/Game/DD_Vehicles_Advanced/Blueprints/Vehicles/BP_NewBaseVehicle.BP_NewBaseVehicle_C|GetSeats (Variables|Default|Getvehicle))
              (Utilities|IsValid (Variables|/Game/DD_Vehicles_Advanced/Blueprints/Vehicles/BP_Seat.BP_Seat_C|GetController _array_element)
                (:Is%20Valid
                  (Default|CEExitCar (Variables|Default|Getvehicle) (Variables|/Game/DD_Vehicles_Advanced/Blueprints/Vehicles/BP_Seat.BP_Seat_C|GetController _array_element))
                  (Variables|/Game/DD_Vehicles_Advanced/Blueprints/Vehicles/BP_NewBaseVehicle.BP_NewBaseVehicle_C|SetInteractionLocked (Variables|Default|Getvehicle) true))))
            (Utilities|FlowControl|Delay 7.0)
            (Utilities|FlowControl|Sequence
              (:then_0
                (goto _label_2 Open))
              (:then_1
                (bind (_array_element_2 _array_index) (Utilities|Array|ForEachLoopwithBreak (Variables|/Game/DD_Vehicles_Advanced/Blueprints/Vehicles/BP_NewBaseVehicle.BP_NewBaseVehicle_C|GetSeats (Variables|Default|Getvehicle)) :!label _label)
                  (:LoopBody
                    (Utilities|IsValid (Variables|/Game/DD_Vehicles_Advanced/Blueprints/Vehicles/BP_Seat.BP_Seat_C|GetController _array_element_2)
                      (:Is%20Valid
                        (if (== _array_index 0)
                          (Default|CeStartCar (Variables|Default|Getvehicle)))
                        (Utilities|FlowControl|Sequence
                          (:then_0
                            (Variables|/Game/DD_Vehicles_Advanced/Blueprints/Vehicles/BP_NewBaseVehicle.BP_NewBaseVehicle_C|SetInteractionLocked (Variables|Default|Getvehicle) false)
                            (goto _label_2 Close))
                          (:then_1
                            (goto _label Break))))))
                  (:Completed
                    (Utilities|FlowControl|Sequence
                      (:then_0
                        (Utilities|FlowControl|Gate false :!label _label_2
                          (:Exit
                            (CallFunction|CEMultiActiveFeedbacks)
                            (Actor|DestroyActor (Variables|Default|Getvehicle)))))
                      (:then_1
                        (Utilities|FlowControl|Delay 1.0)
                        (Variables|Default|Setvehicle 0)))))))
            (else
              (Variables|Default|Setvehicle 0))))))))

(event Custom|CE_Multi_ActiveFeedbacks
  ;[1 1 1] Feedbacks (Multiplayer)
  (Effects|SpawnEmitteratLocation "/Game/DD_Vehicles_Advanced/Particles/PS_Teleport.PS_Teleport" (Transformation|GetActorLocation))
  (Audio|PlaySoundatLocation "/Game/DD_Vehicles_Advanced/Sound/cues/general/SC_teleport.SC_teleport" (Transformation|GetActorLocation) "0, 0, 0" 1.0 1.0 0.0 0 0 0))

(fn ConstructionScript)