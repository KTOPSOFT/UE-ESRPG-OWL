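; BP_Road is a spline-driven road actor in the vehicle test area that builds road geometry along its spline.
; The construction script divides the spline length by a segment distance and adds a scaled Spline Mesh Component with the road mesh for each interval.
; Each segment takes its endpoints from local spline samples and its tangents from the spline direction times a tangent factor, with query and physics collision enabled.
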(event EventTick
  (params (DeltaSeconds :type Float%20%28single-precision%29)))

(fn ConstructionScript
  (bind _spline (Variables|Default|GetSpline))
  (for _index (range 0 (.ReturnValue (Math|Float|Division(WholeandRemainder) (Spline|GetSplineLength (Variables|Default|GetSpline)) (Variables|Default|GetDistance))))
    (Variables|Default|SetLoc1 (Spline|GetLocationatDistanceAlongSpline _spline (* _index (Variables|Default|GetDistance)) "Local"))
    (Variables|Default|SetDirection1 (* (Spline|GetDirectionatDistanceAlongSpline _spline (* _index (Variables|Default|GetDistance)) "Local") (Variables|Default|GetTangent)))
    (Variables|Default|SetLoc2 (Spline|GetLocationatDistanceAlongSpline _spline (+ (* _index (Variables|Default|GetDistance)) (Variables|Default|GetDistance)) "Local"))
    (Variables|Default|SetDirection2 (* (Spline|GetDirectionatDistanceAlongSpline _spline (+ (* _index (Variables|Default|GetDistance)) (Variables|Default|GetDistance)) "Local") (Variables|Default|GetTangent)))
    (bind _returnvalue (AddComponent|AddSplineMeshComponent false (Math|Transform|MakeTransform "0, 0, 0" "0, 0, 0" (Variables|Default|GetScaleRoad))))
    (Components|StaticMesh|SetStaticMesh _returnvalue (Variables|Default|GetRoad))
    (SplineMesh|SetStartandEnd _returnvalue (Variables|Default|GetLoc1) (Variables|Default|GetDirection1) (Variables|Default|GetLoc2) (Variables|Default|GetDirection2) true :!class /Script/Engine.SplineMeshComponent)
    (Collision|SetCollisionEnabled _returnvalue "QueryAndPhysics")))