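; BP_CarSpawner is a test-area pad that spawns a random vehicle when its touch volume is overlapped.
; The server proceeds only if fewer than two actors overlap it, with a DoOnce and delayed reset preventing rapid repeat spawns.
; It fires a multiplayer event for teleport sound and particles, then spawns a class from SpawnableClasses above itself, turned sideways, and gives it a random color.
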(event OnComponentBeginOverlap(char_touch)
  (params (OverlappedComponent :type Primitive%20Component%20Object%20Reference) (OtherActor :type Actor%20Object%20Reference) (OtherComp :type Primitive%20Component%20Object%20Reference) (OtherBodyIndex :type Integer) (bFromSweep :type Boolean) (SweepResult :type Hit%20Result%20Structure%20%28by%20ref%29))
  (bind _returnvalue (Transformation|GetActorRotation))
  (bind _spawnableclasses (Variables|Default|GetSpawnableClasses))
  (bind (_roll _pitch _yaw) (Math|Rotator|BreakRotator _returnvalue))
  ;[1 1 1] Begin Overlap
  (Networking|SwitchHasAuthority
    (:Authority
      (if (< (Utilities|Array|Length (Collision|GetOverlappingActors 0 :!class /Script/Engine.Actor)) 2)
        (Utilities|FlowControl|DoOnce false :!label _label
          (:Completed
            (CallFunction|CEMultiActiveFeedbacks)
            (Utilities|FlowControl|Delay 0.2)
            (bind _returnvalue_2 (Game|SpawnActorfromClass (Utilities|Array|Get(acopy) _spawnableclasses (Math|Random|RandomIntegerinRange 0 (- (Utilities|Array|Length _spawnableclasses) 1))) (Math|Transform|MakeTransform (+ (Transformation|GetActorLocation) "0, 0,50.000000") (Math|Rotator|MakeRotator _roll _pitch (+ _yaw 9e+01))) "Undefined" 0 0))
            (CallFunction|ApplyRandomColortoCar (.AsBP%20New%20Base%20Vehicle (Utilities|Casting|CastToBP_NewBaseVehicle _returnvalue_2)))
            (Utilities|FlowControl|Delay 2.0)
            (goto _label Reset)))))))

(event Custom|CE_Multi_ActiveFeedbacks
  (bind _returnvalue (Transformation|GetActorLocation))
  ;[1 1 1] Feedbacks (Multiplayer)
  (Audio|PlaySoundatLocation "/Game/DD_Vehicles_Advanced/Sound/cues/general/SC_teleport.SC_teleport" _returnvalue "0, 0, 0" 1.0 1.0 0.0 0 0 0 0)
  (Utilities|FlowControl|Delay 0.2)
  (Effects|SpawnEmitteratLocation "/Game/DD_Vehicles_Advanced/Particles/PS_Spawn.PS_Spawn" _returnvalue))

(event EventBeginPlay
  ;[0 1 0] Begin Play
  (Class|PrimitiveComponent|IgnoreComponentwhenMoving (Variables|Default|GetspawnArea) (Variables|Default|Getpodium) true))

(fn ConstructionScript)