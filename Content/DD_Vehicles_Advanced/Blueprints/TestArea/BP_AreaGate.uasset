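; BP_AreaGate is a gate actor for the vehicle test area that displays an area name and carries spotlights.
; Its Construction Script loops over child actor components and casts each child to BP_Spotlight, toggling its light from the LightsOn flag.
; The same loop writes AreaName to two text render components.
; All event graph nodes are disabled placeholders, so it has no runtime logic.
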(event EventBeginPlay)

(event Collision|EventActorBeginOverlap
  (params (OtherActor :type Actor%20Object%20Reference)))

(event EventTick
  (params (DeltaSeconds :type Float%20%28single-precision%29)))

(fn ConstructionScript
  (for _array_element (Actor|GetComponentsByClass "/Script/Engine.ChildActorComponent")
    (bind _asbp_spotlight (Utilities|Casting|CastToBP_Spotlight (Variables|/Script/Engine.ChildActorComponent|GetChildActor _array_element)))
    (Rendering|SetVisibility (Variables|/Game/DD_Vehicles_Advanced/Blueprints/garage/BP_Spotlight.BP_Spotlight_C|GetSpotLight1 _asbp_spotlight) (Variables|Default|GetlightsOn) false)
    (Rendering|Components|TextRender|SetText (Variables|Default|GetTextRender1) (Variables|Default|Getarea%20name))))